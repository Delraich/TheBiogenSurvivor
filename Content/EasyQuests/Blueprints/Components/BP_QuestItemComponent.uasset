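; Quest item component that advances one objective of a quest, identified by QuestID and ObjectiveID.
; On every Tick it looks up and stores the Quest Component, printing a message when none is found.
; The UpdateQuestObjective event adds one to the objective's amount through that stored component, but only while the quest is active.
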(event `self.ReceiveBeginPlay`)

(event `self.ReceiveTick`
  (params (DeltaSeconds :type "Float (single-precision)"))
  (bind (_componentwasfound_ _questcomponent) (`/Game/EasyQuests/Blueprints/BPL/BP_BPL_Quests.GetQuestComponent`))
  (if _componentwasfound_
    (set `self.QuestComponent` _questcomponent)
    (else
      (`KismetSystemLibrary.PrintString` "Quest Component was not found." true true (struct :`R` 1.0 :`G` 0.052861 :`A` 1.0)))))

(event `UpdateQuestObjective`
  (if (`/Game/EasyQuests/Blueprints/BP_BPC_PlayerQuestComponent.IsQuestActive?` (`self.QuestComponent`) (`self.QuestID`))
    (`/Game/EasyQuests/Blueprints/BP_BPC_PlayerQuestComponent.AddObjectiveAmount` (`self.QuestComponent`) (`self.QuestID`) (`self.ObjectiveID`) 1)))