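; Processing component for an inventory station that converts items over time into return items and mutation progress, overriding parent cooking logic.
; UpdateCookingItems syncs slots with inventory and refills empty ones from contents items that carry mutation progress.
; UpdateCookingTimes counts down while switched on, pausing understocked slots and signalling player timers.
; Completed batches consume inputs, stack or drop outputs, and accumulate mutation totals that unlock three data-table tiers.
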(fn `Add Mutation Progress`
  (params (`Cooking Slot` :type "/Game/SurvivalGameKitV2/Blueprints/Other/Structs/S_CookingSlot Structure"))
  (bind _mutationsprogress (`/Game/SurvivalGameKitV2/Blueprints/Other/Interfaces/BP_SGKFunctions.TBS MutationProgress` (make `/Game/SurvivalGameKitV2/Blueprints/Other/Structs/S_InvItem` (`.ItemID_12_BF71A7764CB5AA9C7414C8B6682828FC` (break `/Game/SurvivalGameKitV2/Blueprints/Other/Structs/S_CookingSlot` `Cooking Slot`)))))
  (for _array_element _mutationsprogress
    (bind (_mutation _progress) (break `/Game/SurvivalGameKitV2/Blueprints/Other/Structs/S_MutationProgress` _array_element))
    (`BlueprintMapLibrary.Map_Add` (`self.MutationsProgress`) _mutation (+ (`BlueprintMapLibrary.Map_Find` (`self.MutationsProgress`) _mutation) _progress))
    (bind _keys (`BlueprintMapLibrary.Map_Keys` (`self.MutationsProgress`)))
    (for _array_element_2 _keys
      (bind (_value _returnvalue) (`BlueprintMapLibrary.Map_Find` (`self.MutationsProgress`) _array_element_2))
      (if _returnvalue
        (bind _returnvalue_2 (`|GetDataTableRow` "/Game/SurvivalGameKitV2/Blueprints/Mutations/MutationUnlockList.MutationUnlockList" _array_element_2)
          (:`then`
            (bind (_progressitems _requiredt1 _unlockt1 _requiredt2 _unlockt2 _requiredt3 _unlockt3) (break `/Game/SurvivalGameKitV2/Blueprints/Other/Structs/S_MutationUnlockDetails` _returnvalue_2))
            (if (>= _value _requiredt1)
              (`KismetArrayLibrary.Array_Add` (`self.UnlockedMutations`) _unlockt1)
              (if (>= _value _requiredt2)
                (`KismetArrayLibrary.Array_Add` (`self.UnlockedMutations`) _unlockt2)
                (if (>= _value _requiredt3)
                  (`KismetArrayLibrary.Array_Add` (`self.UnlockedMutations`) _unlockt3))))))))))

(fn `AddReturnedItems`
  (params (CookingSlot :type "/Game/SurvivalGameKitV2/Blueprints/Other/Structs/S_CookingSlot Structure"))
  (locals (ArrayElementL :type "/Game/SurvivalGameKitV2/Blueprints/Other/Structs/S_CraftingCost Structure") (InventorySlotL :type "/Game/SurvivalGameKitV2/Blueprints/Other/Structs/S_InvSlot Structure") (NewItemL :type "/Game/SurvivalGameKitV2/Blueprints/Other/Structs/S_InvItem Structure"))
  (bind _inventoryslotl (`local.InventorySlotL`))
  (bind (_item _amount) (break `/Game/SurvivalGameKitV2/Blueprints/Other/Structs/S_CraftingCost` (`local.ArrayElementL`)))
  (bind (_item_2 _amount_2) (break `/Game/SurvivalGameKitV2/Blueprints/Other/Structs/S_CraftingCost` (`local.ArrayElementL`)))
  (bind (_returnvalue_location _returnvalue_rotation) (`KismetMathLibrary.BreakTransform` (`Actor.GetTransform` (`self.GetOwner`))))
  (`|ExecutionSequence`
    (:`then_0`
      ;[1 1 1] Check processing slot item and play processing sound from item in item list
      (bind (_return_value _processing_item) (`/Game/SurvivalGameKitV2/Blueprints/Other/Interfaces/BP_SGKFunctions.TBS ProcessingItem` (struct)))
      (`/Game/SurvivalGameKitV2/Blueprints/Other/Interfaces/BP_SGKInventoryInterface.SGK ItemSound` (`.ItemID_12_BF71A7764CB5AA9C7414C8B6682828FC` (break `/Game/SurvivalGameKitV2/Blueprints/Other/Structs/S_CookingSlot` CookingSlot)))
      ;[1 1 1] Loop through returned items and search for free slot
      (for _array_element (`.ReturnItems_20_F72E0BD64C726C1B42EF91B824C8152C` (break `/Game/SurvivalGameKitV2/Blueprints/Other/Structs/S_ProcessingItem` _processing_item))
        (bind _output_get (set `local.ArrayElementL` _array_element))
        (bind (_returnvalue _invslot) (`self.FreeSlotCheck` _output_get))
        (if _returnvalue
          (set `local.InventorySlotL` _invslot)
          ;[1 1 1] If space found ad ditem to the stack and add item weight to inventory
          (if (`/Game/SurvivalGameKitV2/Blueprints/Other/Interfaces/BP_SGKFunctions.SGK InvSlotAmount` (`local.InventorySlotL`))
            (`self.SetItemAmount` (struct) (+ (`.Amount_5_62DB2267439500D86A52E0B2266494D2` (break `/Game/SurvivalGameKitV2/Blueprints/Other/Structs/S_InvItem` (`.Item_10_95D912F14C7740665FD844AF7EA87327` (break `/Game/SurvivalGameKitV2/Blueprints/Other/Structs/S_InvSlot` (`local.InventorySlotL`))))) (`.Amount_5_9BB6E2444CD3AA340121BA986DA11205` (break `/Game/SurvivalGameKitV2/Blueprints/Other/Structs/S_CraftingCost` (`local.ArrayElementL`)))))
            (`self.AddItemWeight` (`.Item_10_95D912F14C7740665FD844AF7EA87327` (break `/Game/SurvivalGameKitV2/Blueprints/Other/Structs/S_InvSlot` (`local.InventorySlotL`))) (`.Amount_5_9BB6E2444CD3AA340121BA986DA11205` (break `/Game/SurvivalGameKitV2/Blueprints/Other/Structs/S_CraftingCost` (`local.ArrayElementL`))))
            (else
              ;[1 1 1] If no stack found create new item and add it to empty inventory slot then ad weight and item count to inventory
              (bind _globalinventory (message `/Game/SurvivalGameKitV2/Blueprints/Other/Interfaces/BP_SGKGameModeInterface.SGK GetGlobalInventory` (`GameplayStatics.GetGameMode`)))
              (bind _newitem (`/Game/SurvivalGameKitV2/Blueprints/Other/BP_GlobalInventoryManager.CreateNewItem` _globalinventory (`.RowName` (break `DataTableRowHandle` _item)) _amount false false false true))
              (bind _output_get_2 (set `local.NewItemL` _newitem))
              (`self.SetNewSlotItem` (`.Inventory_13_75D853E34C33E03489A41A94465989CA` (break `/Game/SurvivalGameKitV2/Blueprints/Other/Structs/S_InvSlot` _inventoryslotl)) _inventoryslotl _output_get_2 false)
              (`self.AddItemWeight` (`local.NewItemL`))
              (`self.ChangeItemCount` (`.Amount_5_62DB2267439500D86A52E0B2266494D2` (break `/Game/SurvivalGameKitV2/Blueprints/Other/Structs/S_InvItem` (`local.NewItemL`))))))
          (else
            ;[1 1 1] If no free slot then create item and spawn it's world class then apply item to world class using the item drop function. Spawns item 1.5m from actor forward
            (bind _globalinventory_2 (message `/Game/SurvivalGameKitV2/Blueprints/Other/Interfaces/BP_SGKGameModeInterface.SGK GetGlobalInventory` (`GameplayStatics.GetGameMode`)))
            (bind _newitem_2 (`/Game/SurvivalGameKitV2/Blueprints/Other/BP_GlobalInventoryManager.CreateNewItem` _globalinventory_2 (`.RowName` (break `DataTableRowHandle` _item_2)) _amount_2 true false false true))
            (set `local.NewItemL` _newitem_2)
            (bind _returnvalue_2 (`|SpawnActorFromClass` (`.WorldClass_45_6718387F4F5D57BE9909639A237E57A3` (break `/Game/SurvivalGameKitV2/Blueprints/Other/Structs/S_ItemDetails` (`.ItemDetails` (`/Game/SurvivalGameKitV2/Blueprints/Other/Interfaces/BP_SGKFunctions.SGK ItemDetails` (make `/Game/SurvivalGameKitV2/Blueprints/Other/Structs/S_InvItem` (`.ItemID_12_BF71A7764CB5AA9C7414C8B6682828FC` (break `/Game/SurvivalGameKitV2/Blueprints/Other/Structs/S_CookingSlot` (`local.CookingSlot`)))))))) (`KismetMathLibrary.MakeTransform` (+ _returnvalue_location (* (`KismetMathLibrary.GetForwardVector` _returnvalue_rotation) 150.0))) "AlwaysSpawn" "OverrideRootScale" null null))
            (message `/Game/SurvivalGameKitV2/Blueprints/Other/Interfaces/BP_SGKInteractionInterface.SGK DropItem` _returnvalue_2 (`local.NewItemL`) false false false)))))
    (:`then_1`
      (`self.Add Mutation Progress` CookingSlot))))

(fn `SetNewCookingItem`
  (params (InvSlot :type "/Game/SurvivalGameKitV2/Blueprints/Other/Structs/S_InvSlot Structure"))
  (returns (ReturnValue :type Boolean) (CookingSlot :type "/Game/SurvivalGameKitV2/Blueprints/Other/Structs/S_CookingSlot Structure"))
  (bind _invslot (`local.InvSlot`))
  (bind (_occupied _inventory _rootindex) (break `/Game/SurvivalGameKitV2/Blueprints/Other/Structs/S_InvSlot` _invslot))
  (bind (_id _amount) (break `/Game/SurvivalGameKitV2/Blueprints/Other/Structs/S_InvItem` (`/Game/SurvivalGameKitV2/Blueprints/Other/Interfaces/BP_SGKFunctions.SGK InvSlotItem` _invslot)))
  (bind (_return_value _processing_item) (`/Game/SurvivalGameKitV2/Blueprints/Other/Interfaces/BP_SGKFunctions.TBS ProcessingItem` (`/Game/SurvivalGameKitV2/Blueprints/Other/Interfaces/BP_SGKFunctions.SGK InvSlotItem` InvSlot)))
  (if _return_value
    (`KismetArrayLibrary.Array_Set` (`self.CookingSlots`) _rootindex (make `/Game/SurvivalGameKitV2/Blueprints/Other/Structs/S_CookingSlot` _id (`.ProcessingTime_13_1A30D84540A47981B8B1989067493A64` (break `/Game/SurvivalGameKitV2/Blueprints/Other/Structs/S_ProcessingItem` _processing_item)) _amount _rootindex) true)
    (return false (`|GetArrayItem` (`self.CookingSlots`) (`.RootIndex_4_31C49987405FF01267287D9E3381FC5E` (break `/Game/SurvivalGameKitV2/Blueprints/Other/Structs/S_InvSlot` (`local.InvSlot`)))))))

(fn `UpdateCookingItems`
  (locals (ArrayElementL :type "/Game/SurvivalGameKitV2/Blueprints/Other/Structs/S_InvSlot Structure") (ContentsElementL :type "/Game/SurvivalGameKitV2/Blueprints/Other/Structs/S_InvSlot Structure") (ProcessingElementL :type "/Game/SurvivalGameKitV2/Blueprints/Other/Structs/S_CookingSlot Structure"))
  (bind (_itemid _time _amount _index) (break `/Game/SurvivalGameKitV2/Blueprints/Other/Structs/S_CookingSlot` (`local.ProcessingElementL`)))
  ;[1 1 1] Loop through all the processing slots
  (`KismetArrayLibrary.Array_Clear` (`self.PausedIndexs`))
  (bind (_returnvalue _cookingslots) (`self.GetCookingInvSlots`))
  (if _returnvalue
    (for _array_element _cookingslots
      (set `local.ArrayElementL` _array_element)
      ;[1 1 1] Is processing slot valid
      (if (`KismetArrayLibrary.Array_IsValidIndex` (`self.CookingSlots`) (`.RootIndex_4_31C49987405FF01267287D9E3381FC5E` (break `/Game/SurvivalGameKitV2/Blueprints/Other/Structs/S_InvSlot` (`local.ArrayElementL`))))
        ;[1 1 1] Get processing slot from index
        (set `local.ProcessingElementL` (`|GetArrayItem` (`self.CookingSlots`) (`.RootIndex_4_31C49987405FF01267287D9E3381FC5E` (break `/Game/SurvivalGameKitV2/Blueprints/Other/Structs/S_InvSlot` (`local.ArrayElementL`)))))
        ;[1 1 1] Check if the inventory slot item is the same as the processing slot item
        (if (== (`.ItemID_12_BF71A7764CB5AA9C7414C8B6682828FC` (break `/Game/SurvivalGameKitV2/Blueprints/Other/Structs/S_CookingSlot` (`local.ProcessingElementL`))) (`.ID_2_84C2CB8945979246059C568DCD463423` (break `/Game/SurvivalGameKitV2/Blueprints/Other/Structs/S_InvItem` (`.Item_10_95D912F14C7740665FD844AF7EA87327` (break `/Game/SurvivalGameKitV2/Blueprints/Other/Structs/S_InvSlot` (`local.ArrayElementL`))))))
          ;[1 1 1] Check that the amounts of the inventory sot and processing slot are the same
          (if (== (`.Amount_5_62DB2267439500D86A52E0B2266494D2` (break `/Game/SurvivalGameKitV2/Blueprints/Other/Structs/S_InvItem` (`.Item_10_95D912F14C7740665FD844AF7EA87327` (break `/Game/SurvivalGameKitV2/Blueprints/Other/Structs/S_InvSlot` (`local.ArrayElementL`))))) (`.Amount_9_F5558B58485D7C03264E5DBF5466952D` (break `/Game/SurvivalGameKitV2/Blueprints/Other/Structs/S_CookingSlot` (`local.ProcessingElementL`))))
            ;[1 1 1] Check if the inv item is valid, if it is and switched on unpause client cooking slots
            (if (`/Game/SurvivalGameKitV2/Blueprints/Other/Interfaces/BP_SGKFunctions.SGK InvSlotAmount` (`local.ArrayElementL`))
              (if (`self.SwitchedOn`)
                (`self.ResumeAllPlayerCookingSlots`))
              (elif (`self.SwitchedOn`)
                (bind (_returnvalue_2 _contentsslots) (`self.GetContentsSlots`))
                (if _returnvalue_2
                  (for _array_element_2 _contentsslots
                    (bind _output_get (set `local.ContentsElementL` _array_element_2))
                    (if (`/Game/SurvivalGameKitV2/Blueprints/Other/Interfaces/BP_SGKFunctions.SGK InvSlotAmount` _output_get)
                      (bind (_mutationsprogress _hasmutationprogress) (`/Game/SurvivalGameKitV2/Blueprints/Other/Interfaces/BP_SGKFunctions.TBS MutationProgress` (`.Item_10_95D912F14C7740665FD844AF7EA87327` (break `/Game/SurvivalGameKitV2/Blueprints/Other/Structs/S_InvSlot` _output_get))))
                      (if _hasmutationprogress
                        (`self.MoveCookingItem` (`local.ContentsElementL`) (`local.ArrayElementL`))
                        (bind (_returnvalue_3 _cookingslot) (`self.SetNewCookingItem` (`|GetArrayItem` (`self.Inventory`) (`.RootIndex_4_31C49987405FF01267287D9E3381FC5E` (break `/Game/SurvivalGameKitV2/Blueprints/Other/Structs/S_InvSlot` (`local.ArrayElementL`))))))
                        (if (`self.SwitchedOn`)
                          (`self.StartPlayerCookingSlot` _cookingslot)
                          (break)
                          (else
                            (break)))))))))
            (else
              ;[1 1 1] If not update the processing slot item amount and if switched on upause clients cooking slots
              (`KismetArrayLibrary.Array_Set` (`self.CookingSlots`) _index (make `/Game/SurvivalGameKitV2/Blueprints/Other/Structs/S_CookingSlot` _itemid _time (`.Amount_5_62DB2267439500D86A52E0B2266494D2` (break `/Game/SurvivalGameKitV2/Blueprints/Other/Structs/S_InvItem` (`.Item_10_95D912F14C7740665FD844AF7EA87327` (break `/Game/SurvivalGameKitV2/Blueprints/Other/Structs/S_InvSlot` (`local.ArrayElementL`))))) _index) true)
              (if (`self.SwitchedOn`)
                (`self.ResumeAllPlayerCookingSlots`))))
          (else
            ;[1 1 1] Check item is valid
            (if (`/Game/SurvivalGameKitV2/Blueprints/Other/Interfaces/BP_SGKFunctions.SGK InvSlotAmount` (`local.ArrayElementL`))
              ;[1 1 1] Create new processing Item listing
              (bind (_returnvalue_4 _cookingslot_2) (`self.SetNewCookingItem` (`local.ArrayElementL`)))
              (if _returnvalue_4
                ;[1 1 1] If switched on start processing timer for clients
                (if (`self.SwitchedOn`)
                  (`self.StartPlayerCookingSlot` _cookingslot_2))
                (else
                  ;[1 1 1] If item is not valid clear the processing item and reset the timer for clients processing slots
                  (bind _cookingslot_3 (`self.ClearCookingItem` (`local.ArrayElementL`) :!label _label))
                  (`self.RestartPlayerCookingSlot` _cookingslot_3)))
              (else
                (goto _label)))))))))

(fn `UpdateCookingTimes`
  (locals (ProcessingItemL :type "/Game/SurvivalGameKitV2/Blueprints/Other/Structs/S_ProcessingItem Structure") (ArrayElementL :type "/Game/SurvivalGameKitV2/Blueprints/Other/Structs/S_CookingSlot Structure") (IndexL :type Integer))
  (bind _arrayelementl (`local.ArrayElementL`))
  (bind (_itemid _time _amount _index) (break `/Game/SurvivalGameKitV2/Blueprints/Other/Structs/S_CookingSlot` _arrayelementl))
  (bind (_itemid_2 _time_2 _amount_2 _index_2) (break `/Game/SurvivalGameKitV2/Blueprints/Other/Structs/S_CookingSlot` (`local.ArrayElementL`)))
  (bind (_itemid_3 _time_3 _amount_3 _index_3) (break `/Game/SurvivalGameKitV2/Blueprints/Other/Structs/S_CookingSlot` (`local.ArrayElementL`)))
  (bind ((`ItemID_12_BF71A7764CB5AA9C7414C8B6682828FC` _itemid_4) (`Amount_9_F5558B58485D7C03264E5DBF5466952D` _amount_4) (`Index_11_89DC537F4D6E4AA1FC506594A5C7EF2F` _index_4)) (break `/Game/SurvivalGameKitV2/Blueprints/Other/Structs/S_CookingSlot` (`local.ArrayElementL`)))
  (if (`self.SwitchedOn`)
    ;[1 1 1] Check if switched on, if is loop though processing slots that have valid item
    (for _array_element (`self.CookingSlots`)
      (bind _output_get (set `local.ArrayElementL` _array_element))
      (bind (_itemid_5 _time_4 _amount_5 _index_5) (break `/Game/SurvivalGameKitV2/Blueprints/Other/Structs/S_CookingSlot` _output_get))
      (set `local.IndexL` _index_5)
      (if (> _amount_5 0)
        (bind (_return_value _processing_item) (`/Game/SurvivalGameKitV2/Blueprints/Other/Interfaces/BP_SGKFunctions.TBS ProcessingItem` (make `/Game/SurvivalGameKitV2/Blueprints/Other/Structs/S_InvItem` (`.ItemID_12_BF71A7764CB5AA9C7414C8B6682828FC` (break `/Game/SurvivalGameKitV2/Blueprints/Other/Structs/S_CookingSlot` (`local.ArrayElementL`))))))
        (set `local.ProcessingItemL` _processing_item)
        ;[1 1 1] Check the item has the amount required to process
        (if (>= (`.Amount_9_F5558B58485D7C03264E5DBF5466952D` (break `/Game/SurvivalGameKitV2/Blueprints/Other/Structs/S_CookingSlot` (`local.ArrayElementL`))) (`.StartingItemAmount_12_945D5CDB4CBCF079928C0FB2952280A9` (break `/Game/SurvivalGameKitV2/Blueprints/Other/Structs/S_ProcessingItem` (`local.ProcessingItemL`))))
          (if (`KismetArrayLibrary.Array_Contains` (`self.PausedIndexs`) (`local.IndexL`))
            (`self.Pause/UnPauseSingleSlot` (`local.IndexL`))
            (`KismetArrayLibrary.Array_Remove` (`self.PausedIndexs`) (`local.IndexL`)))
          ;[1 1 1] Check if item has finished processing
          (if (> (- (`.Time_6_51E1F19A4EC9904979CC80B79F2EEE7B` (break `/Game/SurvivalGameKitV2/Blueprints/Other/Structs/S_CookingSlot` (`local.ArrayElementL`))) 0.05) 0.0)
            ;[1 1 1] If not remove time from time value ready for next check
            (bind _structout (setmembers `/Game/SurvivalGameKitV2/Blueprints/Other/Structs/S_CookingSlot` :`StructRef` _arrayelementl :`Time` (- _time 0.05)))
            (`KismetArrayLibrary.Array_Set` (`self.CookingSlots`) _index _structout true)
            (else
              ;[1 1 1] Check if item is empty after remove 1 count
              (if (> (- (`.Amount_9_F5558B58485D7C03264E5DBF5466952D` (break `/Game/SurvivalGameKitV2/Blueprints/Other/Structs/S_CookingSlot` (`local.ArrayElementL`))) (`.StartingItemAmount_12_945D5CDB4CBCF079928C0FB2952280A9` (break `/Game/SurvivalGameKitV2/Blueprints/Other/Structs/S_ProcessingItem` (`local.ProcessingItemL`)))) 0)
                ;[1 1 1] If item amount remaining reset the time to full processing time
                (bind (_return_value_2 _processing_item_2) (`/Game/SurvivalGameKitV2/Blueprints/Other/Interfaces/BP_SGKFunctions.TBS ProcessingItem` (make `/Game/SurvivalGameKitV2/Blueprints/Other/Structs/S_InvItem` _itemid_4)))
                (bind _structout_2 (setmembers `/Game/SurvivalGameKitV2/Blueprints/Other/Structs/S_CookingSlot` :`StructRef` (`local.ArrayElementL`) :`Time` (`.ProcessingTime_13_1A30D84540A47981B8B1989067493A64` (break `/Game/SurvivalGameKitV2/Blueprints/Other/Structs/S_ProcessingItem` _processing_item_2)) :`Amount` (- _amount_4 (`.StartingItemAmount_12_945D5CDB4CBCF079928C0FB2952280A9` (break `/Game/SurvivalGameKitV2/Blueprints/Other/Structs/S_ProcessingItem` (`local.ProcessingItemL`))))))
                (`KismetArrayLibrary.Array_Set` (`self.CookingSlots`) _index_4 _structout_2 true)
                ;[1 1 1] Remove the item cost of processing the item and remove its weight
                (bind (_return_value_3 _processing_item_3) (`/Game/SurvivalGameKitV2/Blueprints/Other/Interfaces/BP_SGKFunctions.TBS ProcessingItem` (make `/Game/SurvivalGameKitV2/Blueprints/Other/Structs/S_InvItem` (`.ItemID_12_BF71A7764CB5AA9C7414C8B6682828FC` (break `/Game/SurvivalGameKitV2/Blueprints/Other/Structs/S_CookingSlot` (`local.ArrayElementL`))))))
                (bind (_startingitem _startingitemamount) (break `/Game/SurvivalGameKitV2/Blueprints/Other/Structs/S_ProcessingItem` _processing_item_3))
                (`self.SetItemAmount` (`|GetArrayItem` (`self.Inventory`) (`.Index_11_89DC537F4D6E4AA1FC506594A5C7EF2F` (break `/Game/SurvivalGameKitV2/Blueprints/Other/Structs/S_CookingSlot` (`local.ArrayElementL`)))) (- (`.Amount_5_62DB2267439500D86A52E0B2266494D2` (break `/Game/SurvivalGameKitV2/Blueprints/Other/Structs/S_InvItem` (`.Item_10_95D912F14C7740665FD844AF7EA87327` (break `/Game/SurvivalGameKitV2/Blueprints/Other/Structs/S_InvSlot` (`|GetArrayItem` (`self.Inventory`) (`.Index_11_89DC537F4D6E4AA1FC506594A5C7EF2F` (break `/Game/SurvivalGameKitV2/Blueprints/Other/Structs/S_CookingSlot` (`local.ArrayElementL`)))))))) _startingitemamount) true true)
                (`self.RemoveItemWeight` (`.Item_10_95D912F14C7740665FD844AF7EA87327` (break `/Game/SurvivalGameKitV2/Blueprints/Other/Structs/S_InvSlot` (`|GetArrayItem` (`self.Inventory`) (`.Index_11_89DC537F4D6E4AA1FC506594A5C7EF2F` (break `/Game/SurvivalGameKitV2/Blueprints/Other/Structs/S_CookingSlot` (`local.ArrayElementL`)))))) _startingitemamount)
                ;[1 1 1] Restart processing timer for clients
                (bind (_return_value_4 _processing_item_4) (`/Game/SurvivalGameKitV2/Blueprints/Other/Interfaces/BP_SGKFunctions.TBS ProcessingItem` (make `/Game/SurvivalGameKitV2/Blueprints/Other/Structs/S_InvItem` _itemid_2)))
                (`self.StartPlayerCookingSlot` (make `/Game/SurvivalGameKitV2/Blueprints/Other/Structs/S_CookingSlot` _itemid_2 (`.ProcessingTime_13_1A30D84540A47981B8B1989067493A64` (break `/Game/SurvivalGameKitV2/Blueprints/Other/Structs/S_ProcessingItem` _processing_item_4)) (- _amount_2 (`.StartingItemAmount_12_945D5CDB4CBCF079928C0FB2952280A9` (break `/Game/SurvivalGameKitV2/Blueprints/Other/Structs/S_ProcessingItem` (`local.ProcessingItemL`)))) _index_2))
                ;[1 1 1] Add processing item
                (`self.AddReturnedItems` (`local.ArrayElementL`))
                (else
                  ;[1 1 1] Clean the processing slot
                  (`KismetArrayLibrary.Array_Set` (`self.CookingSlots`) _index_3 (make `/Game/SurvivalGameKitV2/Blueprints/Other/Structs/S_CookingSlot` "None" 0.0 0 _index_3) true)
                  ;[1 1 1] Remove processing item, weight and item count then restart processing slot timer
                  (`self.RemoveItem` (`|GetArrayItem` (`self.Inventory`) (`.Index_11_89DC537F4D6E4AA1FC506594A5C7EF2F` (break `/Game/SurvivalGameKitV2/Blueprints/Other/Structs/S_CookingSlot` (`local.ArrayElementL`)))) true true true)
                  (`self.RestartPlayerCookingSlot` (`local.ArrayElementL`))
                  ;[1 1 1] Add processed item
                  (`self.AddReturnedItems` (`local.ArrayElementL`))))))
          (elif (not (`KismetArrayLibrary.Array_Contains` (`self.PausedIndexs`) (`local.IndexL`)))
            (`self.Pause/UnPauseSingleSlot` (`local.IndexL`) true)
            (`KismetArrayLibrary.Array_Add` (`self.PausedIndexs`) (`local.IndexL`))))))))