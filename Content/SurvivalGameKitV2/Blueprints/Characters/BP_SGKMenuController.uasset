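; BP_SGKMenuController is the player controller for the Survival Game Kit V2 main menu.
; On BeginPlay, for the local controller only, it creates a widget from MenuWidget owned by player controller 0, stores it as MainMenuWidget and adds it to the viewport.
; It then shows the mouse cursor and switches to UI-only input, focused on the menu without locking the mouse.
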(fn `UserConstructionScript`)