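; BP_IconMaker is an editor utility actor for baking item icon textures from a static or skeletal mesh lit by its own lights and framed by a scene capture.
; Reset restores default transforms for the meshes, lights and capture camera, along with the directional light intensity.
; BaketoRenderTexture clears a render target, draws an icon material into it, then saves it as a named static texture without mipmaps in the UI LOD group.
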(event `Reset`
  (`SceneComponent.ResetRelativeTransform` (`self.StaticMesh`))
  (`SceneComponent.ResetRelativeTransform` (`self.SkeletalMesh`))
  (`SceneComponent.K2_SetRelativeTransform` (`self.DirectionalLight`) (`KismetMathLibrary.MakeTransform` (0.0 0.0 100.0)) false false)
  (`SceneComponent.K2_SetRelativeTransform` (`self.SkyLight`) (`KismetMathLibrary.MakeTransform` (0.0 0.0 50.0)) false false)
  (`SceneComponent.K2_SetRelativeTransform` (`self.SceneCaptureComponent2D`) (`KismetMathLibrary.MakeTransform` (-30.0 0.0 0.0)) false false)
  (`LightComponent.SetIntensity` (`self.DirectionalLight`) 5.0))

(event `Bake to Render Texture`
  (`KismetRenderingLibrary.ClearRenderTarget2D` (`self.RenderTextureSample`))
  (`KismetRenderingLibrary.DrawMaterialToRenderTarget` (`self.RenderTextureSample`) "/Game/SurvivalGameKitV2/Materials/M_RenderIconTexture.M_RenderIconTexture")
  (bind _returnvalue (`KismetRenderingLibrary.RenderTargetCreateStaticTexture2DEditorOnly` (`self.RenderTextureSample`) (`self.TextureName`) "TC_Default" "TMGS_NoMipmaps"))
  (set `Texture.LODGroup` "TEXTUREGROUP_UI" _returnvalue))

(fn `UserConstructionScript`)