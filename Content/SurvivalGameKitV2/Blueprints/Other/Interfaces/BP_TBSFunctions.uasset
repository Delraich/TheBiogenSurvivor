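; Static helper library for the survival kit's mutation and item-processing systems, built on data table lookups.
; Item queries scan the unlock and processing tables by item ID to return mutation progress or a processing recipe.
; AddMutationStats folds mutation rows into one combined stat delta, using helpers that sum reductions and movement speeds by key.
; GetMutationsProgress converts raw progress into capped ratios for three unlock tiers; ItemMutationProgress is an empty stub.
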(fn `TBS Add Movement Speeds`
  (params (InMoveSpeeds1 :type "Map of /Game/SurvivalGameKitV2/Blueprints/Other/Enum/E_CharacterState Enum to Float (double-precision)") (InMoveSpeeds2 :type "Map of /Game/SurvivalGameKitV2/Blueprints/Other/Enum/E_CharacterState Enum to Float (double-precision)") (__WorldContext :type "Object Object Reference"))
  (returns (OutMoveSpeed :type "Map of /Game/SurvivalGameKitV2/Blueprints/Other/Enum/E_CharacterState Enum to Float (double-precision)"))
  (locals (MoveSpeedL :type "Map of /Game/SurvivalGameKitV2/Blueprints/Other/Enum/E_CharacterState Enum to Float (double-precision)"))
  (bind _movespeedl (`local.MoveSpeedL`))
  (bind _keys (`BlueprintMapLibrary.Map_Keys` InMoveSpeeds1))
  (for _array_element _keys
    (`BlueprintMapLibrary.Map_Add` (`local.MoveSpeedL`) _array_element (`BlueprintMapLibrary.Map_Find` (`local.InMoveSpeeds1`) _array_element)))
  (bind _keys_2 (`BlueprintMapLibrary.Map_Keys` InMoveSpeeds2))
  (for _array_element_2 _keys_2
    (bind (_value _returnvalue) (`BlueprintMapLibrary.Map_Find` (`local.MoveSpeedL`) _array_element_2))
    (if _returnvalue
      (bind _value_2 (`BlueprintMapLibrary.Map_Find` (`local.InMoveSpeeds2`) _array_element_2))
      (`BlueprintMapLibrary.Map_Add` _movespeedl _array_element_2 (+ _value _value_2))
      (else
        (`BlueprintMapLibrary.Map_Add` _movespeedl _array_element_2 _value_2))))
  (return (`local.MoveSpeedL`)))

(fn `TBS Add Stat Reductions`
  (params (InReductions1 :type "Array of /Game/SurvivalGameKitV2/Blueprints/Other/Structs/S_StatReduction Structure") (InReductions2 :type "Array of /Game/SurvivalGameKitV2/Blueprints/Other/Structs/S_StatReduction Structure") (__WorldContext :type "Object Object Reference"))
  (returns (OutStatReduction :type "Array of /Game/SurvivalGameKitV2/Blueprints/Other/Structs/S_StatReduction Structure"))
  (locals (ReductionL :type "Array of /Game/SurvivalGameKitV2/Blueprints/Other/Structs/S_StatReduction Structure") (ItemAdded :type Boolean) (ReductionMapL :type "Map of /Game/SurvivalGameKitV2/Blueprints/Other/Enum/E_CharacterState Enum to Float (double-precision)"))
  (for _array_element InReductions1
    (bind (_characterstate _amount) (break `/Game/SurvivalGameKitV2/Blueprints/Other/Structs/S_StatReduction` _array_element))
    (`BlueprintMapLibrary.Map_Add` (`local.ReductionMapL`) _characterstate _amount))
  (for _array_element_2 InReductions2
    (bind (_characterstate_2 _amount_2) (break `/Game/SurvivalGameKitV2/Blueprints/Other/Structs/S_StatReduction` _array_element_2))
    (bind (_value _returnvalue) (`BlueprintMapLibrary.Map_Find` (`local.ReductionMapL`) _characterstate_2))
    (if _returnvalue
      (`BlueprintMapLibrary.Map_Add` (`local.ReductionMapL`) _characterstate_2 (+ _value _amount_2))
      (else
        (`BlueprintMapLibrary.Map_Add` (`local.ReductionMapL`) _characterstate_2 _amount_2))))
  (bind _keys (`BlueprintMapLibrary.Map_Keys` (`local.ReductionMapL`)))
  (for _array_element_3 _keys
    (`KismetArrayLibrary.Array_Add` (`local.ReductionL`) (make `/Game/SurvivalGameKitV2/Blueprints/Other/Structs/S_StatReduction` _array_element_3 (`BlueprintMapLibrary.Map_Find` (`local.ReductionMapL`) _array_element_3))))
  (return (`local.ReductionL`)))

(fn `TBS AddMutationStats`
  (params (InMutations :type "Array of DataTableRowHandle Structure") (__WorldContext :type "Object Object Reference"))
  (returns (OutMutationDetails :type "/Game/SurvivalGameKitV2/Blueprints/Other/Structs/S_MutationDetails Structure"))
  (locals (MutationDetailsL :type "/Game/SurvivalGameKitV2/Blueprints/Other/Structs/S_MutationDetails Structure"))
  (bind (_mutationdetailsl_name _mutationdetailsl_shortname _mutationdetailsl_description _mutationdetailsl_type _mutationdetailsl_mutationicon _mutationdetailsl_maxhungerdelta _mutationdetailsl_hungerreductiondelta _mutationdetailsl_hungerreductiontimedelta _mutationdetailsl_maxthirstdelta _mutationdetailsl_thirstreductiondelta _mutationdetailsl_thirstreductiontimedelta _mutationdetailsl_maxhealthdelta _mutationdetailsl_maxstaminadelta _mutationdetailsl_staminarechargedelta _mutationdetailsl_movementspeeddelta _mutationdetailsl_usehealthregen _mutationdetailsl_healthregenamount _mutationdetailsl_healthregenminhunger _mutationdetailsl_healthregenminthirst _mutationdetailsl_healthregenticktime _mutationdetailsl_falldamagedelta) (break `/Game/SurvivalGameKitV2/Blueprints/Other/Structs/S_MutationDetails` (`local.MutationDetailsL`)))
  (for _array_element InMutations
    (bind _returnvalue (`|GetDataTableRow` "/Game/SurvivalGameKitV2/Blueprints/Mutations/MutationList.MutationList" (`.RowName` (break `DataTableRowHandle` _array_element)))
      (:`then`
        (bind (_name _shortname _description _type _mutationicon _maxhungerdelta _hungerreductiondelta _hungerreductiontimedelta _maxthirstdelta _thirstreductiondelta _thirstreductiontimedelta _maxhealthdelta _maxstaminadelta _staminarechargedelta _movementspeeddelta _usehealthregen _healthregenamount _healthregenminhunger _healthregenminthirst _healthregenticktime _falldamagedelta) (break `/Game/SurvivalGameKitV2/Blueprints/Other/Structs/S_MutationDetails` _returnvalue))
        (bind _outstatreduction (`self.TBS Add Stat Reductions` _hungerreductiondelta _mutationdetailsl_hungerreductiondelta))
        (bind _outstatreduction_2 (`self.TBS Add Stat Reductions` _thirstreductiondelta _mutationdetailsl_thirstreductiondelta))
        (bind _outmovespeed (`self.TBS Add Movement Speeds` _movementspeeddelta _mutationdetailsl_movementspeeddelta))
        (set `local.MutationDetailsL` (make `/Game/SurvivalGameKitV2/Blueprints/Other/Structs/S_MutationDetails` "" "" "" "NewEnumerator0" null (+ _maxhungerdelta _mutationdetailsl_maxhungerdelta) _outstatreduction (+ _hungerreductiontimedelta _mutationdetailsl_hungerreductiontimedelta) (+ _maxthirstdelta _mutationdetailsl_maxthirstdelta) _outstatreduction_2 (+ _thirstreductiontimedelta _mutationdetailsl_thirstreductiontimedelta) (+ _maxhealthdelta _mutationdetailsl_maxhealthdelta) (+ _maxstaminadelta _mutationdetailsl_maxstaminadelta) (+ _staminarechargedelta _mutationdetailsl_staminarechargedelta) _outmovespeed (or _usehealthregen _mutationdetailsl_usehealthregen) (+ _healthregenamount _mutationdetailsl_healthregenamount) (+ _healthregenminhunger _mutationdetailsl_healthregenminhunger) (+ _healthregenminthirst _mutationdetailsl_healthregenminthirst) (+ _healthregenticktime _mutationdetailsl_healthregenticktime) (+ _falldamagedelta _mutationdetailsl_falldamagedelta))))
      (:`RowNotFound`
        (`KismetSystemLibrary.PrintString` null "Row not found"))))
  (return (`local.MutationDetailsL`)))

(fn `TBS AddStaminaRecharge`
  (params (StaminaRechargeStates :type "Map of /Game/SurvivalGameKitV2/Blueprints/Other/Enum/E_CharacterState Enum to Float (double-precision)") (RechargeDelta :type "Float (double-precision)") (__WorldContext :type "Object Object Reference"))
  (returns (OutRechargeStates :type "Map of /Game/SurvivalGameKitV2/Blueprints/Other/Enum/E_CharacterState Enum to Float (double-precision)"))
  (locals (RechargeStatesL :type "Map of /Game/SurvivalGameKitV2/Blueprints/Other/Enum/E_CharacterState Enum to Float (double-precision)"))
  (bind _keys (`BlueprintMapLibrary.Map_Keys` StaminaRechargeStates))
  (for _array_element _keys
    (`BlueprintMapLibrary.Map_Add` (`local.RechargeStatesL`) _array_element (+ (`BlueprintMapLibrary.Map_Find` (`local.StaminaRechargeStates`) _array_element) (`local.RechargeDelta`))))
  (return (`local.RechargeStatesL`)))

(fn `TBS GetMutationsProgress`
  (params (MutationProgress :type "Map of Name to Float (double-precision)"))
  (returns (Mutations :type "Map of Name to Float (double-precision)"))
  (locals (MutationsL :type "Map of Name to Float (double-precision)") (RowNameL :type Name) (ProgressL :type "Float (double-precision)"))
  (bind (_value _returnvalue) (`BlueprintMapLibrary.Map_Find` (`local.MutationProgress`) (`local.RowNameL`)))
  (bind _keys (`BlueprintMapLibrary.Map_Keys` MutationProgress))
  (for _array_element _keys
    (set `local.RowNameL` _array_element)
    (if _returnvalue
      (set `local.ProgressL` _value)
      (bind _returnvalue_2 (`|GetDataTableRow` "/Game/SurvivalGameKitV2/Blueprints/Mutations/MutationUnlockList.MutationUnlockList" (`local.RowNameL`))
        (:`then`
          (bind (_progressitems _requiredt1 _unlockt1 _requiredt2 _unlockt2 _requiredt3 _unlockt3) (break `/Game/SurvivalGameKitV2/Blueprints/Other/Structs/S_MutationUnlockDetails` _returnvalue_2))
          (if (>= (`local.ProgressL`) _requiredt1)
            (bind (_datatable _rowname) (break `DataTableRowHandle` _unlockt1))
            (`BlueprintMapLibrary.Map_Add` (`local.MutationsL`) _rowname 1.0)
            (else
              (`BlueprintMapLibrary.Map_Add` (`local.MutationsL`) _rowname (/ (`local.ProgressL`) _requiredt1))))
          (if (>= (`local.ProgressL`) _requiredt2)
            (bind (_datatable_2 _rowname_2) (break `DataTableRowHandle` _unlockt2))
            (`BlueprintMapLibrary.Map_Add` (`local.MutationsL`) _rowname_2 1.0)
            (else
              (`BlueprintMapLibrary.Map_Add` (`local.MutationsL`) _rowname_2 (/ (`local.ProgressL`) _requiredt2))))
          (if (>= (`local.ProgressL`) _requiredt3)
            (bind (_datatable_3 _rowname_3) (break `DataTableRowHandle` _unlockt3))
            (`BlueprintMapLibrary.Map_Add` (`local.MutationsL`) _rowname_3 1.0)
            (else
              (`BlueprintMapLibrary.Map_Add` (`local.MutationsL`) _rowname_3 (/ (`local.ProgressL`) _requiredt3))))))))
  (return (`local.MutationsL`)))

(fn `TBS ItemMutationProgress`
  (params (__WorldContext :type "Object Object Reference")))

(fn `TBS MutationProgress`
  (params (Item :type "/Game/SurvivalGameKitV2/Blueprints/Other/Structs/S_InvItem Structure") (__WorldContext :type "Object Object Reference"))
  (returns (MutationsProgress :type "Array of /Game/SurvivalGameKitV2/Blueprints/Other/Structs/S_MutationProgress Structure") (HasMutationProgress :type Boolean))
  (locals (output :type "Array of /Game/SurvivalGameKitV2/Blueprints/Other/Structs/S_MutationProgress Structure"))
  (bind _output (`local.output`))
  (bind _outrownames (`DataTableFunctionLibrary.GetDataTableRowNames` "/Game/SurvivalGameKitV2/Blueprints/Mutations/MutationUnlockList.MutationUnlockList"))
  (for _array_element _outrownames
    (bind _returnvalue (`|GetDataTableRow` "/Game/SurvivalGameKitV2/Blueprints/Mutations/MutationUnlockList.MutationUnlockList" _array_element)
      (:`then`
        (for _array_element_2 (`.ProgressItems_24_D38824A64524A8B4C6ADBEA4C0254894` (break `/Game/SurvivalGameKitV2/Blueprints/Other/Structs/S_MutationUnlockDetails` _returnvalue))
          (bind (_item _progressvalue) (break `/Game/SurvivalGameKitV2/Blueprints/Other/Structs/S_MutationUnlockItemDetails` _array_element_2))
          (if (== (`.RowName` (break `DataTableRowHandle` _item)) (`.ID_2_84C2CB8945979246059C568DCD463423` (break `/Game/SurvivalGameKitV2/Blueprints/Other/Structs/S_InvItem` (`local.Item`))))
            (`KismetArrayLibrary.Array_Add` (`local.output`) (make `/Game/SurvivalGameKitV2/Blueprints/Other/Structs/S_MutationProgress` _array_element _progressvalue)))))))
  (return _output (> (`KismetArrayLibrary.Array_Length` _output) 0)))

(fn `TBS ProcessingItem`
  (params (Item :type "/Game/SurvivalGameKitV2/Blueprints/Other/Structs/S_InvItem Structure") (__WorldContext :type "Object Object Reference"))
  (returns (`Return Value` :type Boolean) (`Processing Item` :type "/Game/SurvivalGameKitV2/Blueprints/Other/Structs/S_ProcessingItem Structure"))
  (locals (`Processing Item L` :type "/Game/SurvivalGameKitV2/Blueprints/Other/Structs/S_ProcessingItem Structure"))
  (bind _outrownames (`DataTableFunctionLibrary.GetDataTableRowNames` "/Game/SurvivalGameKitV2/Blueprints/Mutations/ProcessingItemList.ProcessingItemList"))
  (for _array_element _outrownames
    (bind _returnvalue (`|GetDataTableRow` "/Game/SurvivalGameKitV2/Blueprints/Mutations/ProcessingItemList.ProcessingItemList" _array_element)
      (:`then`
        (set `local.Processing Item L` _returnvalue)
        (if (== (`.RowName` (break `DataTableRowHandle` (`.StartingItem_11_1581F7DB44E1EE628672AC9EBC5289E6` (break `/Game/SurvivalGameKitV2/Blueprints/Other/Structs/S_ProcessingItem` _returnvalue)))) (`.ID_2_84C2CB8945979246059C568DCD463423` (break `/Game/SurvivalGameKitV2/Blueprints/Other/Structs/S_InvItem` (`local.Item`))))
          (return true (`local.Processing Item L`)))))))