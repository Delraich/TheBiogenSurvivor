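; Blueprint interface for the Survival Game Kit game instance, exposing save, menu and settings state to other Blueprints without a direct cast.
; It declares getters and setters for the save slot name, the load-save flag, the menu-opened-level flag and mouse sensitivity.
; It also declares calls to save settings and options and to set sound volume, with all behavior left to the implementer.
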(fn `SGK GetLoadSaveGame`
  (returns (LoadSaveGame :type Boolean))
  (return false))

(fn `SGK GetMenuOpenedLevel`
  (returns (MenuOpenedLevel :type Boolean))
  (return false))

(fn `SGK GetMouseSense`
  (returns (MouseSense :type "Float (double-precision)"))
  (return 0.0))

(fn `SGK GetSaveGameSlotName`
  (returns (SaveGameSlotName :type String))
  (return ""))

(fn `SGK Options Save`
  (returns (Settings :type "/Game/SurvivalGameKitV2/Blueprints/Saving/BP_SGKSettingsSaveData Object Reference"))
  (return null))

(fn `SGK SaveSettings`)

(fn `SGK SetLoadSaveGame`
  (params (LoadSaveGame :type Boolean)))

(fn `SGK SetMenuOpenedLevel`
  (params (MenuOpenedLevel :type Boolean))
  (return))

(fn `SGK SetMouseSense`
  (params (MouseSense :type "Float (double-precision)")))

(fn `SGK SetSaveGameSlotName`
  (params (SaveGameSlotName :type String)))

(fn `SGK SetVolume`
  (params (Sound :type "/Game/SurvivalGameKitV2/Blueprints/Other/Enum/E_SoundVolumes Enum" :default "NewEnumerator0") (Volume :type "Float (double-precision)")))