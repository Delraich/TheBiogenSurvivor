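; BP_WaterCan is a holdable item that waters farm plots through its primary action.
; On key press, the server event casts the player inventory's client interaction hit actor to BP_MasterFarmBuildPart, stopping if the cast fails.
; It then calls SRVAddWater on the owner's CFarmingSystem component with a fixed amount.
; Finally, it sends the client a "Watered" notification naming the plot via its interact name message.
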(event `/Game/SurvivalGameKitV2/Blueprints/Other/Interfaces/BP_SGKHoldableInterface.SGK ServerPrimaryAction`
  (params (KeyDown :type Boolean))
  (bind (_bblockinghit _binitialoverlap _time _distance _location _impactpoint _normal _impactnormal _physmat _hitactor) (`GameplayStatics.BreakHitResult` (`/Game/SurvivalGameKitV2/Blueprints/Components/BP_PlayerInventory.ClientInteractHitResult` (`self.PlayerInventory`))))
  (if KeyDown
    (bind _asbp_master_farm_build_part (cast `/Game/TheBiogenSurvivor/Blueprints/BuildParts/BP_MasterFarmBuildPart` _hitactor))
    (`/Game/FarmingSystem/Blueprints/C-FarmingSystem.SRV_AddWater` (`self.GetComponentByClass` (`ActorComponent.GetOwner` (`self.PlayerInventory`)) "/Game/FarmingSystem/Blueprints/C-FarmingSystem.C-FarmingSystem_C") _asbp_master_farm_build_part 10.0)
    (bind _interactname (message `/Game/SurvivalGameKitV2/Blueprints/Other/Interfaces/BP_SGKInteractionInterface.SGK InteractName` _hitactor))
    (`/Game/SurvivalGameKitV2/Blueprints/Components/BP_PlayerInventory.ClientCreateNotification` (`self.PlayerInventory`) (make `/Game/SurvivalGameKitV2/Blueprints/Other/Structs/S_NotificationDetails` (`|FormatText` "Watered {plot}" _interactname) (struct :`R` 1.0 :`G` 1.0 :`B` 1.0 :`A` 1.0) "/Game/SurvivalGameKitV2/Textures/UI/T_Info_UI.T_Info_UI"))))

(fn `UserConstructionScript`
  (`parent.UserConstructionScript`))