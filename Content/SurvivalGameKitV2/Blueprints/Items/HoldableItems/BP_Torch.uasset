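; BP_Torch is a holdable torch item in the Survival Game Kit that wears out over time.
; Each tick, after the parent logic, it tells the player inventory to lower the held item's durability by DurabilityCostPerUse scaled by delta time, so that value acts as a per-second drain.
; It overrides the holdable mesh function to return its static mesh component.
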(event `self.ReceiveTick`
  (params (DeltaSeconds :type "Float (single-precision)"))
  (`parent.ReceiveTick` DeltaSeconds)
  (`/Game/SurvivalGameKitV2/Components/BP_PlayerInventory.DecreaseHeldItemDurability` (`self.PlayerInventory`) (* DeltaSeconds (`self.DurabilityCostPerUse`))))

(fn `SGK HoldableMesh`
  (returns (Mesh :type "PrimitiveComponent Object Reference"))
  (`parent.SGK HoldableMesh`)
  (return (`self.StaticMesh`)))

(fn `UserConstructionScript`
  (`parent.UserConstructionScript`))