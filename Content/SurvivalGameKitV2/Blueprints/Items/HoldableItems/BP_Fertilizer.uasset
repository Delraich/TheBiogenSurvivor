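; BP_Fertilizer is a holdable item that fertilizes farm build parts.
; On primary-action press, it casts the player's interact hit actor to BP_MasterFarmBuildPart and compares its current fertilizer to the maximum.
; If below max, it adds a fixed amount through the owner's CFarmingSystem component and removes one item from the held slot.
; Otherwise, it shows a notification that the plant does not need fertilizer.
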(event `/Game/SurvivalGameKitV2/Blueprints/Other/Interfaces/BP_SGKHoldableInterface.SGK ServerPrimaryAction`
  (params (KeyDown :type Boolean))
  (bind _holdinginvslot (`/Game/SurvivalGameKitV2/Blueprints/Components/BP_PlayerInventory.HoldingInvSlot` (`self.PlayerInventory`)))
  (if KeyDown
    (bind _asbp_master_farm_build_part (cast `/Game/TheBiogenSurvivor/Blueprints/BuildParts/BP_MasterFarmBuildPart` (`.HitActor` (`GameplayStatics.BreakHitResult` (`/Game/SurvivalGameKitV2/Blueprints/Components/BP_PlayerInventory.ClientInteractHitResult` (`self.PlayerInventory`))))))
    (bind (_seedplanted _finishedgrowing _isgrowing _growthpercent _currentwateramount _currenthealth _currentfertilizer _maxhealth _maxwater _maxfertilizer) (break `/Game/FarmingSystem/Blueprints/Data/Structs/STR_PlantState` (`/Game/TheBiogenSurvivor/Blueprints/BuildParts/BP_MasterFarmBuildPart.PlantState` _asbp_master_farm_build_part)))
    (if (< _currentfertilizer _maxfertilizer)
      (`/Game/FarmingSystem/Blueprints/C-FarmingSystem.SRV_AddFertilizer` (`self.GetComponentByClass` (`ActorComponent.GetOwner` (`self.PlayerInventory`)) "/Game/FarmingSystem/Blueprints/C-FarmingSystem.C-FarmingSystem_C") _asbp_master_farm_build_part 100.0)
      (`/Game/SurvivalGameKitV2/Blueprints/Components/BP_MasterInventory.RemoveItemAmount` (`.Inventory_13_75D853E34C33E03489A41A94465989CA` (break `/Game/SurvivalGameKitV2/Blueprints/Other/Structs/S_InvSlot` _holdinginvslot)) _holdinginvslot 1 false)
      (else
        (`/Game/SurvivalGameKitV2/Blueprints/Components/BP_PlayerInventory.ClientCreateNotification` (`self.PlayerInventory`) (make `/Game/SurvivalGameKitV2/Blueprints/Other/Structs/S_NotificationDetails` (`|FormatText` "Plant does not need fertilizer") (struct :`R` 1.0 :`G` 1.0 :`B` 1.0 :`A` 1.0) "/Game/SurvivalGameKitV2/Textures/UI/T_Info_UI.T_Info_UI"))))))

(fn `SGK HoldableMesh`
  (returns (Mesh :type "PrimitiveComponent Object Reference"))
  (`parent.SGK HoldableMesh`)
  (return (`self.StaticMesh`)))

(fn `UserConstructionScript`
  (`parent.UserConstructionScript`))