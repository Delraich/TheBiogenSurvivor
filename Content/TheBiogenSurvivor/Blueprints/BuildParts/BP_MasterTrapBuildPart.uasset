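; Master animal trap build part with its own inventory, which players open to access contents and set when inactive.
; While set, BaitSphere sends roaming AI toward the trap if its inventory holds bait listed for that animal class in AnimalBaitList.
; On server TrapBox overlap, the trap disarms and clears matching bait; classes matching TrapTriggers also spring the mesh, are destroyed and yield resources into the inventory.
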(event `self.ReceiveBeginPlay`
  (`parent.ReceiveBeginPlay`)
  (`StaticMeshComponent.SetStaticMesh` (`self.StaticMesh`) (`self.StartMesh`)))

(event `self.TrapBox.OnComponentBeginOverlap`
  (params (OverlappedComponent :type "PrimitiveComponent Object Reference") (OtherActor :type "Actor Object Reference") (OtherComp :type "PrimitiveComponent Object Reference") (OtherBodyIndex :type Integer) (bFromSweep :type Boolean) (SweepResult :type "HitResult Structure (by ref)"))
  (bind _returnvalue (`GameplayStatics.GetObjectClass` OtherActor))
  (if (`self.TrapActive`)
    (`/Engine/EditorBlueprintResources/ActorMacros.Switch Has Authority`
      (:`Authority`
        (`StaticMeshComponent.SetStaticMesh` (`self.StaticMesh`) (`self.StartMesh`))
        (set `self.TrapActive` false)
        (`self.ClearAllBaitForAnimal` _returnvalue)
        (for _array_element (`self.TrapTriggers`)
          (bind (_activatetype _returnresources) (break `/Game/TheBiogenSurvivor/Blueprints/Other/Structs/S_TrapCreatureDetails` _array_element))
          (if (== _activatetype _returnvalue)
            (`StaticMeshComponent.SetStaticMesh` (`self.StaticMesh`) (`self.SprungMesh`))
            (`self.K2_DestroyActor` OtherActor)
            ;[1 1 1] Add the resources to the inventory
            (for _array_element_2 _returnresources
              (bind _globalinventory (message `/Game/SurvivalGameKitV2/Blueprints/Other/Interfaces/BP_SGKGameModeInterface.SGK GetGlobalInventory` (`GameplayStatics.GetGameMode`)))
              (bind (_item _amount) (break `/Game/SurvivalGameKitV2/Blueprints/Other/Structs/S_CraftingCost` _array_element_2))
              (bind _newitem (`/Game/SurvivalGameKitV2/Blueprints/Other/BP_GlobalInventoryManager.CreateNewItem` _globalinventory (`.RowName` (break `DataTableRowHandle` _item)) _amount false false false false))
              (`/Game/SurvivalGameKitV2/Components/BP_MasterInventory.AddItem` (`self.BP_MasterInventory`) _newitem true false))))))))

(event `self.BaitSphere.OnComponentBeginOverlap`
  (params (OverlappedComponent :type "PrimitiveComponent Object Reference") (OtherActor :type "Actor Object Reference") (OtherComp :type "PrimitiveComponent Object Reference") (OtherBodyIndex :type Integer) (bFromSweep :type Boolean) (SweepResult :type "HitResult Structure (by ref)"))
  ;[1 1 1] Only activate bait if the animal is roaming
  (bind _asbp_master_aicharacter (cast `/Game/SmartAI/Blueprints/AI/AICharacters/BP_MasterAICharacter` OtherActor))
  (if (`|EnumEquality` (`/Game/SmartAI/Blueprints/AI/Components/BP_SmartAIComponent.AI Current Behaviour` (`self.GetComponentByClass` _asbp_master_aicharacter "/Game/SmartAI/Blueprints/AI/Components/BP_SmartAIComponent.BP_SmartAIComponent_C")) "NewEnumerator15")
    (if (`self.TrapActive`)
      (bind _returnvalue (`|GetDataTableRow` "/Game/TheBiogenSurvivor/Blueprints/Animals/AnimalBaitList.AnimalBaitList" (`KismetStringLibrary.Conv_StringToName` (`KismetSystemLibrary.GetClassDisplayName` (`GameplayStatics.GetObjectClass` OtherActor))))
        (:`then`
          (for _array_element (`.BaitItems_11_0A09AD6C4CAD952B2D41B2919D5D19C7` (break `/Game/TheBiogenSurvivor/Blueprints/Other/Structs/S_AnimalBait` _returnvalue)) :!label _label
            (bind _rootslots (`/Game/SurvivalGameKitV2/Components/BP_MasterInventory.AllItems` (`self.BP_MasterInventory`)))
            (for _array_element_2 _rootslots
              (if (== (`.ID_2_84C2CB8945979246059C568DCD463423` (break `/Game/SurvivalGameKitV2/Blueprints/Other/Structs/S_InvItem` (`.Item_10_95D912F14C7740665FD844AF7EA87327` (break `/Game/SurvivalGameKitV2/Blueprints/Other/Structs/S_InvSlot` _array_element_2)))) (`.RowName` (break `DataTableRowHandle` _array_element)))
                (bind _asbp_master_aicharacter_2 (cast `/Game/SmartAI/Blueprints/AI/AICharacters/BP_MasterAICharacter` OtherActor))
                (`AITask_MoveTo.AIMoveTo` (`AIBlueprintHelperLibrary.GetAIController` _asbp_master_aicharacter_2) (0.0 0.0 0.0) self
                  (:`then`
                    (goto _label :!via `Break`)))))))))))

(fn `ClearAllBaitForAnimal`
  (params (Animal :type "Actor Class Reference"))
  (bind _returnvalue (`|GetDataTableRow` "/Game/TheBiogenSurvivor/Blueprints/Animals/AnimalBaitList.AnimalBaitList" (`KismetStringLibrary.Conv_StringToName` (`KismetSystemLibrary.GetClassDisplayName` Animal)))
    (:`then`
      (for _array_element (`.BaitItems_11_0A09AD6C4CAD952B2D41B2919D5D19C7` (break `/Game/TheBiogenSurvivor/Blueprints/Other/Structs/S_AnimalBait` _returnvalue))
        (bind _rootslots (`/Game/SurvivalGameKitV2/Components/BP_MasterInventory.AllItems` (`self.BP_MasterInventory`)))
        (for _array_element_2 _rootslots
          (if (== (`.ID_2_84C2CB8945979246059C568DCD463423` (break `/Game/SurvivalGameKitV2/Blueprints/Other/Structs/S_InvItem` (`.Item_10_95D912F14C7740665FD844AF7EA87327` (break `/Game/SurvivalGameKitV2/Blueprints/Other/Structs/S_InvSlot` _array_element_2)))) (`.RowName` (break `DataTableRowHandle` _array_element)))
            (`/Game/SurvivalGameKitV2/Components/BP_MasterInventory.RemoveItem` (`self.BP_MasterInventory`) _array_element_2 true true false)))))))

(fn `SGK AllowInteraction`
  (returns (AllowInteraction :type Boolean))
  (`parent.SGK AllowInteraction`)
  (return true))

(fn `SGK Interact`
  (params (PlayerInventory :type "/Game/SurvivalGameKitV2/Components/BP_PlayerInventory Object Reference") (Action :type "/Game/SurvivalGameKitV2/Blueprints/Other/Enum/E_WorldActions Enum" :default "NewEnumerator0"))
  (returns (ReturnValue :type Boolean))
  (switch `/Game/SurvivalGameKitV2/Blueprints/Other/Enum/E_WorldActions` Action
    (:`NewEnumerator3`
      (`/Game/SurvivalGameKitV2/Components/BP_PlayerInventory.ServerOpenExtInv` PlayerInventory (`self.BP_MasterInventory`))
      (return true))
    (:`NewEnumerator12`
      (set `self.TrapActive` true)
      (`StaticMeshComponent.SetStaticMesh` (`self.StaticMesh`) (`self.SetMesh`)))))

(fn `SGK PossibleActions`
  (params (PlayerInventory :type "/Game/SurvivalGameKitV2/Components/BP_PlayerInventory Object Reference"))
  (returns (ActionsFound :type Boolean) (PossibleActions :type "Array of /Game/SurvivalGameKitV2/Blueprints/Other/Structs/S_WorldAction Structure"))
  (bind _s_worldaction (make `/Game/SurvivalGameKitV2/Blueprints/Other/Structs/S_WorldAction` "NewEnumerator3" "OPEN"))
  (if (`self.TrapActive`)
    (return true (`|MakeArray` _s_worldaction))
    (else
      (return true (`|MakeArray` _s_worldaction (make `/Game/SurvivalGameKitV2/Blueprints/Other/Structs/S_WorldAction` "NewEnumerator12" "SET"))))))

(fn `UserConstructionScript`
  (`parent.UserConstructionScript`))