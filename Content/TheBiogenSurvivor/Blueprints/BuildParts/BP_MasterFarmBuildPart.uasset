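; Master farm build part where a planted seed grows with water and fertilizer, then can be harvested through SGK interaction.
; Interface events set seed data, water, fertilizer and resets; server-side looping timers handle growth and water drain, with health following water.
; RepNotifies on plant data and state update the mesh and its timeline-driven scale.
; Plant state and data save and reload per level, restarting timers for planted seeds.
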(event `StartDrainingWater`
  ;[1 1 1] Start Draining Water
  (`/Engine/EditorBlueprintResources/ActorMacros.Switch Has Authority`
    (:`Authority`
      (bind _returnvalue (`KismetSystemLibrary.K2_SetTimerDelegate` (`|CreateDelegate` :!event `ReduceWater`) (`.WaterDrainRate_37_46013C6E4106D0AB5530D0B439F7C7A1` (break `/Game/FarmingSystem/Blueprints/Data/Structs/STR_FarmingSystem` (`self.PlantData`))) true))
      (set `self.WaterDrainTimer` _returnvalue))))

(event `GrowPlantMesh`
  ;[1 1 1] Plant Grow Timeline
  (bind (_direction _growthalpha) (`Timeline|GrowthTimeLine` :!via `PlayFromStart`)
    (:`Update`
      (`SceneComponent.SetWorldScale3D` (`self.PlantMesh`) (`KismetMathLibrary.VLerp` (`SceneComponent.K2_GetComponentScale` (`self.PlantMesh`)) (`KismetMathLibrary.Conv_DoubleToVector` (* (`.PlantMatureScale_21_6A7B8C774369A5465E1718B8878E227C` (break `/Game/FarmingSystem/Blueprints/Data/Structs/STR_FarmingSystem` (`self.PlantData`))) (`self.GetGrowthPercent`))) _growthalpha)))))

(event `/Game/FarmingSystem/Blueprints/Interfaces/BPI_FarmingSystem.BPI_ResetFarmActor`
  ;[1 1 1] Interface Events
  (`/Engine/EditorBlueprintResources/ActorMacros.Switch Has Authority`
    (:`Authority`
      (`self.SetFinishedGrowing` false)
      (`self.SetGrowthPercent` 0.0)
      (`self.SetSeedPlanted` false)
      (`KismetSystemLibrary.K2_ClearAndInvalidateTimerHandle` (`self.PlantGrowthTimer`))
      (`KismetSystemLibrary.K2_ClearAndInvalidateTimerHandle` (`self.WaterDrainTimer`)))))

(event `/Game/FarmingSystem/Blueprints/Interfaces/BPI_FarmingSystem.BPI_SetPlantData`
  (params (Data :type "/Game/FarmingSystem/Blueprints/Data/Structs/STR_FarmingSystem Structure"))
  ;[1 1 1] Interface Events
  (`/Engine/EditorBlueprintResources/ActorMacros.Switch Has Authority`
    (:`Authority`
      (`self.SetPlantData` Data)
      (`self.SetSeedPlanted` true)
      (`self.SetStartingHealth`)
      (bind _returnvalue (`KismetSystemLibrary.K2_SetTimerDelegate` (`|CreateDelegate` :!event `PlantGrowth`) 1.0 true))
      (set `self.PlantGrowthTimer` _returnvalue)
      (`self.StartDrainingWater`))))

(event `/Game/FarmingSystem/Blueprints/Interfaces/BPI_FarmingSystem.BPI_AddWater`
  (params (Amount :type "Float (double-precision)"))
  ;[1 1 1] Interface Events
  (`/Engine/EditorBlueprintResources/ActorMacros.Switch Has Authority`
    (:`Authority`
      (`self.SetWaterAmount` (+ Amount (`self.GetWaterAmount`))))))

(event `/Game/FarmingSystem/Blueprints/Interfaces/BPI_FarmingSystem.BPI_AddFertilizer`
  (params (Amount :type "Float (double-precision)"))
  ;[1 1 1] Interface Events
  (`/Engine/EditorBlueprintResources/ActorMacros.Switch Has Authority`
    (:`Authority`
      (`self.Set Fertilizer Amount` (+ Amount (`self.GetFertilizerAmount`))))))

(event `self.LoadExtraData`
  (params (SaveGame :type "/Game/SurvivalGameKitV2/Blueprints/Saving/BP_SGKSaveGame Object Reference") (Index :type Integer))
  (`self.LoadPlantData` SaveGame Index))

(fn `BPI_GetFarmActorMesh`
  (returns (Mesh :type "StaticMeshComponent Object Reference"))
  (return (`self.StaticMesh`)))

(fn `BPI_GetPlantData`
  (returns (PlantData :type "/Game/FarmingSystem/Blueprints/Data/Structs/STR_FarmingSystem Structure") (PlantState :type "/Game/FarmingSystem/Blueprints/Data/Structs/STR_PlantState Structure"))
  (return (`self.PlantData`) (`self.PlantState`)))

(fn `GetFertilizerAmount`
  (returns (CurrentFertilizerAmount :type "Float (double-precision)"))
  (return (`.CurrentFertilizer_15_069F9A7944F87E1317FDDAB69F81A85C` (break `/Game/FarmingSystem/Blueprints/Data/Structs/STR_PlantState` (`self.PlantState`)))))

(fn `GetFertilizerPercent`
  (returns (FertilizerPercent :type "Float (double-precision)"))
  (return (`.FertilizerPercent_24_F5A986494509574A1188B3A0E2F55278` (break `/Game/FarmingSystem/Blueprints/Data/Structs/STR_PlantState` (`self.PlantState`)))))

(fn `GetFinishedGrowing`
  (returns (FinishedGrowing :type Boolean))
  (return (`.FinishedGrowing_3_2F31DF0645566BA76D38C98D3ACAB7A4` (break `/Game/FarmingSystem/Blueprints/Data/Structs/STR_PlantState` (`self.PlantState`)))))

(fn `GetGrowthPercent`
  (returns (GrowthPercent :type "Float (double-precision)"))
  (return (`.GrowthPercent_8_1742713942EEC2D2AB0CEABDAEB62C9D` (break `/Game/FarmingSystem/Blueprints/Data/Structs/STR_PlantState` (`self.PlantState`)))))

(fn `GetHasFertilizer`
  (returns (HasFertilizer :type Boolean))
  (return (> (`.CurrentFertilizer_15_069F9A7944F87E1317FDDAB69F81A85C` (break `/Game/FarmingSystem/Blueprints/Data/Structs/STR_PlantState` (`self.PlantState`))) 0.0)))

(fn `GetHasWater`
  (returns (HasWater :type Boolean))
  (return (> (`.CurrentWaterAmount_10_079907774EDF4B4A7342EB8053F626EA` (break `/Game/FarmingSystem/Blueprints/Data/Structs/STR_PlantState` (`self.PlantState`))) 0.0)))

(fn `GetHealth`
  (returns (Health :type "Float (double-precision)"))
  (return (`.CurrentHealth_13_7E626B06489C69418013D2B879F1DF09` (break `/Game/FarmingSystem/Blueprints/Data/Structs/STR_PlantState` (`self.PlantState`)))))

(fn `GetSeedPlanted`
  (returns (SeedPlanted :type Boolean))
  (return (`.SeedPlanted_1_15E3D9AB4465F80843FB5D9848F33BE6` (break `/Game/FarmingSystem/Blueprints/Data/Structs/STR_PlantState` (`self.PlantState`)))))

(fn `GetWaterAmount`
  (returns (CurrentWaterAmount :type "Float (double-precision)"))
  (return (`.CurrentWaterAmount_10_079907774EDF4B4A7342EB8053F626EA` (break `/Game/FarmingSystem/Blueprints/Data/Structs/STR_PlantState` (`self.PlantState`)))))

(fn `Health On Water`
  (params (Heal :type Boolean))
  (if Heal
    (`self.SetHealth` (+ (`.CurrentHealth_13_7E626B06489C69418013D2B879F1DF09` (break `/Game/FarmingSystem/Blueprints/Data/Structs/STR_PlantState` (`self.PlantState`))) (`.WaterDrainAmount_34_531397214252805318BBA4A46DA248F3` (break `/Game/FarmingSystem/Blueprints/Data/Structs/STR_FarmingSystem` (`self.PlantData`)))))
    (else
      (`self.SetHealth` (- (`.CurrentHealth_13_7E626B06489C69418013D2B879F1DF09` (break `/Game/FarmingSystem/Blueprints/Data/Structs/STR_PlantState` (`self.PlantState`))) (`.WaterDrainAmount_34_531397214252805318BBA4A46DA248F3` (break `/Game/FarmingSystem/Blueprints/Data/Structs/STR_FarmingSystem` (`self.PlantData`))))))))

(fn `LoadPlantData`
  (params (`Save Game` :type "/Game/SurvivalGameKitV2/Blueprints/Saving/BP_SGKSaveGame Object Reference") (Index :type Integer))
  (returns (OwnerLocation :type "Vector Structure"))
  (locals (LevelSaveDataL :type "/Game/SurvivalGameKitV2/Blueprints/Other/Structs/S_LevelSaveData Structure"))
  (bind (_plantstatedata _farmingsystemdata _growthpercentdata _ownerlocation) (break `/Game/TheBiogenSurvivor/Blueprints/Other/Structs/S_PlantSave` (`|GetArrayItem` (`.PlantSaveData_72_C249817D4B5DCC5B1877C184219585AB` (break `/Game/SurvivalGameKitV2/Blueprints/Other/Structs/S_LevelSaveData` (`local.LevelSaveDataL`))) (`local.Index`))))
  (bind _returnvalue (`GameplayStatics.GetCurrentLevelName` true))
  (bind (_savefound _levelsavedata) (`/Game/SurvivalGameKitV2/Blueprints/Saving/BP_SGKSaveGame.SelectLevelSaveData` `Save Game` _returnvalue))
  (if _savefound
    (set `local.LevelSaveDataL` _levelsavedata)
    (else
      (bind _structout (setmembers `/Game/SurvivalGameKitV2/Blueprints/Other/Structs/S_LevelSaveData` :`StructRef` (`local.LevelSaveDataL`) :`Level Name` _returnvalue))
      (set `local.LevelSaveDataL` _structout)))
  (set `self.PlantState` _plantstatedata)
  (set `self.PlantData` _farmingsystemdata)
  (set `self.GrowthPercent` _growthpercentdata)
  (if (`.SeedPlanted_1_15E3D9AB4465F80843FB5D9848F33BE6` (break `/Game/FarmingSystem/Blueprints/Data/Structs/STR_PlantState` (`self.PlantState`)))
    (bind _returnvalue_2 (`KismetSystemLibrary.K2_SetTimerDelegate` (`|CreateDelegate` :!event `PlantGrowth`) 1.0 true))
    (set `self.PlantGrowthTimer` _returnvalue_2)
    (bind _returnvalue_3 (`KismetSystemLibrary.K2_SetTimerDelegate` (`|CreateDelegate` :!event `ReduceWater`) 1.0 true))
    (set `self.WaterDrainTimer` _returnvalue_3))
  (return _ownerlocation))

(fn `OnRep_PlantData`
  (`StaticMeshComponent.SetStaticMesh` (`self.PlantMesh`) (`.PlantMesh_25_69838FF64A6C27D3FDC1CFA82B7F7157` (break `/Game/FarmingSystem/Blueprints/Data/Structs/STR_FarmingSystem` (`self.PlantData`))))
  (`SceneComponent.SetWorldScale3D` (`self.PlantMesh`) (`KismetMathLibrary.Conv_DoubleToVector` (`.PlantBeginScale_19_3547C4794EEC7BC2B55147BF4D7B99C1` (break `/Game/FarmingSystem/Blueprints/Data/Structs/STR_FarmingSystem` (`self.PlantData`)))))
  (return))

(fn `OnRep_PlantState`
  (`SceneComponent.SetVisibility` (`self.PlantMesh`) (`self.GetSeedPlanted`) false)
  (if (`self.GetHasWater`)
    (if (`KismetSystemLibrary.K2_IsTimerPausedHandle` (`self.PlantGrowthTimer`))
      (`KismetSystemLibrary.K2_UnPauseTimerHandle` (`self.PlantGrowthTimer`)))
    (if (`self.GetFinishedGrowing`)
      (`SceneComponent.SetWorldScale3D` (`self.PlantMesh`) (`KismetMathLibrary.Conv_DoubleToVector` (`.PlantMatureScale_21_6A7B8C774369A5465E1718B8878E227C` (break `/Game/FarmingSystem/Blueprints/Data/Structs/STR_FarmingSystem` (`self.PlantData`)))))
      (return)
      (else
        (`TimelineComponent.SetPlayRate` (`self.GrowthTimeLine`) (/ 1.0 (`.GrowthTime_5_07B9DD8B43BBEC038BD14497AFE1A1B4` (break `/Game/FarmingSystem/Blueprints/Data/Structs/STR_FarmingSystem` (`self.PlantData`)))))
        (`self.GrowPlantMesh`)
        (return)))))

(fn `PlantGrowth`
  (bind ((`PlantID_52_CE32E1CF475F7885F464A1AE98E46F04` _plantid) (`GrowthTime_5_07B9DD8B43BBEC038BD14497AFE1A1B4` _growthtime) (`WaterDrainRate_37_46013C6E4106D0AB5530D0B439F7C7A1` _waterdrainrate) (`RewardOnHarvest_41_55CDDBE644BE12EBABC9C5B71890D607` _rewardonharvest) (`MaxHealth_44_D35BDE8D4151D1C87E875C8513C8AF3D` _maxhealth) (`WaterDrainAmountMature_47_12025AAF47742B59DD0F6A9BDAAED519` _waterdrainamountmature) (`FertilizerDrainAmount_49_5D28646C4E904C89EFB4A680E18F0DBC` _fertilizerdrainamount)) (break `/Game/FarmingSystem/Blueprints/Data/Structs/STR_FarmingSystem` (`self.PlantData`)))
  (bind _returnvalue (/ 1.0 _growthtime))
  (`/Engine/EditorBlueprintResources/ActorMacros.Switch Has Authority`
    (:`Authority`
      (if (`self.GetHasWater`)
        (if (`self.GetHasFertilizer`)
          (`self.Set Fertilizer Amount` (- (`self.GetFertilizerAmount`) _fertilizerdrainamount))
          (`self.SetFertilizerPercent` (+ (`self.GetFertilizerPercent`) _returnvalue)))
        (`self.SetGrowthPercent` (+ _returnvalue (`self.GetGrowthPercent`)))
        (if (>= (`self.GetGrowthPercent`) 1.0)
          (`self.SetFinishedGrowing` true)
          (return)
          (else
            (return)))
        (else
          (`KismetSystemLibrary.K2_PauseTimerHandle` (`self.PlantGrowthTimer`))
          (return))))
    (:`Remote`
      (return))))

(fn `ReduceWater`
  (`/Engine/EditorBlueprintResources/ActorMacros.Switch Has Authority`
    (:`Authority`
      (`self.Health On Water` (`self.GetHasWater`))
      (if (`self.GetFinishedGrowing`)
        (`self.SetWaterAmount` (`KismetMathLibrary.FClamp` (- (`self.GetWaterAmount`) (`.WaterDrainAmountMature_47_12025AAF47742B59DD0F6A9BDAAED519` (break `/Game/FarmingSystem/Blueprints/Data/Structs/STR_FarmingSystem` (`self.PlantData`)))) 0.0 (`.MaxWater_19_BFCB775F4D3FA92F2786B7B745BA83CD` (break `/Game/FarmingSystem/Blueprints/Data/Structs/STR_PlantState` (`self.PlantState`)))))
        (else
          (`self.SetWaterAmount` (`KismetMathLibrary.FClamp` (- (`self.GetWaterAmount`) (`.WaterDrainAmount_34_531397214252805318BBA4A46DA248F3` (break `/Game/FarmingSystem/Blueprints/Data/Structs/STR_FarmingSystem` (`self.PlantData`)))) 0.0 (`.MaxWater_19_BFCB775F4D3FA92F2786B7B745BA83CD` (break `/Game/FarmingSystem/Blueprints/Data/Structs/STR_PlantState` (`self.PlantState`))))))))))

(fn `SaveExtraData`
  (params (SaveGame :type "/Game/SurvivalGameKitV2/Blueprints/Saving/BP_SGKSaveGame Object Reference") (LevelSaveData :type "/Game/SurvivalGameKitV2/Blueprints/Other/Structs/S_LevelSaveData Structure"))
  (returns (ExtraDataIndex :type Integer) (NewLevelSaveData :type "/Game/SurvivalGameKitV2/Blueprints/Other/Structs/S_LevelSaveData Structure"))
  ;[1 1 1] Prepare Plant Data for saving
  (bind (_returnvalue _newlevelsavedata) (`self.SavePlantData` SaveGame LevelSaveData))
  (return _returnvalue _newlevelsavedata))

(fn `SavePlantData`
  (params (SaveGame :type "/Game/SurvivalGameKitV2/Blueprints/Saving/BP_SGKSaveGame Object Reference") (LevelSaveData :type "/Game/SurvivalGameKitV2/Blueprints/Other/Structs/S_LevelSaveData Structure"))
  (returns (ReturnValue :type Integer) (NewLevelSaveData :type "/Game/SurvivalGameKitV2/Blueprints/Other/Structs/S_LevelSaveData Structure"))
  (locals (LevelSaveDataL :type "/Game/SurvivalGameKitV2/Blueprints/Other/Structs/S_LevelSaveData Structure") (LocationL :type "Vector Structure"))
  (bind _returnvalue (`self.GetAttachParentActor`))
  (bind (_levelname _itemsavedata _itemspawnersavedata _buildpartdata _locksavedata _storagesavedata _cookingsavedata _craftingsavedata _vendersavedata _equipmentsavedata _resourcedata _respawnnames _buildparton _bioprocessorsavedata _plantsavedata) (break `/Game/SurvivalGameKitV2/Blueprints/Other/Structs/S_LevelSaveData` (`local.LevelSaveDataL`)))
  (set `local.LevelSaveDataL` LevelSaveData)
  (`/Engine/EditorBlueprintResources/StandardMacros.IsValid` _returnvalue
    (:`Is Valid`
      (set `local.LocationL` (`self.K2_GetActorLocation` _returnvalue)))
    (:`Is Not Valid`
      _))
  (bind _returnvalue_2 (`KismetArrayLibrary.Array_Add` _plantsavedata (make `/Game/TheBiogenSurvivor/Blueprints/Other/Structs/S_PlantSave` (`self.PlantState`) (`self.PlantData`) (`self.GrowthPercent`) (`local.LocationL`))))
  (setmembers `/Game/SurvivalGameKitV2/Blueprints/Other/Structs/S_LevelSaveData` :`StructRef` (`local.LevelSaveDataL`) :`PlantSaveData` _plantsavedata)
  (return _returnvalue_2 (`local.LevelSaveDataL`)))

(fn `Set Fertilizer Amount`
  (params (Fertilizer :type "Float (double-precision)"))
  (`/Engine/EditorBlueprintResources/ActorMacros.Switch Has Authority`
    (:`Authority`
      (bind _structout (setmembers `/Game/FarmingSystem/Blueprints/Data/Structs/STR_PlantState` :`StructRef` (`self.PlantState`) :`CurrentFertilizer` Fertilizer))
      (set `self.PlantState` _structout)
      (return))
    (:`Remote`
      (return))))

(fn `SetFertilizerPercent`
  (params (FertilizerPercent :type "Float (double-precision)"))
  (`/Engine/EditorBlueprintResources/ActorMacros.Switch Has Authority`
    (:`Authority`
      (bind _structout (setmembers `/Game/FarmingSystem/Blueprints/Data/Structs/STR_PlantState` :`StructRef` (`self.PlantState`) :`FertilizerPercent` (`KismetMathLibrary.FClamp` FertilizerPercent)))
      (set `self.PlantState` _structout)
      (return))
    (:`Remote`
      (return))))

(fn `SetFinishedGrowing`
  (params (FinishedGrowing :type Boolean))
  (locals (FinishedGrowingL :type Boolean))
  (set `local.FinishedGrowingL` FinishedGrowing)
  (`/Engine/EditorBlueprintResources/ActorMacros.Switch Has Authority`
    (:`Authority`
      (bind _structout (setmembers `/Game/FarmingSystem/Blueprints/Data/Structs/STR_PlantState` :`StructRef` (`self.PlantState`) :`FinishedGrowing` (`local.FinishedGrowingL`)))
      (set `self.PlantState` _structout)
      (if (`local.FinishedGrowingL`)
        (`KismetSystemLibrary.K2_ClearAndInvalidateTimerHandle` (`self.PlantGrowthTimer`))
        (return)
        (else
          (return))))
    (:`Remote`
      (return))))

(fn `SetGrowthPercent`
  (params (GrowthPercent :type "Float (double-precision)"))
  (`/Engine/EditorBlueprintResources/ActorMacros.Switch Has Authority`
    (:`Authority`
      (bind _structout (setmembers `/Game/FarmingSystem/Blueprints/Data/Structs/STR_PlantState` :`StructRef` (`self.PlantState`) :`GrowthPercent` (`KismetMathLibrary.FClamp` GrowthPercent)))
      (set `self.PlantState` _structout)
      (return))
    (:`Remote`
      (return))))

(fn `SetHealth`
  (params (Health :type "Float (double-precision)"))
  (`/Engine/EditorBlueprintResources/ActorMacros.Switch Has Authority`
    (:`Authority`
      (bind _structout (setmembers `/Game/FarmingSystem/Blueprints/Data/Structs/STR_PlantState` :`StructRef` (`self.PlantState`) :`CurrentHealth` (`KismetMathLibrary.FClamp` Health 0.0 (`.MaxHealth_17_3E058ED54A55EBAE482D9BA30D949673` (break `/Game/FarmingSystem/Blueprints/Data/Structs/STR_PlantState` (`self.PlantState`))))))
      (set `self.PlantState` _structout)
      (return))
    (:`Remote`
      (return))))

(fn `SetPlantData`
  (params (PlantData :type "/Game/FarmingSystem/Blueprints/Data/Structs/STR_FarmingSystem Structure"))
  (`/Engine/EditorBlueprintResources/ActorMacros.Switch Has Authority`
    (:`Authority`
      (set `self.PlantData` PlantData)
      (return))))

(fn `SetSeedPlanted`
  (params (SeedPlanted :type Boolean))
  (`/Engine/EditorBlueprintResources/ActorMacros.Switch Has Authority`
    (:`Authority`
      (bind _structout (setmembers `/Game/FarmingSystem/Blueprints/Data/Structs/STR_PlantState` :`StructRef` (`self.PlantState`) :`SeedPlanted` SeedPlanted))
      (set `self.PlantState` _structout)
      (return))
    (:`Remote`
      (return))))

(fn `SetStartingHealth`
  (bind (_plantid _plantname _growthtime _plantbeginscale _plantmaturescale _waterdrainamount _waterdrainrate _plantmesh _thumbnail _rewardonharvest _maxhealth) (break `/Game/FarmingSystem/Blueprints/Data/Structs/STR_FarmingSystem` (`self.PlantData`)))
  (setmembers `/Game/FarmingSystem/Blueprints/Data/Structs/STR_PlantState` :`StructRef` (`self.PlantState`) :`CurrentHealth` _maxhealth :`MaxHealth` _maxhealth))

(fn `SetWaterAmount`
  (params (CurrentWaterAmount :type "Float (double-precision)"))
  (`/Engine/EditorBlueprintResources/ActorMacros.Switch Has Authority`
    (:`Authority`
      (bind _structout (setmembers `/Game/FarmingSystem/Blueprints/Data/Structs/STR_PlantState` :`StructRef` (`self.PlantState`) :`CurrentWaterAmount` (`KismetMathLibrary.FClamp` CurrentWaterAmount 0.0 (`.MaxWater_19_BFCB775F4D3FA92F2786B7B745BA83CD` (break `/Game/FarmingSystem/Blueprints/Data/Structs/STR_PlantState` (`self.PlantState`))))))
      (set `self.PlantState` _structout))
    (:`Remote`
      (return))))

(fn `SGK AllowInteraction`
  (returns (AllowInteraction :type Boolean))
  (`parent.SGK AllowInteraction`)
  (return (`.FinishedGrowing_3_2F31DF0645566BA76D38C98D3ACAB7A4` (break `/Game/FarmingSystem/Blueprints/Data/Structs/STR_PlantState` (`self.PlantState`)))))

(fn `SGK Interact`
  (params (PlayerInventory :type "/Game/SurvivalGameKitV2/Blueprints/Components/BP_PlayerInventory Object Reference") (Action :type "/Game/SurvivalGameKitV2/Blueprints/Other/Enum/E_WorldActions Enum" :default "NewEnumerator0"))
  (returns (ReturnValue :type Boolean))
  (switch `/Game/SurvivalGameKitV2/Blueprints/Other/Enum/E_WorldActions` Action
    (:`NewEnumerator8`
      (bind _asbp_sgkcontroller (cast `/Game/SurvivalGameKitV2/Blueprints/Characters/BP_SGKController` (`ActorComponent.GetOwner` (`local.PlayerInventory`))))
      (`/Game/FarmingSystem/Blueprints/C-FarmingSystem.SRV_HarvestPlant` (`self.GetComponentByClass` _asbp_sgkcontroller "/Game/FarmingSystem/Blueprints/C-FarmingSystem.C-FarmingSystem_C") self)
      (`/Game/SurvivalGameKitV2/Blueprints/Components/BP_PlayerInventory.ServerSetIgnoreActor` (`local.PlayerInventory`) self 0.2)
      (return true))))

(fn `SGK PossibleActions`
  (params (PlayerInventory :type "/Game/SurvivalGameKitV2/Blueprints/Components/BP_PlayerInventory Object Reference"))
  (returns (ActionsFound :type Boolean) (PossibleActions :type "Array of /Game/SurvivalGameKitV2/Blueprints/Other/Structs/S_WorldAction Structure"))
  (return true (`|MakeArray` (make `/Game/SurvivalGameKitV2/Blueprints/Other/Structs/S_WorldAction` "NewEnumerator8" "HARVEST"))))

(fn `UserConstructionScript`
  (`parent.UserConstructionScript`))