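; Master player character for The Biogen Survivor, with modular body meshes following the main mesh via leader pose.
; Vision input flip-flops post-process materials chosen from the controller's active mutations.
; Stats, journal and quest log inputs toggle PlayerInventory panels unless input is blocked.
; It also serves the quest system, tracking gold and cumulative experience with growing level thresholds, toggling mouse mode, and sphere-tracing forward to send interact messages.
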(event `/Game/EasyQuests/Blueprints/BPI/BP_BPI_Quests.ToggleMouseInput`
  (`self.MouseInput`))

(event `AddExperience`
  (params (Amount :type "Float (double-precision)"))
  (bind _output_get (set `self.Experience` (+ (`self.Experience`) Amount)))
  (while (>= _output_get (`self.NeededExperience`))
    (`/Engine/EditorBlueprintResources/StandardMacros.IncrementInt` (`self.Level`)
      (:`  `
        (set `self.NeededExperience` (* (`self.NeededExperience`) 1.5))))))

(event `AddGold`
  (params (Amount :type Integer))
  (set `self.Gold` (+ (`self.Gold`) Amount)))

(event `/Game/EasyQuests/Blueprints/BPI/BP_BPI_Quests.ModifyGold`
  (params (Amount :type Integer))
  (`self.AddGold` Amount))

(event `/Game/EasyQuests/Blueprints/BPI/BP_BPI_Quests.ModifyExperience`
  (params (Amount :type "Float (double-precision)"))
  (`self.AddExperience` Amount))

(event `SaveEXPGold`
  (`/Game/EasyQuests/Blueprints/BP_BPC_PlayerQuestComponent.SaveQuests` (`self.BP_BPC_PlayerQuestComponent`)))

(event `/Game/EasyQuests/Blueprints/BPI/BP_BPI_Quests.LoadExpGoldInfo`
  (params (Level :type Integer) (Gold :type Integer) (Experience :type "Float (double-precision)") (NeededExperience :type "Float (double-precision)"))
  (set `self.Level` Level)
  (set `self.Gold` Gold)
  (set `self.Experience` Experience)
  (set `self.NeededExperience` NeededExperience))

(event `InputAction|QuestInteract`
  (params (Key :type "Key Structure"))
  (bind _returnvalue (`self.K2_GetActorLocation`))
  (:`Pressed`
    (bind (_outhit _returnvalue_2) (`KismetSystemLibrary.SphereTraceSingleForObjects` _returnvalue (+ _returnvalue (* (`SceneComponent.GetForwardVector` (`self.CapsuleComponent`)) (`self.InteractionRange`))) 50.0 (`|MakeArray` "ObjectTypeQuery2" "ObjectTypeQuery3" :!type "EObjectTypeQuery Enum") false (`|MakeArray` self :!type "Actor Object Reference")))
    (if _returnvalue_2
      (message `/Game/EasyQuests/Blueprints/BPI/BP_BPI_QuestsInteraction.OnInteract` (`.HitActor` (`GameplayStatics.BreakHitResult` _outhit)) self))))

(event `ActivateVision`
  (`/Engine/EditorBlueprintResources/StandardMacros.FlipFlop`
    (:`A`
      (bind _asbp_sgkcontroller (cast `/Game/SurvivalGameKitV2/Blueprints/Characters/BP_SGKController` (`self.GetOwner`)))
      (bind _ppsettings (`/Game/TheBiogenSurvivor/Blueprints/Other/Interfaces/BP_TBSFunctions.TBS GetMutationVisionSettings` (`/Game/TheBiogenSurvivor/Blueprints/Components/BP_PlayerMutations_TBS.ActiveMutations` (`/Game/SurvivalGameKitV2/Blueprints/Characters/BP_SGKController.BP_PlayerMutations_TBS` _asbp_sgkcontroller))))
      (setmembers `PostProcessSettings` :`StructRef` (`PostProcessComponent.Settings` (`self.PostProcess`)) :`WeightedBlendables` (`.WeightedBlendables` (break `PostProcessSettings` _ppsettings))))
    (:`B`
      (setmembers `PostProcessSettings` :`StructRef` (`PostProcessComponent.Settings` (`self.PostProcess`)) :`WeightedBlendables` (make `WeightedBlendables` _)))))

(event `EnhancedInput|/Game/TheBiogenSurvivor/Blueprints/Controls/VisionInput`
  (params (ActionValue :type Boolean) (ElapsedSeconds :type "Float (double-precision)") (TriggeredSeconds :type "Float (double-precision)") (InputAction :type "InputAction Object Reference" :default "/Game/TheBiogenSurvivor/Blueprints/Controls/VisionInput.VisionInput"))
  (:`Started`
    (`self.ActivateVision`)))

(event `EnhancedInput|/Game/TheBiogenSurvivor/Blueprints/Controls/CharacterStatInput`
  (params (ActionValue :type Boolean) (ElapsedSeconds :type "Float (double-precision)") (TriggeredSeconds :type "Float (double-precision)") (InputAction :type "InputAction Object Reference" :default "/Game/TheBiogenSurvivor/Blueprints/Controls/CharacterStatInput.CharacterStatInput"))
  (:`Started`
    (`self.IsInputBlocked`
      (:`Fasle`
        (`/Game/TheBiogenSurvivor/Blueprints/Components/BP_TBS_PlayerInventory.TogglePlayerStats` (`self.PlayerInventory`))))))

(event `EnhancedInput|/Game/TheBiogenSurvivor/Blueprints/Controls/JournalInput`
  (params (ActionValue :type Boolean) (ElapsedSeconds :type "Float (double-precision)") (TriggeredSeconds :type "Float (double-precision)") (InputAction :type "InputAction Object Reference" :default "/Game/TheBiogenSurvivor/Blueprints/Controls/JournalInput.JournalInput"))
  (:`Started`
    (`self.IsInputBlocked`
      (:`Fasle`
        (`/Game/TheBiogenSurvivor/Blueprints/Components/BP_TBS_PlayerInventory.ToggleJournal` (`self.PlayerInventory`))))))

(event `EnhancedInput|/Game/TheBiogenSurvivor/Blueprints/Controls/QuestLogInput`
  (params (ActionValue :type Boolean) (ElapsedSeconds :type "Float (double-precision)") (TriggeredSeconds :type "Float (double-precision)") (InputAction :type "InputAction Object Reference" :default "/Game/TheBiogenSurvivor/Blueprints/Controls/QuestLogInput.QuestLogInput"))
  (:`Started`
    (`self.IsInputBlocked`
      (:`Fasle`
        (`/Game/TheBiogenSurvivor/Blueprints/Components/BP_TBS_PlayerInventory.ToggleQuestLog` (`self.PlayerInventory`))))))

(fn `GetCharacterLevel`
  (returns (Level :type Integer))
  (return (`self.Level`)))

(fn `GetExperience`
  (returns (Experience :type "Float (double-precision)"))
  (return (`self.Experience`)))

(fn `GetGold`
  (returns (TotalGold :type Integer))
  (return (`self.Gold`)))

(fn `GetNeededExperience`
  (returns (NeededExperience :type "Float (double-precision)"))
  (return (`self.NeededExperience`)))

(fn `MouseInput`
  (bind _returnvalue (`GameplayStatics.GetPlayerController` 0))
  (if (`self.MouseVisibility`)
    (set `PlayerController.bShowMouseCursor` false _returnvalue)
    (`WidgetBlueprintLibrary.SetInputMode_GameOnly` _returnvalue)
    (set `self.MouseVisibility` false)
    (else
      (set `PlayerController.bShowMouseCursor` true _returnvalue)
      (`WidgetBlueprintLibrary.SetInputMode_GameAndUIEx` _returnvalue null)
      (set `self.MouseVisibility` true))))

(fn `Toggle Vision`
  (`/Engine/EditorBlueprintResources/StandardMacros.FlipFlop`
    (:`A`
      (bind _asbp_sgkcontroller (cast `/Game/SurvivalGameKitV2/Blueprints/Characters/BP_SGKController` (`self.GetOwner`)))
      (bind _ppsettings (`/Game/TheBiogenSurvivor/Blueprints/Other/Interfaces/BP_TBSFunctions.TBS GetMutationVisionSettings` (`/Game/TheBiogenSurvivor/Blueprints/Components/BP_PlayerMutations_TBS.ActiveMutations` (`/Game/SurvivalGameKitV2/Blueprints/Characters/BP_SGKController.BP_PlayerMutations_TBS` _asbp_sgkcontroller))))
      (setmembers `PostProcessSettings` :`StructRef` (`PostProcessComponent.Settings` (`self.PostProcess`)) :`WeightedBlendables` (`.WeightedBlendables` (break `PostProcessSettings` _ppsettings))))
    (:`B`
      (setmembers `PostProcessSettings` :`StructRef` (`PostProcessComponent.Settings` (`self.PostProcess`)) :`WeightedBlendables` (make `WeightedBlendables` _)))))

(fn `UserConstructionScript`
  (`parent.UserConstructionScript`)
  (`SkinnedMeshComponent.SetLeaderPoseComponent` (`self.Legs`) (`self.Mesh`) false false)
  (`SkinnedMeshComponent.SetLeaderPoseComponent` (`self.Head`) (`self.Mesh`) false false)
  (`SkinnedMeshComponent.SetLeaderPoseComponent` (`self.Feet`) (`self.Mesh`) false false)
  (`SkinnedMeshComponent.SetLeaderPoseComponent` (`self.Trousers`) (`self.Mesh`) false false)
  (`SkinnedMeshComponent.SetLeaderPoseComponent` (`self.Torso`) (`self.Mesh`) false false))