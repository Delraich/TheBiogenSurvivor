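; Time-of-day actor that runs the game clock, rotates the sun and moon, and derives world temperature.
; Tick advances a Timespan by SunSpeed, signals on zero minutes, sets both light rotations from it and flags night from sun pitch.
; A looping timer samples TempCurve by day fraction.
; It registers with the SGK save system, retrying if needed, to persist time per level; day/night intensity blending exists but is unwired.
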(event `self.ReceiveBeginPlay`
  (set `self.Time` (`KismetMathLibrary.MakeTimespan` 0 8))
  (`self.InitializeComponentSaveSystem`)
  (`KismetSystemLibrary.K2_SetTimer` null "UpdateWorldTemperature" (/ 1.0 (`self.TemperatureUpdateRate`)) true))

(event `self.ReceiveTick`
  (params (DeltaSeconds :type "Float (single-precision)"))
  (bind (_time_days _time_hours _time_minutes) (`KismetMathLibrary.BreakTimespan` (`self.Time`)))
  (bind (_returnvalue_roll _returnvalue_pitch) (`KismetMathLibrary.BreakRotator` (`self.K2_GetActorRotation` (`self.Sun`))))
  (bind _returnvalue (* (`KismetMathLibrary.SafeDivide` (`KismetMathLibrary.Conv_IntToDouble` (+ (* (+ _time_hours 6) 60) _time_minutes)) 1440.0) 360.0))
  ;[1 1 1] Update current time
  (bind _output_get (set `self.New Time Delta` (* DeltaSeconds (`self.Sun Speed`))))
  (`self.Update Time` _output_get)
  (`self.K2_SetActorRotation` (`self.Sun`) (`KismetMathLibrary.MakeRotator` 0.0 _returnvalue) false)
  (`self.K2_SetActorRotation` (`self.Moon`) (`KismetMathLibrary.MakeRotator` 0.0 (- _returnvalue 180.0)) false)
  ;[1 1 1] Check if the rotation is between 0 - 100 for night time
  (bind _output_get_2 (set `self.Night` (`KismetMathLibrary.InRange_FloatFloat` _returnvalue_pitch 0.0 100.0))))

(event `self.SGKSave`
  (params (Save :type "/Game/SurvivalGameKitV2/Blueprints/Saving/BP_SGKSaveGame Object Reference"))
  ;[1 1 1] Save system
  (`self.SaveComponentData` Save))

(event `InitializeComponentSaveSystem`
  ;[1 1 1] Save system
  (bind _savegame (message `/Game/SurvivalGameKitV2/Blueprints/Other/Interfaces/BP_SGKGameModeInterface.SGK GetSaveGame` (`GameplayStatics.GetGameMode`) :!label _label))
  (bind _output_get (set `self.SaveSystem` _savegame))
  (`/Engine/EditorBlueprintResources/StandardMacros.IsValid` _output_get
    (:`Is Valid`
      (`KismetArrayLibrary.Array_AddUnique` (`/Game/SurvivalGameKitV2/Blueprints/Saving/BP_SaveSystem.SaveActors` (`self.SaveSystem`)) self)
      (add `/Game/SurvivalGameKitV2/Blueprints/Saving/BP_SaveSystem.LoadData` (`self.SaveSystem`) (delegate `LoadComponent`))
      (if (`/Game/SurvivalGameKitV2/Blueprints/Saving/BP_SaveSystem.PlayerLoadSave` (`self.SaveSystem`))
        (`self.LoadComponentData` (`/Game/SurvivalGameKitV2/Blueprints/Saving/BP_SaveSystem.LoadedSaveGameData` (`self.SaveSystem`)))))
    (:`Is Not Valid`
      (`/Engine/EditorBlueprintResources/StandardMacros.Do N` 10
        (:`Exit`
          (`KismetSystemLibrary.Delay` 0.2)
          (goto _label))))))

(event `LoadComponent`
  (params (SaveGame :type "/Game/SurvivalGameKitV2/Blueprints/Saving/BP_SGKSaveGame Object Reference"))
  ;[1 1 1] Save system
  (`self.InGameLoadComponentData` SaveGame))

(fn `Actor Attack Target`
  (returns (`Attack Target` :type "Actor Object Reference"))
  (return null))

(fn `AI Can Interact?`
  (returns (`Can Interact` :type Boolean))
  (return false))

(fn `AI Is Dead?`
  (returns (Dead :type Boolean))
  (return false))

(fn `Day Lighting`
  (params (Delta :type "Float (double-precision)"))
  (bind _lightcomponent (`Light.LightComponent` (`self.Sun`)))
  (bind _lightcomponent_2 (`SkyLight.LightComponent` (`self.Skylight`)))
  ;[1 1 1] Set directional light intensity
  (`LightComponent.SetIntensity` _lightcomponent (`KismetMathLibrary.FInterpTo` (`LightComponentBase.Intensity` _lightcomponent) 3.0 (/ Delta 64.0) 4.0))
  ;[1 1 1] Set skylight intensity
  (`SkyLightComponent.SetIntensity` _lightcomponent_2 (`KismetMathLibrary.FInterpTo` (`LightComponentBase.Intensity` _lightcomponent_2) 0.5 (/ (`local.Delta`) 64.0) 8.0)))

(fn `InGameLoadComponentData`
  (params (Save :type "/Game/SurvivalGameKitV2/Blueprints/Saving/BP_SGKSaveGame Object Reference"))
  (`self.LoadComponentData` Save))

(fn `LoadComponentData`
  (params (SaveGame :type "/Game/SurvivalGameKitV2/Blueprints/Saving/BP_SGKSaveGame Object Reference"))
  (returns (LoadComplete :type Boolean))
  (bind _returnvalue (`GameplayStatics.GetCurrentLevelName` true))
  (bind (_savefound _levelsavedata) (`/Game/SurvivalGameKitV2/Blueprints/Saving/BP_SGKSaveGame.SelectLevelSaveData` (`local.SaveGame`) _returnvalue))
  (if _savefound
    (set `self.Time` (`.TimeOfDay_77_7DC0304348CD9349875496B5AFC4F637` (break `/Game/SurvivalGameKitV2/Blueprints/Other/Structs/S_LevelSaveData` _levelsavedata)))
    (return true)
    (else
      (return false))))

(fn `Night Lighting`
  (params (Delta :type "Float (double-precision)"))
  (bind _lightcomponent (`Light.LightComponent` (`self.Sun`)))
  ;[1 1 1] Set the directional light intensity
  (`LightComponent.SetIntensity` _lightcomponent (`KismetMathLibrary.FInterpTo` (`LightComponentBase.Intensity` _lightcomponent) (`self.NightIntensity`) (/ (`local.Delta`) 64.0) 12.0))
  ;[1 1 1] Set skylight intensity
  (`SkyLightComponent.SetIntensity` (`SkyLight.LightComponent` (`self.Skylight`)) (`KismetMathLibrary.FInterpTo` (`LightComponentBase.Intensity` (`SkyLight.LightComponent` (`self.Skylight`))) (`self.NightSkyIntensity`) (/ (`local.Delta`) 64.0) 8.0)))

(fn `SaveComponentData`
  (params (SaveGame :type "/Game/SurvivalGameKitV2/Blueprints/Saving/BP_SGKSaveGame Object Reference"))
  (locals (LevelSaveDataL :type "/Game/SurvivalGameKitV2/Blueprints/Other/Structs/S_LevelSaveData Structure"))
  (bind _returnvalue (`GameplayStatics.GetCurrentLevelName` true))
  (bind (_savefound _levelsavedata) (`/Game/SurvivalGameKitV2/Blueprints/Saving/BP_SGKSaveGame.SelectLevelSaveData` (`local.SaveGame`) _returnvalue))
  (if _savefound
    (set `local.LevelSaveDataL` _levelsavedata)
    (else
      (setmembers `/Game/SurvivalGameKitV2/Blueprints/Other/Structs/S_LevelSaveData` :`StructRef` (`local.LevelSaveDataL`) :`Level Name` _returnvalue)))
  (bind _structout (setmembers `/Game/SurvivalGameKitV2/Blueprints/Other/Structs/S_LevelSaveData` :`StructRef` (`local.LevelSaveDataL`) :`TimeOfDay` (`self.Time`)))
  (`/Game/SurvivalGameKitV2/Blueprints/Saving/BP_SGKSaveGame.SetLevelData` (`local.SaveGame`) _structout))

(fn `Update Time`
  (params (Delta :type "Float (double-precision)"))
  (bind (_days _hours _minutes _seconds) (`KismetMathLibrary.BreakTimespan` (`self.Time`)))
  ;[1 1 1] Update tick time
  ;[1 1 1] Set new time
  (bind _output_get (set `self.Time` (`KismetMathLibrary.MakeTimespan` _days _hours _minutes (+ _seconds (`KismetMathLibrary.FTrunc` (* Delta 240.0))))))
  (bind (_days_2 _hours_2 _minutes_2) (`KismetMathLibrary.BreakTimespan` _output_get))
  ;[1 1 1] On each new hour call time hour event and if debug text is true print time
  (if (== _minutes_2 0)
    (`self.Time Hour` _hours_2))
  (if (`self.Debug Text`)
    (`KismetSystemLibrary.PrintString` (`KismetStringLibrary.Concat_StrStr` (`KismetStringLibrary.Conv_IntToString` _hours_2) ":" (`KismetStringLibrary.Conv_IntToString` _minutes_2)))))

(fn `UpdateWorldTemperature`
  (bind (_days _hours _minutes _seconds) (`KismetMathLibrary.BreakTimespan` (`self.Time`)))
  (set `self.FinalWorldTemperature` (`CurveFloat.GetFloatValue` (`self.TempCurve`) (+ (/ _hours 24.0) (/ _minutes 1440.0) (/ _seconds 86400.0)))))

(fn `UserConstructionScript`)