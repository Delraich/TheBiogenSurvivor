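; BP_WaterBodyOcean is an ocean water body that switches player-type characters in and out of swimming through overlap events.
; When a BP_TBSMasterCharacter begins overlapping it, the ocean calls StartSwimming on that character, and when the overlap ends it calls ResetWaterZ.
; The SGK interaction, item and code functions are empty stubs returning default values, and BeginPlay, Tick and the construction script do nothing.
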(event `self.ReceiveBeginPlay`)

(event `self.ReceiveActorBeginOverlap`
  (params (OtherActor :type "Actor Object Reference"))
  (bind _asbp_tbsmaster_character (cast `/Game/TheBiogenSurvivor/Blueprints/Character/BP_TBSMasterCharacter` OtherActor))
  (`/Game/SurvivalGameKitV2/Blueprints/Characters/BP_SGKMasterCharacter.StartSwimming` _asbp_tbsmaster_character))

(event `self.ReceiveActorEndOverlap`
  (params (OtherActor :type "Actor Object Reference"))
  (bind _asbp_tbsmaster_character (cast `/Game/TheBiogenSurvivor/Blueprints/Character/BP_TBSMasterCharacter` OtherActor))
  (`/Game/SurvivalGameKitV2/Blueprints/Characters/BP_SGKMasterCharacter.ResetWaterZ` _asbp_tbsmaster_character))

(fn `SGK AllowInteraction`
  (returns (AllowInteraction :type Boolean))
  (return false))

(fn `SGK CodeCheck`
  (params (Code :type Text))
  (returns (CodeAccepted :type Boolean))
  (return false))

(fn `SGK DropItem`
  (params (InvItem :type "/Game/SurvivalGameKitV2/Blueprints/Other/Structs/S_InvItem Structure") (Dropped :type Boolean) (Spawned :type Boolean) (SaveLoaded :type Boolean))
  (returns (ReturnValue :type Boolean))
  (return false))

(fn `SGK EndInteraction`
  (params (PlayerInventory :type "/Game/SurvivalGameKitV2/Components/BP_PlayerInventory Object Reference"))
  (returns (ReturnValue :type Boolean))
  (return false))

(fn `SGK GetVerifiedPlayers`
  (returns (VerifiedPlayers :type "Array of Text"))
  (return))

(fn `SGK Interact`
  (params (PlayerInventory :type "/Game/SurvivalGameKitV2/Components/BP_PlayerInventory Object Reference") (Action :type "/Game/SurvivalGameKitV2/Blueprints/Other/Enum/E_WorldActions Enum" :default "NewEnumerator0"))
  (returns (ReturnValue :type Boolean))
  (return false))

(fn `SGK InteractName`
  (returns (InteractName :type Text))
  (return ""))

(fn `SGK InvItem`
  (returns (IsItem :type Boolean) (InvItem :type "/Game/SurvivalGameKitV2/Blueprints/Other/Structs/S_InvItem Structure"))
  (return false))

(fn `SGK ItemAmount`
  (returns (Amount :type Integer))
  (return 0))

(fn `SGK Mesh`
  (returns (Mesh :type "PrimitiveComponent Object Reference"))
  (return null))

(fn `SGK PossibleActions`
  (params (PlayerInventory :type "/Game/SurvivalGameKitV2/Components/BP_PlayerInventory Object Reference"))
  (returns (ActionsFound :type Boolean) (PossibleActions :type "Array of /Game/SurvivalGameKitV2/Blueprints/Other/Structs/S_WorldAction Structure"))
  (return false))

(fn `SGK UpdateCode`
  (params (Code :type Text))
  (returns (ReturnValue :type Boolean))
  (return false))

(fn `SGK VerifyPlayer`
  (params (Text :type Text))
  (returns (ReturnValue :type Boolean))
  (return false))

(fn `UserConstructionScript`)