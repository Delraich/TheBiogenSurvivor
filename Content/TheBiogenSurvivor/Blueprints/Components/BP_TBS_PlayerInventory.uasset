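; Player inventory component for The Biogen Survivor, extending the SGK parent with survival, quest and menu logic.
; Initialization starts server timers for hunger, thirst, temperature and regeneration, plus a local look trace.
; Consuming applies mutation-specific stats and disease effects; adding, moving or dropping items updates quest objective counts.
; Stats, journal and quest toggles switch tabs in one guide book widget; respawning uses a named build part or random PlayerStart.
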(event `self.ServerKillPlayerCharacter`
  (`self.Close Journal`)
  (`self.ClosePlayerStats`)
  (`self.CloseQuestLog`)
  (`parent.ServerKillPlayerCharacter`))

(event `ServerSetPlayerStatsOpen`
  (params (PlayerStatsOpen :type Boolean))
  ;[1 1 1] Server sets player stats open
  (bind _output_get (set `self.PlayerStatsOpen` PlayerStatsOpen))
  (if _output_get
    _))

(event `ClientSetPlayerStatsOpen`
  (params (PlayerStatsOpen :type Boolean))
  ;[1 1 1] Client sets player stats open
  (set `self.PlayerStatsOpen` PlayerStatsOpen))

(event `ServerSetJournalOpen`
  (params (`Journal Open` :type Boolean))
  ;[1 1 1] ServerSets Journal Open
  (set `self.JournalOpen` `Journal Open`))

(event `ClientSetJournalOpen`
  (params (JournalOpen :type Boolean))
  ;[1 1 1] Client sets Journal open
  (set `self.JournalOpen` JournalOpen))

(event `ServerSetQuestLogOpen`
  (params (QuestLogOpen :type Boolean))
  ;[1 1 1] Server sets Quest Log open
  (set `self.QuestLogOpen` QuestLogOpen))

(event `ClientSetQuestLogOpen`
  (params (QuestLogOpen :type Boolean))
  ;[1 1 1] Client sets quest log open
  (set `self.QuestLogOpen` QuestLogOpen))

(event `ServerSetGuideBookOpen`
  (params (GuideBookOpen :type Boolean))
  ;[1 1 1] Server sets Guide Book Open
  (set `self.GuideBookOpen` GuideBookOpen))

(event `ClientSetGuideBookOpen`
  (params (GuideBookOpen :type Boolean))
  ;[1 1 1] Client sets Guide Book open
  (set `self.GuideBookOpen` GuideBookOpen))

(fn `AddJournalEntry`
  (params (EntryName :type Name))
  (locals (EntryFound :type Boolean))
  (bind _keys (`BlueprintMapLibrary.Map_Keys` (`self.JournalEntries`)))
  (for _array_element _keys
    (if (== _array_element (`local.EntryName`))
      (return)))
  (`BlueprintMapLibrary.Map_Add` (`self.JournalEntries`) (`local.EntryName`) true))

(fn `AttemptToAddItem`
  (params (InvItem :type "/Game/SurvivalGameKitV2/Blueprints/Other/Structs/S_InvItem Structure") (StackSearch :type Boolean) (ShowNotifications :type Boolean))
  (returns (RemainingItem :type Boolean) (RemainingInvItem :type "/Game/SurvivalGameKitV2/Blueprints/Other/Structs/S_InvItem Structure") (NewItemSlot :type "/Game/SurvivalGameKitV2/Blueprints/Other/Structs/S_InvSlotID Structure"))
  (locals (InvItemL :type "/Game/SurvivalGameKitV2/Blueprints/Other/Structs/S_InvItem Structure"))
  (bind (_remainingitem _remaininginvitem _newitemslot) (`parent.AttemptToAddItem` InvItem StackSearch ShowNotifications))
  (`self.Update Quest Items Count` InvItem)
  (return _remainingitem _remaininginvitem _newitemslot))

(fn `Close Journal`
  (bind _closeinventorysound (`self.CloseInventorySound`))
  (if (not (`self.UIOpen`))
    (set `self.JournalOpen` false)
    (`self.ServerSetJournalOpen` (`self.JournalOpen`))
    (`self.Journal`
      (:`then`
        (set `PlayerController.bShowMouseCursor` false (`GameplayStatics.GetPlayerController` 0))
        (`Controller.SetIgnoreLookInput` (`GameplayStatics.GetPlayerController` 0) false)
        (`WidgetBlueprintLibrary.SetInputMode_GameOnly` (`GameplayStatics.GetPlayerController` 0))
        (`Widget.RemoveFromParent` (`self.Journal`))
        (`/Engine/EditorBlueprintResources/StandardMacros.IsValid` _closeinventorysound
          (:`Is Valid`
            (`GameplayStatics.PlaySound2D` _closeinventorysound 1.0 1.0 0.0 null null))))
      (:`else`))))

(fn `CloseGenetics`
  (bind _closeinventorysound (`self.CloseInventorySound`))
  (if (not (`self.UIOpen`))
    (`self.EndInteraction`)
    (set `self.InventoryOpen` false)
    ;[1 1 1] Start game input
    (`self.PlayerHUD`
      (:`then`
        (set `PlayerController.bShowMouseCursor` false (`GameplayStatics.GetPlayerController` 0))
        (`WidgetBlueprintLibrary.CancelDragDrop`)
        (`Controller.SetIgnoreLookInput` (`GameplayStatics.GetPlayerController` 0) false)
        (`WidgetBlueprintLibrary.SetInputMode_GameOnly` (`GameplayStatics.GetPlayerController` 0))
        ;[1 1 1] Hide inventory screen
        (`/Game/SurvivalGameKitV2/Blueprints/Widgets/BP_InventoryHUD.CloseInventoryScreen` (`self.PlayerHUD`))
        ;[1 1 1] Clear interacted with component and call event bind
        (`self.InventoryToggled` (`self.InventoryOpen`))
        (set `self.ExtCookingComponent` null)
        (set `self.ExtCraftingComponent` null)
        (set `self.ExtInventoryComponent` null)
        (set `self.VenderComponent` null)
        (`/Engine/EditorBlueprintResources/StandardMacros.IsValid` _closeinventorysound
          (:`Is Valid`
            (`GameplayStatics.PlaySound2D` _closeinventorysound 1.0 1.0 0.0 null null))))
      (:`else`))))

(fn `CloseGuideBook`
  (bind _closeinventorysound (`self.CloseInventorySound`))
  (if (not (`self.UIOpen`))
    (set `self.GuideBookOpen` false)
    (`self.ServerSetGuideBookOpen` (`self.GuideBookOpen`))
    (`self.GuideBook`
      (:`then`
        (set `PlayerController.bShowMouseCursor` false (`GameplayStatics.GetPlayerController` 0))
        (`Controller.SetIgnoreLookInput` (`GameplayStatics.GetPlayerController` 0) false)
        (`WidgetBlueprintLibrary.SetInputMode_GameOnly` (`GameplayStatics.GetPlayerController` 0))
        (`Widget.RemoveFromParent` (`self.GuideBook`))
        (`/Engine/EditorBlueprintResources/StandardMacros.IsValid` _closeinventorysound
          (:`Is Valid`
            (`GameplayStatics.PlaySound2D` _closeinventorysound 1.0 1.0 0.0 null null))))
      (:`else`))))

(fn `ClosePlayerStats`
  (bind _closeinventorysound (`self.CloseInventorySound`))
  (if (not (`self.UIOpen`))
    (set `self.PlayerStatsOpen` false)
    (`self.ServerSetPlayerStatsOpen` (`self.PlayerStatsOpen`))
    (`self.PlayerStats`
      (:`then`
        (set `PlayerController.bShowMouseCursor` false (`GameplayStatics.GetPlayerController` 0))
        (`Controller.SetIgnoreLookInput` (`GameplayStatics.GetPlayerController` 0) false)
        (`WidgetBlueprintLibrary.SetInputMode_GameOnly` (`GameplayStatics.GetPlayerController` 0))
        (`Widget.RemoveFromParent` (`self.PlayerStats`))
        (`/Engine/EditorBlueprintResources/StandardMacros.IsValid` _closeinventorysound
          (:`Is Valid`
            (`GameplayStatics.PlaySound2D` _closeinventorysound 1.0 1.0 0.0 null null))))
      (:`else`))))

(fn `CloseQuestLog`
  (bind _closeinventorysound (`self.CloseInventorySound`))
  (if (`self.UIOpen`)
    _
    (elif (`self.QuestLogOpen`)
      (set `self.QuestLogOpen` false)
      (`self.ServerSetQuestLogOpen` (`self.QuestLogOpen`))
      (bind _asbp_tbsmaster_character (cast `/Game/TheBiogenSurvivor/Blueprints/Character/BP_TBSMasterCharacter` (`GameplayStatics.GetPlayerCharacter` 0)))
      (bind _bp_bpc_playerquestcomponent (`/Game/TheBiogenSurvivor/Blueprints/Character/BP_TBSMasterCharacter.BP_BPC_PlayerQuestComponent` _asbp_tbsmaster_character)
        (:`then`
          (`/Game/EasyQuests/Blueprints/BP_BPC_PlayerQuestComponent.Toggle Quest Log Visibility` _bp_bpc_playerquestcomponent)
          (`/Engine/EditorBlueprintResources/StandardMacros.IsValid` _closeinventorysound
            (:`Is Valid`
              (`GameplayStatics.PlaySound2D` _closeinventorysound 1.0 1.0 0.0 null null))))
        (:`else`)))))

(fn `ConsumeItem`
  (params (Item :type "/Game/SurvivalGameKitV2/Blueprints/Other/Structs/S_InvItem Structure"))
  (returns (Consumed :type Boolean))
  (locals (ItemConsumableDetails :type "/Game/SurvivalGameKitV2/Blueprints/Other/Structs/S_ConsumableDetails Structure"))
  (bind (_itemfound _itemdetails) (`/Game/SurvivalGameKitV2/Blueprints/Other/Interfaces/BP_SGKFunctions.SGK ItemDetails` Item))
  (if (`.HasUseAmount_52_D5C2AD8E4B9EB866F11B6BAF17E2BBE7` (break `/Game/SurvivalGameKitV2/Blueprints/Other/Structs/S_ConsumableDetails` (`.ItemDetails` (`/Game/SurvivalGameKitV2/Blueprints/Other/Interfaces/BP_SGKFunctions.SGK ItemConsumableDetails` Item))))
    (if (> (`.UseAmount_21_73BF7A6447A384E099761EA48F7DB753` (break `/Game/SurvivalGameKitV2/Blueprints/Other/Structs/S_InvItem` Item)) 0)
      ;[1 1 1] Check if item can be consumed
      (if _itemfound :!label _label
        ;[1 1 1] Gets consumable details based on mutations
        (bind _asbp_sgkcontroller (cast `/Game/SurvivalGameKitV2/Blueprints/Characters/BP_SGKController` (`self.GetOwner` self)))
        (bind (_consumable_details _found) (`/Game/TheBiogenSurvivor/Blueprints/Other/Interfaces/BP_TBSFunctions.TBS GetMutationConsumable` (`.ID_2_84C2CB8945979246059C568DCD463423` (break `/Game/SurvivalGameKitV2/Blueprints/Other/Structs/S_InvItem` (`local.Item`))) _asbp_sgkcontroller))
        (if _found
          (set `local.ItemConsumableDetails` _consumable_details)
          (else
            (set `local.ItemConsumableDetails` (`.ConsumableDetails_77_3E970B0D497E2A71D3B074A210E6F3F1` (break `/Game/SurvivalGameKitV2/Blueprints/Other/Structs/S_ItemDetails` _itemdetails)))))
        (if (`.CanConsume_1_F33B573C44E7F10E734CE98A8F8B397B` (break `/Game/SurvivalGameKitV2/Blueprints/Other/Structs/S_ConsumableDetails` (`local.ItemConsumableDetails`)))
          (`|ExecutionSequence`
            (:`then_0`
              ;[1 1 1] Effect players stats
              (`self.IncreaseHunger` (`.Hunger_9_0D90519F43945DD23F8A98A10994E8C6` (break `/Game/SurvivalGameKitV2/Blueprints/Other/Structs/S_ConsumableDetails` (`local.ItemConsumableDetails`))))
              (`self.IncreaseStamina` (`.Stamina_12_C4F7061C4ECC1EC288DC08B8F0EB32DD` (break `/Game/SurvivalGameKitV2/Blueprints/Other/Structs/S_ConsumableDetails` (`local.ItemConsumableDetails`))))
              (`self.IncreaseThirst` (`.Thirst_10_D9ED71A24C1DAC5DFF4104823F0A5337` (break `/Game/SurvivalGameKitV2/Blueprints/Other/Structs/S_ConsumableDetails` (`local.ItemConsumableDetails`))))
              (`self.IncreaseHealth` (`.Health_4_58F2B2E648683BE1B8D783B5F9DE5F26` (break `/Game/SurvivalGameKitV2/Blueprints/Other/Structs/S_ConsumableDetails` (`local.ItemConsumableDetails`)))))
            (:`then_1`
              ;[1 1 1] If stop bleeds then stop bleed timer
              (if (`.StopBleeding_34_8697A21F49FD77710EEA589D8104FE58` (break `/Game/SurvivalGameKitV2/Blueprints/Other/Structs/S_ConsumableDetails` (`local.ItemConsumableDetails`)))
                (`self.ClearBleed`)))
            (:`then_2`
              ;[1 1 1] Apply curing effects
              (bind _asbp_sgkcontroller_2 (cast `/Game/SurvivalGameKitV2/Blueprints/Characters/BP_SGKController` (`self.GetOwner` self)))
              (`/Game/TheBiogenSurvivor/Blueprints/Components/BP_DiseaseComponent.InfectionEvent` (`/Game/SurvivalGameKitV2/Blueprints/Characters/BP_SGKController.BP_DiseaseComponent` _asbp_sgkcontroller_2) (`.ID_2_84C2CB8945979246059C568DCD463423` (break `/Game/SurvivalGameKitV2/Blueprints/Other/Structs/S_InvItem` (`local.Item`)))))
            (:`then_3`
              ;[1 1 1] Apply curing effects
              (bind _asbp_sgkcontroller_3 (cast `/Game/SurvivalGameKitV2/Blueprints/Characters/BP_SGKController` (`self.GetOwner` self)))
              (`/Game/TheBiogenSurvivor/Blueprints/Components/BP_DiseaseComponent.CureEvent` (`/Game/SurvivalGameKitV2/Blueprints/Characters/BP_SGKController.BP_DiseaseComponent` _asbp_sgkcontroller_3) (`.ID_2_84C2CB8945979246059C568DCD463423` (break `/Game/SurvivalGameKitV2/Blueprints/Other/Structs/S_InvItem` (`local.Item`)))))
            (:`then_4`
              ;[1 1 1] Play consume sound
              (`self.PlayItemSound` (`.ID_2_84C2CB8945979246059C568DCD463423` (break `/Game/SurvivalGameKitV2/Blueprints/Other/Structs/S_InvItem` (`local.Item`))))
              (return true)))
          (else
            (`KismetSystemLibrary.PrintString` "ERROR : Item cannot be consumed \"Can Consume\" must be set to true in item list!")))))
    (else
      (goto _label))))

(fn `DropItemFromSlot`
  (params (SlotID :type "/Game/SurvivalGameKitV2/Blueprints/Other/Structs/S_InvSlotID Structure") (SpecialType :type "/Game/SurvivalGameKitV2/Blueprints/Other/Enum/E_SpecialSlotType Enum" :default "NewEnumerator0") (Split :type Boolean))
  (locals (InvItemL :type "/Game/SurvivalGameKitV2/Blueprints/Other/Structs/S_InvItem Structure"))
  (bind _invslot (`/Game/SurvivalGameKitV2/Blueprints/Other/Interfaces/BP_SGKFunctions.SGK InvSlotFromSlotID` SlotID))
  (set `local.InvItemL` (`/Game/SurvivalGameKitV2/Blueprints/Other/Interfaces/BP_SGKFunctions.SGK InvSlotItem` _invslot))
  (`parent.DropItemFromSlot` SlotID SpecialType Split)
  (`self.Update Quest Items Count` (`local.InvItemL`)))

(fn `FindSpawnPoint`
  (params (Random :type Boolean))
  (returns (SpawnLocation :type "Transform Structure"))
  (locals (PlayerStartsL :type "Array of PlayerStart Object Reference"))
  (bind _returnvalue (`Actor.GetTransform` (`|GetArrayItem` (`local.PlayerStartsL`) (`KismetMathLibrary.RandomIntegerInRange` 0 (- (`KismetArrayLibrary.Array_Length` (`local.PlayerStartsL`)) 1)))))
  (if (`KismetTextLibrary.TextIsEmpty` (`self.RespawnPointName`))
    _
    (elif (not (`local.Random`))
      (bind _outactors (`GameplayStatics.GetAllActorsOfClass` "/Game/TheBiogenSurvivor/Blueprints/BuildParts/BP_MasterProcessingBuildPart.BP_MasterProcessingBuildPart_C"))
      (for _array_element _outactors
        (if (`KismetTextLibrary.EqualEqual_TextText` (`/Game/TheBiogenSurvivor/Blueprints/Components/BP_ProcessingComponent.RespawnPointName` (`/Game/TheBiogenSurvivor/Blueprints/BuildParts/BP_MasterProcessingBuildPart.BP_ProcessingComponent` _array_element)) (`self.RespawnPointName`))
          (bind (_returnvalue_location _returnvalue_rotation) (`KismetMathLibrary.BreakTransform` (`SceneComponent.K2_GetComponentToWorld` (`/Game/TheBiogenSurvivor/Blueprints/BuildParts/BP_MasterProcessingBuildPart.RespawnLocation` _array_element))))
          (return (`KismetMathLibrary.MakeTransform` _returnvalue_location (`KismetMathLibrary.MakeRotator` 0.0 0.0 (.yaw _returnvalue_rotation))))))))
  (bind _outactors_2 (`GameplayStatics.GetAllActorsOfClass` "/Script/Engine.PlayerStart"))
  (bind _output_get (set `local.PlayerStartsL` _outactors_2))
  (if (> (`KismetArrayLibrary.Array_Length` _output_get) 0)
    (return (`KismetMathLibrary.MakeTransform` (.location _returnvalue) (`KismetMathLibrary.MakeRotator` 0.0 0.0 (.yaw (.rotation _returnvalue)))))
    (else
      (`KismetSystemLibrary.PrintString` "ERROR : You have no PlayerStart actors in your level, these are used for \nrespawning you can find the actor in the Modes panel in the Basic section. Player will be spawned at 0,0,0 now" true true (struct :`R` 1.0 :`A` 1.0) 20.0)
      (return (`KismetMathLibrary.MakeTransform` (0.0 0.0 0.0))))))

(fn `HasNewJournalEntry`
  (returns (NewEntry :type Boolean))
  (bind _values (`BlueprintMapLibrary.Map_Values` (`self.JournalEntries`)))
  (for _array_element _values
    (if _array_element
      (return true)))
  (return false))

(fn `InitializePlayerInventory`
  ;[1 1 1] Add self to using players
  (`self.AddUsingPlayer` self)
  ;[1 1 1] Set Character and building component
  (bind _output_get (set `self.SGKCharacter` (`self.OwningCharacter`)))
  (set `self.PlayerBuildingComponent` (`Actor.GetComponentByClass` (`Pawn.GetController` _output_get) "/Game/SurvivalGameKitV2/Components/BP_PlayerBuildingComponent.BP_PlayerBuildingComponent_C"))
  ;[1 1 1] Start state timers and if not server run LookAtTrace timer
  (`self.IsServer`
    (:`True`
      (`KismetSystemLibrary.K2_SetTimer` null "HungerState" (`self.HungerReductionTime`) true 1.0)
      (`KismetSystemLibrary.K2_SetTimer` null "ThirstState" (`self.ThirstReductionTime`) true 1.0)
      (`KismetSystemLibrary.K2_SetTimer` null "StarvationState" (`self.StarvationDamageTime`) true 1.0)
      (`KismetSystemLibrary.K2_SetTimer` null "DehydrationState" (`self.DehydrationDamageTime`) true 1.0)
      (`KismetSystemLibrary.K2_SetTimer` null "SetEnvironmentEffects" (`self.TemperatureTickRate`) true)
      (`KismetSystemLibrary.K2_SetTimer` null "AdjustBodyTemperature" (`self.TemperatureTickRate`) true)
      ;[1 1 1] Start health regen timer if UseHealthRegeneration is true
      (if (and (> (`self.RegenerationTickTime`) 0.0) (`self.UseHealthRegeneration`))
        (`KismetSystemLibrary.K2_SetTimer` null "HealthRegeneration" (`self.RegenerationTickTime`) true 1.0))
      ;[1 1 1] If single player or locally controlled run LookAtTrace
      (if (or (`Pawn.IsLocallyControlled` (`self.OwningCharacter`)) (`KismetSystemLibrary.IsStandalone`))
        (`KismetSystemLibrary.K2_SetTimer` null "LookAtTrace" 0.1 true)))
    (:`False`
      (`KismetSystemLibrary.K2_SetTimer` null "LookAtTrace" 0.1 true))))

(fn `MoveItem`
  (params (StartSlotID :type "/Game/SurvivalGameKitV2/Blueprints/Other/Structs/S_InvSlotID Structure") (EndSlotID :type "/Game/SurvivalGameKitV2/Blueprints/Other/Structs/S_InvSlotID Structure") (Rotated :type Boolean) (Split :type Boolean) (SpecialType :type "/Game/SurvivalGameKitV2/Blueprints/Other/Enum/E_SpecialSlotType Enum" :default "NewEnumerator0") (ShowNotifications :type Boolean))
  (returns (ItemMoved :type Boolean))
  (locals (InvItemL :type "/Game/SurvivalGameKitV2/Blueprints/Other/Structs/S_InvItem Structure"))
  (bind _invslot (`/Game/SurvivalGameKitV2/Blueprints/Other/Interfaces/BP_SGKFunctions.SGK InvSlotFromSlotID` StartSlotID))
  (set `local.InvItemL` (`/Game/SurvivalGameKitV2/Blueprints/Other/Interfaces/BP_SGKFunctions.SGK InvSlotItem` _invslot))
  (bind _itemmoved (`parent.MoveItem` StartSlotID EndSlotID Rotated Split SpecialType ShowNotifications))
  (if _itemmoved
    (`self.Update Quest Items Count` (`local.InvItemL`)))
  (return _itemmoved))

(fn `OpenGenetics`
  (bind _openinventorysound (`self.OpenInventorySound`))
  (`self.PlayerHUD`
    (:`then`
      (if (not (`self.UIOpen`))
        (set `self.InventoryOpen` true)
        ;[1 1 1] Start UI input mode
        (set `PlayerController.bShowMouseCursor` true (`GameplayStatics.GetPlayerController` 0))
        (`Controller.SetIgnoreLookInput` (`GameplayStatics.GetPlayerController` 0) true)
        (`WidgetBlueprintLibrary.SetInputMode_GameAndUIEx` (`GameplayStatics.GetPlayerController` 0) (`self.PlayerHUD`) "DoNotLock" false)
        ;[1 1 1] Call server update inventory open and call event bind
        (`self.ServerSetInventoryOpen` (`self.InventoryOpen`))
        (`self.InventoryToggled` (`self.InventoryOpen`))
        (`/Game/SurvivalGameKitV2/Components/BP_PlayerBuildingComponent.ClientRemoveMenu` (`self.PlayerBuildingComponent`))
        (`/Engine/EditorBlueprintResources/StandardMacros.IsValid` _openinventorysound
          (:`Is Valid`
            (`GameplayStatics.PlaySound2D` _openinventorysound 1.0 1.0 0.0 null null)))))
    (:`else`)))

(fn `OpenGuideBook`
  (bind _openinventorysound (`self.OpenInventorySound`))
  (`self.GuideBook`
    (:`then`
      _)
    (:`else`
      (bind _returnvalue (`|CreateWidget` "/Game/TheBiogenSurvivor/Blueprints/Widgets/BP_Guides.BP_Guides_C" (`GameplayStatics.GetPlayerController` 0)))
      (bind _output_get (set `self.GuideBook` _returnvalue))))
  (if (`self.UIOpen`)
    _
    (else
      _))
  (`self.CloseInventory`)
  (`/Game/SurvivalGameKitV2/Components/BP_PlayerBuildingComponent.ClientRemoveMenu` (`self.PlayerBuildingComponent`))
  (set `self.GuideBookOpen` true)
  (set `PlayerController.bShowMouseCursor` true (`GameplayStatics.GetPlayerController` 0))
  (`Controller.SetIgnoreLookInput` (`GameplayStatics.GetPlayerController` 0) true)
  (`UserWidget.AddToViewport` _output_get 0)
  (`WidgetBlueprintLibrary.SetInputMode_GameAndUIEx` (`GameplayStatics.GetPlayerController` 0) (`self.GuideBook`) "DoNotLock" false)
  (`self.ServerSetGuideBookOpen` (`self.GuideBookOpen`))
  (`/Engine/EditorBlueprintResources/StandardMacros.IsValid` _openinventorysound
    (:`Is Valid`
      (`GameplayStatics.PlaySound2D` _openinventorysound 1.0 1.0 0.0 null null))))

(fn `OpenInventory`
  (`self.Close Journal`)
  (`self.ClosePlayerStats`)
  (`self.CloseQuestLog`)
  (`parent.OpenInventory`))

(fn `OpenJournal`
  (bind _openinventorysound (`self.OpenInventorySound`))
  (`self.Journal`
    (:`then`
      _)
    (:`else`
      (bind _returnvalue (`|CreateWidget` "/Game/TheBiogenSurvivor/Blueprints/Widgets/BP_InfoLog.BP_InfoLog_C" (`GameplayStatics.GetPlayerController` 0)))
      (bind _output_get (set `self.Journal` _returnvalue))))
  (if (`self.UIOpen`)
    _
    (else
      _))
  (`self.CloseInventory`)
  (`/Game/SurvivalGameKitV2/Components/BP_PlayerBuildingComponent.ClientRemoveMenu` (`self.PlayerBuildingComponent`))
  (`self.CloseQuestLog`)
  (`self.ClosePlayerStats`)
  (set `self.JournalOpen` true)
  (set `PlayerController.bShowMouseCursor` true (`GameplayStatics.GetPlayerController` 0))
  (`Controller.SetIgnoreLookInput` (`GameplayStatics.GetPlayerController` 0) true)
  (`UserWidget.AddToViewport` _output_get 0)
  (`WidgetBlueprintLibrary.SetInputMode_GameAndUIEx` (`GameplayStatics.GetPlayerController` 0) (`self.Journal`) "DoNotLock" false)
  (`self.ServerSetJournalOpen` (`self.JournalOpen`))
  (`/Engine/EditorBlueprintResources/StandardMacros.IsValid` _openinventorysound
    (:`Is Valid`
      (`GameplayStatics.PlaySound2D` _openinventorysound 1.0 1.0 0.0 null null))))

(fn `OpenPlayerStats`
  (bind _openinventorysound (`self.OpenInventorySound`))
  (`self.PlayerStats`
    (:`then`
      _)
    (:`else`
      (bind _returnvalue (`|CreateWidget` "/Game/TheBiogenSurvivor/Blueprints/Widgets/BP_CharacterStats.BP_CharacterStats_C" (`GameplayStatics.GetPlayerController` 0)))
      (bind _output_get (set `self.PlayerStats` _returnvalue))))
  (if (not (`self.UIOpen`))
    (`self.CloseInventory`)
    (`/Game/SurvivalGameKitV2/Components/BP_PlayerBuildingComponent.ClientRemoveMenu` (`self.PlayerBuildingComponent`))
    (`self.CloseQuestLog`)
    (`self.Close Journal`)
    (set `self.PlayerStatsOpen` true)
    (set `PlayerController.bShowMouseCursor` true (`GameplayStatics.GetPlayerController` 0))
    (`Controller.SetIgnoreLookInput` (`GameplayStatics.GetPlayerController` 0) true)
    (`UserWidget.AddToViewport` _output_get 0)
    (`WidgetBlueprintLibrary.SetInputMode_GameAndUIEx` (`GameplayStatics.GetPlayerController` 0) (`self.PlayerStats`) "DoNotLock" false)
    (`self.ServerSetPlayerStatsOpen` (`self.PlayerStatsOpen`))
    (`/Game/TheBiogenSurvivor/Blueprints/Widgets/BP_CharacterStats.InitializeStatsBox` (`self.PlayerStats`))
    (`/Game/TheBiogenSurvivor/Blueprints/Widgets/BP_CharacterStats.InitializeStatusEffectsBox` (`self.PlayerStats`))
    (`/Engine/EditorBlueprintResources/StandardMacros.IsValid` _openinventorysound
      (:`Is Valid`
        (`GameplayStatics.PlaySound2D` _openinventorysound 1.0 1.0 0.0 null null)))))

(fn `OpenQuestLog`
  (bind _openinventorysound (`self.OpenInventorySound`))
  (if (not (`self.UIOpen`))
    (`self.CloseInventory`)
    (`/Game/SurvivalGameKitV2/Components/BP_PlayerBuildingComponent.ClientRemoveMenu` (`self.PlayerBuildingComponent`))
    (`self.Close Journal`)
    (`self.ClosePlayerStats`)
    (set `self.QuestLogOpen` true)
    (bind _asbp_tbsmaster_character (cast `/Game/TheBiogenSurvivor/Blueprints/Character/BP_TBSMasterCharacter` (`GameplayStatics.GetPlayerCharacter` 0)))
    (bind _bp_bpc_playerquestcomponent (`/Game/TheBiogenSurvivor/Blueprints/Character/BP_TBSMasterCharacter.BP_BPC_PlayerQuestComponent` _asbp_tbsmaster_character)
      (:`then`
        (`/Game/EasyQuests/Blueprints/BP_BPC_PlayerQuestComponent.Toggle Quest Log Visibility` _bp_bpc_playerquestcomponent)
        (`self.ServerSetQuestLogOpen` (`self.QuestLogOpen`))
        (`/Engine/EditorBlueprintResources/StandardMacros.IsValid` _openinventorysound
          (:`Is Valid`
            (`GameplayStatics.PlaySound2D` _openinventorysound 1.0 1.0 0.0 null null))))
      (:`else`))))

(fn `ToggleGenetics`
  (if (`self.InventoryOpen`)
    (`self.CloseGenetics`)
    (else
      (`self.OpenGenetics`))))

(fn `ToggleGuideBook`
  (bind _guidebook (`self.GuideBook`))
  (bind _guidebook_2 (`self.GuideBook`))
  (if (`self.GuideBookOpen`)
    (if (== (`WidgetSwitcher.GetActiveWidget` (`/Game/TheBiogenSurvivor/Blueprints/Widgets/BP_Guides.WidgetSwitcher` _guidebook)) (`/Game/TheBiogenSurvivor/Blueprints/Widgets/BP_Guides.BP_GuidePage` _guidebook))
      (`self.CloseGuideBook`)
      (else
        (`WidgetSwitcher.SetActiveWidget` (`/Game/TheBiogenSurvivor/Blueprints/Widgets/BP_Guides.WidgetSwitcher` _guidebook_2) (`/Game/TheBiogenSurvivor/Blueprints/Widgets/BP_Guides.BP_GuidePage` _guidebook_2) :!label _label)))
    (else
      (`self.OpenGuideBook`)
      (goto _label))))

(fn `ToggleJournal`
  (bind _guidebook (`self.GuideBook`))
  (bind _guidebook_2 (`self.GuideBook`))
  (if (`self.GuideBookOpen`)
    (if (== (`WidgetSwitcher.GetActiveWidget` (`/Game/TheBiogenSurvivor/Blueprints/Widgets/BP_Guides.WidgetSwitcher` _guidebook)) (`/Game/TheBiogenSurvivor/Blueprints/Widgets/BP_Guides.BP_InfoLog` _guidebook))
      (`self.CloseGuideBook`)
      (else
        (`WidgetSwitcher.SetActiveWidget` (`/Game/TheBiogenSurvivor/Blueprints/Widgets/BP_Guides.WidgetSwitcher` _guidebook_2) (`/Game/TheBiogenSurvivor/Blueprints/Widgets/BP_Guides.BP_InfoLog` _guidebook_2) :!label _label)))
    (else
      (`self.OpenGuideBook`)
      (goto _label))))

(fn `TogglePlayerStats`
  (bind _guidebook (`self.GuideBook`))
  (bind _guidebook_2 (`self.GuideBook`))
  (if (`self.GuideBookOpen`)
    (if (== (`WidgetSwitcher.GetActiveWidget` (`/Game/TheBiogenSurvivor/Blueprints/Widgets/BP_Guides.WidgetSwitcher` _guidebook)) (`/Game/TheBiogenSurvivor/Blueprints/Widgets/BP_Guides.BP_CharacterStats` _guidebook))
      (`self.CloseGuideBook`)
      (else
        (`WidgetSwitcher.SetActiveWidget` (`/Game/TheBiogenSurvivor/Blueprints/Widgets/BP_Guides.WidgetSwitcher` _guidebook_2) (`/Game/TheBiogenSurvivor/Blueprints/Widgets/BP_Guides.BP_CharacterStats` _guidebook_2) :!label _label)))
    (else
      (`self.OpenGuideBook`)
      (goto _label))))

(fn `ToggleQuestLog`
  (bind _guidebook (`self.GuideBook`))
  (bind _guidebook_2 (`self.GuideBook`))
  (if (`self.GuideBookOpen`)
    (if (== (`WidgetSwitcher.GetActiveWidget` (`/Game/TheBiogenSurvivor/Blueprints/Widgets/BP_Guides.WidgetSwitcher` _guidebook)) (`/Game/TheBiogenSurvivor/Blueprints/Widgets/BP_Guides.WBP_QuestLog` _guidebook))
      (`self.CloseGuideBook`)
      (else
        (`WidgetSwitcher.SetActiveWidget` (`/Game/TheBiogenSurvivor/Blueprints/Widgets/BP_Guides.WidgetSwitcher` _guidebook_2) (`/Game/TheBiogenSurvivor/Blueprints/Widgets/BP_Guides.WBP_QuestLog` _guidebook_2) :!label _label)))
    (else
      (`self.OpenGuideBook`)
      (goto _label))))

(fn `Update Quest Items Count`
  (params (InvItem :type "/Game/SurvivalGameKitV2/Blueprints/Other/Structs/S_InvItem Structure"))
  (bind (_componentwasfound_ _questcomponent) (`/Game/EasyQuests/Blueprints/BPL/BP_BPL_Quests.GetQuestComponent`))
  (bind _amount (`/Game/TheBiogenSurvivor/Blueprints/Other/Interfaces/BP_TBSFunctions.TBSGet Total Amount in Inventory` InvItem self))
  (if _componentwasfound_
    (for _array_element (`/Game/EasyQuests/Blueprints/BP_BPC_PlayerQuestComponent.ActiveQuests` _questcomponent)
      (`/Game/EasyQuests/Blueprints/BP_BPC_PlayerQuestComponent.SetObjectiveAmount` _questcomponent (`.QuestID_2_E9DD1B8B405D0E58BEEA3AA29273D9A7` (break `/Game/EasyQuests/Blueprints/Structures/ST_Quest_Info` _array_element)) (`.ID_2_84C2CB8945979246059C568DCD463423` (break `/Game/SurvivalGameKitV2/Blueprints/Other/Structs/S_InvItem` (`local.InvItem`))) _amount))))