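; Disease component for the player controller that handles infection, progression, cures and resistance.
; A looping timer advances or regresses each active disease, then drains health, stamina, thirst and hunger scaled by progress.
; Infection and cure events read data table rows: resistance lowers infection chance, while cures add resistance, reduce progress and may trigger remission.
; Remissive diseases that reach zero are dropped and grant survival resistance.
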(event `self.ReceiveBeginPlay`
  (`KismetSystemLibrary.K2_SetTimer` null "DiseaseTickEvent" 10.0 true))

(fn `Add Resistance`
  (params (DiseaseName :type Name) (DiseaseResitance :type "Float (double-precision)"))
  (bind (_value _returnvalue) (`BlueprintMapLibrary.Map_Find` (`self.DiseaseResistances`) DiseaseName))
  ;[1 1 1] Add resistance
  (if _returnvalue
    (`BlueprintMapLibrary.Map_Add` (`self.DiseaseResistances`) (`local.DiseaseName`) (`KismetMathLibrary.FClamp` (+ DiseaseResitance _value)))
    (else
      (`BlueprintMapLibrary.Map_Add` (`self.DiseaseResistances`) (`local.DiseaseName`) DiseaseResitance))))

(fn `CureEvent`
  (params (ItemName :type Name))
  (locals (DiseaseNameL :type Name) (ResistanceL :type "Float (double-precision)"))
  (bind (_value _returnvalue) (`BlueprintMapLibrary.Map_Find` (`self.ActiveDiseases`) (`local.DiseaseNameL`)))
  (bind (_remissive _progress) (break `/Game/TheBiogenSurvivor/Blueprints/Other/Structs/S_DiseaseProgressDetails` _value))
  (bind _returnvalue_2 (`|GetDataTableRow` "/Game/TheBiogenSurvivor/Blueprints/Diseases/DiseaseCureList.DiseaseCureList" ItemName)
    (:`then`
      (for _array_element (`.CureDetails_14_0813D9B543E67422902C20A98E4D76B0` (break `/Game/TheBiogenSurvivor/Blueprints/Other/Structs/S_DiseaseCure` _returnvalue_2))
        (bind (_disease _progressiondecrease _regressionchance _resistanceincrease) (break `/Game/TheBiogenSurvivor/Blueprints/Other/Structs/S_CureDetails` _array_element))
        (bind _output_get (set `local.DiseaseNameL` (`.RowName` (break `DataTableRowHandle` _disease))))
        (`self.Add Resistance` _output_get _resistanceincrease)
        (if _returnvalue
          (`BlueprintMapLibrary.Map_Add` (`self.ActiveDiseases`) (`local.DiseaseNameL`) (make `/Game/TheBiogenSurvivor/Blueprints/Other/Structs/S_DiseaseProgressDetails` (or _remissive (< (`KismetMathLibrary.RandomFloat`) _regressionchance)) (`KismetMathLibrary.FClamp` (- _progress _progressiondecrease))))
          (else
            (`KismetSystemLibrary.PrintString` "Could not find disease when processing cure")))))))

(fn `DiseaseTickEvent`
  (`self.ProgessDiseases`)
  (`self.TriggerDiseaseEffects`))

(fn `InfectionEvent`
  (params (InfectionEvent :type Name))
  (locals (DiseaseNameL :type Name) (DiseaseHasEvent :type Boolean))
  (bind (_value _returnvalue) (`BlueprintMapLibrary.Map_Find` (`self.ActiveDiseases`) (`local.DiseaseNameL`)))
  (bind _returnvalue_2 (`|GetDataTableRow` "/Game/TheBiogenSurvivor/Blueprints/Diseases/DiseaseCureList.DiseaseCureList" InfectionEvent)
    (:`then`
      (for _array_element (`.InfectionDetails_22_449C2E4149EF26408BA32AA441041268` (break `/Game/TheBiogenSurvivor/Blueprints/Other/Structs/S_DiseaseCure` _returnvalue_2))
        (bind (_disease _infectionchance _progression) (break `/Game/TheBiogenSurvivor/Blueprints/Other/Structs/S_InfectionDetails` _array_element))
        (set `local.DiseaseNameL` (`.RowName` (break `DataTableRowHandle` _disease)))
        (if (<= (`KismetMathLibrary.RandomFloat`) (* _infectionchance (- 1.0 (`BlueprintMapLibrary.Map_Find` (`self.DiseaseResistances`) (`local.DiseaseNameL`)))))
          (if _returnvalue
            (`BlueprintMapLibrary.Map_Add` (`self.ActiveDiseases`) (`local.DiseaseNameL`) (make `/Game/TheBiogenSurvivor/Blueprints/Other/Structs/S_DiseaseProgressDetails` false (`KismetMathLibrary.FClamp` (+ (`.Progress_4_31983FA64C8D039E80A6E5BE1B5827FB` (break `/Game/TheBiogenSurvivor/Blueprints/Other/Structs/S_DiseaseProgressDetails` _value)) _progression))))
            (else
              (`BlueprintMapLibrary.Map_Add` (`self.ActiveDiseases`) (`local.DiseaseNameL`) (make `/Game/TheBiogenSurvivor/Blueprints/Other/Structs/S_DiseaseProgressDetails` false _progression))
              (bind _playerinventory (`self.GetPlayerInventory`)
                (:`NewParam`
                  (`/Game/TheBiogenSurvivor/Blueprints/Components/BP_TBS_PlayerInventory.AddJournalEntry` _playerinventory "Diseases"))))))))))

(fn `InitializeDiseaseComponent`
  (`BlueprintMapLibrary.Map_Clear` (`self.ActiveDiseases`))
  (`BlueprintMapLibrary.Map_Clear` (`self.DiseaseResistances`)))

(fn `ProgessDiseases`
  (locals (DiseaseNameL :type Name) (DiseaseProgressL :type "Map of Name to /Game/TheBiogenSurvivor/Blueprints/Other/Structs/S_DiseaseProgressDetails Structure") (ResistanceL :type "Float (double-precision)"))
  (bind (_remissive _progress) (break `/Game/TheBiogenSurvivor/Blueprints/Other/Structs/S_DiseaseProgressDetails` (`BlueprintMapLibrary.Map_Find` (`self.ActiveDiseases`) (`local.DiseaseNameL`))))
  (bind _keys (`BlueprintMapLibrary.Map_Keys` (`self.ActiveDiseases`)))
  (for _array_element _keys
    (bind _output_get (set `local.DiseaseNameL` _array_element))
    (bind _returnvalue (`|GetDataTableRow` "/Game/TheBiogenSurvivor/Blueprints/Diseases/DiseaseDetailsList.DiseaseDetailsList" _output_get)
      (:`then`
        (if _remissive
          (bind (_name _shortname _description _progressionrate _effects _resistanceonsurvival) (break `/Game/TheBiogenSurvivor/Blueprints/Other/Structs/S_DiseaseDetails` _returnvalue))
          (bind _returnvalue_2 (`KismetMathLibrary.FClamp` (- (`.Progress_4_31983FA64C8D039E80A6E5BE1B5827FB` (break `/Game/TheBiogenSurvivor/Blueprints/Other/Structs/S_DiseaseProgressDetails` (`BlueprintMapLibrary.Map_Find` (`self.ActiveDiseases`) (`local.DiseaseNameL`)))) _progressionrate)))
          ;[1 1 1] Disease is in remission. Decrease progress and remove from active diseases in cured
          (if (> _returnvalue_2 0.0)
            (`BlueprintMapLibrary.Map_Add` (`local.DiseaseProgressL`) (`local.DiseaseNameL`) (make `/Game/TheBiogenSurvivor/Blueprints/Other/Structs/S_DiseaseProgressDetails` true _returnvalue_2))
            (else
              (`self.Add Resistance` (`local.DiseaseNameL`) _resistanceonsurvival)))
          (else
            ;[1 1 1] Disease is not in remission, so increase the progress
            (`BlueprintMapLibrary.Map_Add` (`local.DiseaseProgressL`) (`local.DiseaseNameL`) (make `/Game/TheBiogenSurvivor/Blueprints/Other/Structs/S_DiseaseProgressDetails` false (`KismetMathLibrary.FClamp` (+ _progressionrate _progress)))))))))
  (set `self.ActiveDiseases` (`local.DiseaseProgressL`)))

(fn `TriggerDiseaseEffects`
  (locals (DiseaseNameL :type Name))
  (bind (_remissive _progress) (break `/Game/TheBiogenSurvivor/Blueprints/Other/Structs/S_DiseaseProgressDetails` (`BlueprintMapLibrary.Map_Find` (`self.ActiveDiseases`) (`local.DiseaseNameL`))))
  (bind _keys (`BlueprintMapLibrary.Map_Keys` (`self.ActiveDiseases`)))
  (for _array_element _keys
    (bind _output_get (set `local.DiseaseNameL` _array_element))
    (bind _returnvalue (`|GetDataTableRow` "/Game/TheBiogenSurvivor/Blueprints/Diseases/DiseaseDetailsList.DiseaseDetailsList" _output_get)
      (:`then`
        (bind _playerinventory (`self.GetPlayerInventory`)
          (:`NewParam`
            (bind (_hungerdrainamount _thirstdrainamount _staminadrainamount _healthdrainamount) (break `/Game/TheBiogenSurvivor/Blueprints/Other/Structs/S_DiseaseEffects` (`.Effects_25_484197FB44A7FBBA29E0F69B5A86412B` (break `/Game/TheBiogenSurvivor/Blueprints/Other/Structs/S_DiseaseDetails` _returnvalue))))
            (`/Game/SurvivalGameKitV2/Blueprints/Components/BP_PlayerInventory.DecreaseHealth` _playerinventory (`KismetMathLibrary.Conv_Int64ToInt` (`KismetMathLibrary.Round64` (* _healthdrainamount _progress))) false)
            (`/Game/SurvivalGameKitV2/Blueprints/Components/BP_PlayerInventory.DecreaseStamina` _playerinventory (* _staminadrainamount _progress))
            (`/Game/SurvivalGameKitV2/Blueprints/Components/BP_PlayerInventory.DecreaseThirst` _playerinventory (* _thirstdrainamount _progress))
            (`/Game/SurvivalGameKitV2/Blueprints/Components/BP_PlayerInventory.DecreaseHunger` _playerinventory (* _hungerdrainamount _progress))))))))