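; BP_QuestCollectable is a component that controls the quest world marker on a collectable item.
; On BeginPlay it finds the quest component, binds to tracked-quest changes and points the WBP_WorldMarker widget at its owner.
; UpdateWorldMarker hides the marker, then shows it only if the owning BP_StaticMasterItem's row name matches the quest's current, marker-enabled objective and the quest is not aborted.
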(event `self.ReceiveBeginPlay`
  (bind (_componentwasfound_ _questcomponent) (`/Game/EasyQuests/Blueprints/BPL/BP_BPL_Quests.GetQuestComponent`))
  (if _componentwasfound_
    (bind _output_get (set `self.QuestComponent` _questcomponent))
    (add `/Game/EasyQuests/Blueprints/BP_BPC_PlayerQuestComponent.OnTrackedQuestChanged` _output_get (`|CreateDelegate` :!event `UpdateWorldMarker`))
    (`self.UpdateWorldMarker` "None")
    (bind _worldmarker (`self.WorldMarker`)
      (:`then`
        (bind _aswbp_world_marker (cast `/Game/EasyQuests/Widgets/WBP_WorldMarker` (`WidgetComponent.GetUserWidgetObject` _worldmarker)))
        (set `/Game/EasyQuests/Widgets/WBP_WorldMarker.Actor` (`self.GetOwner`) _aswbp_world_marker))
      (:`else`))
    (else
      (`KismetSystemLibrary.PrintString` "Quest Component was not found." true true (struct :`R` 1.0 :`G` 0.052861 :`A` 1.0)))))

(fn `UpdateWorldMarker`
  (params (QuestID :type Name) (Quest :type "/Game/EasyQuests/Blueprints/Structures/ST_Quest_Info Structure"))
  (bind (_foundobjective_ _foundobjectiveinfo) (`/Game/EasyQuests/Blueprints/BP_BPC_PlayerQuestComponent.GetCurrentObjectiveForActiveQuest` (`self.QuestComponent`) (`local.QuestID`)))
  (bind _worldmarker (`self.WorldMarker`)
    (:`then`
      (`SceneComponent.SetVisibility` _worldmarker false false)
      (if (== (`.QuestID_2_E9DD1B8B405D0E58BEEA3AA29273D9A7` (break `/Game/EasyQuests/Blueprints/Structures/ST_Quest_Info` (`local.Quest`))) (`local.QuestID`))
        (for _array_element (`.Objectives_21_50C63F1D4C80B7AA25F0B7B40D0F2E3D` (break `/Game/EasyQuests/Blueprints/Structures/ST_Quest_Info` (`local.Quest`)))
          (bind _asbp_static_master_item (cast `/Game/SurvivalGameKitV2/Blueprints/Items/WorldItems/BP_StaticMasterItem` (`self.GetOwner`)))
          (set `self.ObjectiveID` (`.RowName` (break `DataTableRowHandle` (`/Game/SurvivalGameKitV2/Blueprints/Items/WorldItems/BP_StaticMasterItem.Item` _asbp_static_master_item))))
          (if (and (== (`.Objective_ID_7_60CB1B1749DC486E0E91F796FB540B67` (break `/Game/EasyQuests/Blueprints/Structures/ST_Quest_Objectives` _array_element)) (`self.ObjectiveID`)) (`.HasWorldMarker?_29_8F94CDC742A85DD762B02897AC787295` (break `/Game/EasyQuests/Blueprints/Structures/ST_Quest_Objectives` _array_element)) _foundobjective_ (== (`.Objective_ID_7_60CB1B1749DC486E0E91F796FB540B67` (break `/Game/EasyQuests/Blueprints/Structures/ST_Quest_Objectives` _foundobjectiveinfo)) (`self.ObjectiveID`)) (not (`/Game/EasyQuests/Blueprints/BP_BPC_PlayerQuestComponent.WasQuestAborted?` (`self.QuestComponent`) (`local.QuestID`))))
            (`SceneComponent.SetVisibility` (`self.WorldMarker`) true false)
            (return)))
        (else
          (`KismetSystemLibrary.PrintString` "Not Quest ID"))))
    (:`else`)))