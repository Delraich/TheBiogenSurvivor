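; Player controller component that manages a survivor's genetic mutations, birth defects and cancers, and opens the biogenetics research menu through server-to-client events.
; Next mutations are merged and applied over inventory class defaults to become active.
; Random data-table birth defects modify current stats and post-process vision.
; Mutation events can randomly trigger cancers, which a looping timer advances through stages, stacking each stage's stat effects.
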(event `self.ReceiveBeginPlay`
  (`parent.ReceiveBeginPlay`)
  (`KismetSystemLibrary.K2_SetTimer` null "GrowCancers" 10.0 true))

(event `ServerOpenBiogeneticsMenu`
  (params (ProcessorInventory :type "/Game/SurvivalGameKitV2/Blueprints/Components/BP_MasterInventory Object Reference"))
  (bind _extprocessingcomponent (`self.ExtProcessingComponent`))
  ;[1 1 1] Server opens biogenetics menu
  (bind _output_get (set `self.ExtProcessingComponent` ProcessorInventory))
  (bind _inventory (`self.PlayerInventory`)
    (:`exec`
      (set `/Game/SurvivalGameKitV2/Blueprints/Components/BP_PlayerInventory.InteractedActor` (`self.GetOwner` _output_get) _inventory)
      (`/Game/SurvivalGameKitV2/Blueprints/Components/BP_MasterInventory.AddUsingPlayer` _extprocessingcomponent _inventory)
      (`self.ClientOpenBiogeneticsMenu` _extprocessingcomponent))))

(event `ClientOpenBiogeneticsMenu`
  (params (ProcessingComponent :type "/Game/SurvivalGameKitV2/Blueprints/Components/BP_MasterInventory Object Reference"))
  ;[1 1 1] Client opens biogenetic menu
  (bind _output_get (set `self.ExtProcessingComponent` ProcessingComponent))
  (`self.OpenBiogeneticsMenu` _output_get))

(event `ClientRefreshResearchList`
  ;[1 1 1] Refresh the research list
  (bind _inventory (`self.PlayerInventory`)
    (:`exec`
      (bind _playerhud (`/Game/SurvivalGameKitV2/Blueprints/Components/BP_PlayerInventory.PlayerHUD` _inventory))
      (`/Engine/EditorBlueprintResources/StandardMacros.IsValid` _playerhud
        (:`Is Valid`
          (`/Game/TheBiogenSurvivor/Blueprints/Widgets/BP_BiogeneticsInterface.PopulateMutrationsList` (`/Game/SurvivalGameKitV2/Blueprints/Widgets/BP_InventoryHUD.BP_BiogeneticsInterface` _playerhud) "NewEnumerator0" null))))))

(fn `ApplyStatModifiers`
  (params (MutationDetails :type "/Game/TheBiogenSurvivor/Blueprints/Other/Structs/S_MutationDetails Structure"))
  (bind (_name _shortname _description _type _mutationicon _maxhungerdelta _hungerreductiondelta _hungerreductiontimedelta _maxthirstdelta _thirstreductiondelta _thirstreductiontimedelta _maxhealthdelta _maxstaminadelta _staminarechargedelta _movementspeeddelta _usehealthregen _healthregenamount _healthregenminhunger _healthregenminthirst _healthregenticktime _falldamagedelta) (break `/Game/TheBiogenSurvivor/Blueprints/Other/Structs/S_MutationDetails` MutationDetails))
  (bind _inventory (`self.PlayerInventory`)
    (:`exec`
      (bind _inventory_2 (`self.PlayerInventory`)
        (:`exec`
          (set `/Game/SurvivalGameKitV2/Blueprints/Components/BP_PlayerInventory.MaxHunger` (+ _maxhungerdelta (`/Game/SurvivalGameKitV2/Blueprints/Components/BP_PlayerInventory.MaxHunger` _inventory)) _inventory_2)
          (bind _outstatreduction (`/Game/TheBiogenSurvivor/Blueprints/Other/Interfaces/BP_TBSFunctions.TBS Add Stat Reductions` (`/Game/SurvivalGameKitV2/Blueprints/Components/BP_PlayerInventory.HungerReduction` _inventory) _hungerreductiondelta))
          (set `/Game/SurvivalGameKitV2/Blueprints/Components/BP_PlayerInventory.HungerReduction` _outstatreduction _inventory_2)
          (set `/Game/SurvivalGameKitV2/Blueprints/Components/BP_PlayerInventory.HungerReductionTime` (+ _hungerreductiontimedelta (`/Game/SurvivalGameKitV2/Blueprints/Components/BP_PlayerInventory.HungerReductionTime` _inventory)) _inventory_2)
          (set `/Game/SurvivalGameKitV2/Blueprints/Components/BP_PlayerInventory.MaxThirst` (+ _maxthirstdelta (`/Game/SurvivalGameKitV2/Blueprints/Components/BP_PlayerInventory.MaxThirst` _inventory)) _inventory_2)
          (bind _outstatreduction_2 (`/Game/TheBiogenSurvivor/Blueprints/Other/Interfaces/BP_TBSFunctions.TBS Add Stat Reductions` (`/Game/SurvivalGameKitV2/Blueprints/Components/BP_PlayerInventory.ThirstReduction` _inventory) _thirstreductiondelta))
          (set `/Game/SurvivalGameKitV2/Blueprints/Components/BP_PlayerInventory.ThirstReduction` _outstatreduction_2 _inventory_2)
          (set `/Game/SurvivalGameKitV2/Blueprints/Components/BP_PlayerInventory.ThirstReductionTime` (+ _thirstreductiontimedelta (`/Game/SurvivalGameKitV2/Blueprints/Components/BP_PlayerInventory.ThirstReductionTime` _inventory)) _inventory_2)
          (set `/Game/SurvivalGameKitV2/Blueprints/Components/BP_PlayerInventory.MaxHealth` (+ _maxhealthdelta (`/Game/SurvivalGameKitV2/Blueprints/Components/BP_PlayerInventory.MaxHealth` _inventory)) _inventory_2)
          (set `/Game/SurvivalGameKitV2/Blueprints/Components/BP_PlayerInventory.MaxStamina` (+ _maxstaminadelta (`/Game/SurvivalGameKitV2/Blueprints/Components/BP_PlayerInventory.MaxStamina` _inventory)) _inventory_2)
          (bind _outrechargestates (`/Game/TheBiogenSurvivor/Blueprints/Other/Interfaces/BP_TBSFunctions.TBS AddStaminaRecharge` (`/Game/SurvivalGameKitV2/Blueprints/Components/BP_PlayerInventory.StaminaRecharge` _inventory) _staminarechargedelta))
          (set `/Game/SurvivalGameKitV2/Blueprints/Components/BP_PlayerInventory.StaminaRecharge` _outrechargestates _inventory_2)
          (bind _outmovespeed (`/Game/TheBiogenSurvivor/Blueprints/Other/Interfaces/BP_TBSFunctions.TBS Add Movement Speeds` _movementspeeddelta (`/Game/SurvivalGameKitV2/Blueprints/Components/BP_PlayerInventory.MovementSpeeds` _inventory)))
          (set `/Game/SurvivalGameKitV2/Blueprints/Components/BP_PlayerInventory.MovementSpeeds` _outmovespeed _inventory_2)
          (set `/Game/SurvivalGameKitV2/Blueprints/Components/BP_PlayerInventory.UseHealthRegeneration` (or _usehealthregen (`/Game/SurvivalGameKitV2/Blueprints/Components/BP_PlayerInventory.UseHealthRegeneration` _inventory)) _inventory_2)
          (set `/Game/SurvivalGameKitV2/Blueprints/Components/BP_PlayerInventory.HealthRegenerationTickAmount` (+ _healthregenamount (`/Game/SurvivalGameKitV2/Blueprints/Components/BP_PlayerInventory.HealthRegenerationTickAmount` _inventory)) _inventory_2)
          (set `/Game/SurvivalGameKitV2/Blueprints/Components/BP_PlayerInventory.MinHealthRegenerationHunger` (+ _healthregenminhunger (`/Game/SurvivalGameKitV2/Blueprints/Components/BP_PlayerInventory.MinHealthRegenerationHunger` _inventory)) _inventory_2)
          (set `/Game/SurvivalGameKitV2/Blueprints/Components/BP_PlayerInventory.MinHealthRegenerationThirst` (+ _healthregenminthirst (`/Game/SurvivalGameKitV2/Blueprints/Components/BP_PlayerInventory.MinHealthRegenerationThirst` _inventory)) _inventory_2)
          (set `/Game/SurvivalGameKitV2/Blueprints/Components/BP_PlayerInventory.RegenerationTickTime` (+ _healthregenticktime (`/Game/SurvivalGameKitV2/Blueprints/Components/BP_PlayerInventory.RegenerationTickTime` _inventory)) _inventory_2)
          (set `/Game/SurvivalGameKitV2/Blueprints/Components/BP_PlayerInventory.FallDamage` (+ _falldamagedelta (`/Game/SurvivalGameKitV2/Blueprints/Components/BP_PlayerInventory.FallDamage` _inventory)) _inventory_2))))))

(fn `ClearCancers`
  (`BlueprintMapLibrary.Map_Clear` (`self.ActiveCancers`)))

(fn `EventCancerChecks`
  (params (MutationEvent :type "/Game/TheBiogenSurvivor/Blueprints/Other/Enum/E_MutationEvents Enum" :default "NewEnumerator0"))
  (locals (CancerForStageL :type Boolean) (NewLocalVar_0 :type "TimerHandle Structure"))
  (bind _outrownames (`DataTableFunctionLibrary.GetDataTableRowNames` "/Game/TheBiogenSurvivor/Blueprints/Mutations/CancerList.CancerList"))
  (for _array_element _outrownames
    (if (not (`.ReturnValue` (`BlueprintMapLibrary.Map_Find` (`self.ActiveCancers`) _array_element)))
      (bind _returnvalue (`|GetDataTableRow` "/Game/TheBiogenSurvivor/Blueprints/Mutations/CancerList.CancerList" _array_element)
        (:`then`
          (set `local.CancerForStageL` false)
          (bind (_name _shortname _description _triggerevents _baseprobability) (break `/Game/TheBiogenSurvivor/Blueprints/Other/Structs/S_CancerDetails` _returnvalue))
          (for _array_element_2 _triggerevents
            (if (`|EnumEquality` _array_element_2 (`local.MutationEvent`))
              (set `local.CancerForStageL` true)
              (break)))
          (if (`local.CancerForStageL`)
            (if (<= (`KismetMathLibrary.RandomFloat`) _baseprobability)
              (`BlueprintMapLibrary.Map_Add` (`self.ActiveCancers`) _array_element "NewEnumerator0"))))))))

(fn `GrowCancers`
  (locals (CurrentStageL :type "/Game/TheBiogenSurvivor/Blueprints/Other/Enum/E_CancerStages Enum") (NextStageIndexL :type Integer) (CancerNameL :type Name) (CancerGrewL :type Boolean))
  (bind _keys (`BlueprintMapLibrary.Map_Keys` (`self.ActiveCancers`)))
  (for _array_element _keys
    (bind _output_get (set `local.CancerNameL` _array_element))
    (set `local.CurrentStageL` (`BlueprintMapLibrary.Map_Find` (`self.ActiveCancers`) (`local.CancerNameL`)))
    (bind _returnvalue (`|GetDataTableRow` "/Game/TheBiogenSurvivor/Blueprints/Mutations/CancerList.CancerList" _output_get)
      (:`then`
        (set `local.CancerGrewL` false)
        (bind (_name _shortname _description _triggerevents _baseprobability _cancerstages) (break `/Game/TheBiogenSurvivor/Blueprints/Other/Structs/S_CancerDetails` _returnvalue))
        ;[1 1 1] Find the cancer stage and check if it grows
        (for (_array_element_2 _array_index) _cancerstages
          (bind (_stage _growthprobability) (break `/Game/TheBiogenSurvivor/Blueprints/Other/Structs/S_CancerStageDetails` _array_element_2))
          (if (`|EnumEquality` _stage (`local.CurrentStageL`))
            (bind _output_get_2 (set `local.CancerGrewL` (< (`KismetMathLibrary.RandomFloat`) _growthprobability)))
            (if _output_get_2
              (set `local.NextStageIndexL` (+ _array_index 1))
              (break)
              (else
                (break)))))
        ;[1 1 1] Check if cancer grew, and if so, move to the next stage and apply effects
        (if (`local.CancerGrewL`)
          (if (< (`local.NextStageIndexL`) (enumcount `/Game/TheBiogenSurvivor/Blueprints/Other/Enum/E_CancerStages`))
            (bind (_stage_2 _growthprobability_2 _stageeffects) (break `/Game/TheBiogenSurvivor/Blueprints/Other/Structs/S_CancerStageDetails` (`|GetArrayItem` _cancerstages (`local.NextStageIndexL`))))
            (`self.ApplyStatModifiers` _stageeffects)
            (`BlueprintMapLibrary.Map_Add` (`self.ActiveCancers`) (`local.CancerNameL`) _stage_2)))))))

(fn `MergeMutationStats`
  (params (InMutations :type "Array of DataTableRowHandle Structure"))
  (returns (OutMutationDetails :type "/Game/TheBiogenSurvivor/Blueprints/Other/Structs/S_MutationDetails Structure"))
  (bind _outmutationdetails (`/Game/TheBiogenSurvivor/Blueprints/Other/Interfaces/BP_TBSFunctions.TBS AddMutationStats` InMutations))
  (return _outmutationdetails))

(fn `OpenBiogeneticsMenu`
  (params (ProcessingComponent :type "/Game/SurvivalGameKitV2/Blueprints/Components/BP_MasterInventory Object Reference"))
  ;[1 1 1] Show Biogenetics panel and toggle inventory
  (bind _inventory (`self.PlayerInventory`)
    (:`exec`
      (set `/Game/SurvivalGameKitV2/Blueprints/Components/BP_PlayerInventory.InteractedActor` (`self.GetOwner`) _inventory)
      (set `/Game/SurvivalGameKitV2/Blueprints/Widgets/BP_InventoryHUD.BioResearchVisibility` "Visible" (`/Game/SurvivalGameKitV2/Blueprints/Components/BP_PlayerInventory.PlayerHUD` _inventory))
      (bind _inventory_2 (`self.PlayerInventory`)
        (:`exec`
          (`/Game/SurvivalGameKitV2/Blueprints/Components/BP_PlayerInventory.ToggleInventory` _inventory_2)
          (`/Game/TheBiogenSurvivor/Blueprints/Widgets/BP_BiogeneticsInterface.PopulateMutrationsList` (`/Game/SurvivalGameKitV2/Blueprints/Widgets/BP_InventoryHUD.BP_BiogeneticsInterface` (`/Game/SurvivalGameKitV2/Blueprints/Components/BP_PlayerInventory.PlayerHUD` _inventory_2)) "NewEnumerator11" (`local.ProcessingComponent`)))))))

(fn `SetActiveBirthDefects`
  (locals (HasDefectL :type Boolean) (DefectNameL :type Name))
  (bind _returnvalue (`KismetMathLibrary.RandomIntegerInRange` (`self.MinBirthDefects`) (`self.MaxBirthDefects`)))
  (bind _asbp_sgkcontroller (cast `/Game/SurvivalGameKitV2/Blueprints/Characters/BP_SGKController` (`self.GetOwner`)))
  (bind _asbp_tbsmaster_character (cast `/Game/TheBiogenSurvivor/Blueprints/Character/BP_TBSMasterCharacter` (`/Game/SurvivalGameKitV2/Blueprints/Characters/BP_SGKController.MasterCharacter` _asbp_sgkcontroller)))
  (set `PostProcessComponent.Settings` (`self.DefaultPP`) (`/Game/TheBiogenSurvivor/Blueprints/Character/BP_TBSMasterCharacter.PostProcess` _asbp_tbsmaster_character))
  (`KismetArrayLibrary.Array_Clear` (`self.ActiveBirthDefects`))
  (bind _outrownames (`DataTableFunctionLibrary.GetDataTableRowNames` "/Game/TheBiogenSurvivor/Blueprints/Mutations/BirthDefectList.BirthDefectList"))
  (if (> _returnvalue 0)
    (for _ (range (+ _returnvalue 1))
      (set `local.HasDefectL` false)
      (set `local.DefectNameL` (`|GetArrayItem` _outrownames (`KismetMathLibrary.RandomIntegerInRange` 0 (- (`KismetArrayLibrary.Array_Length` _outrownames) 1))))
      (for _array_element (`self.ActiveBirthDefects`)
        (if (== (`.RowName` (break `DataTableRowHandle` _array_element)) (`local.DefectNameL`))
          (set `local.HasDefectL` true)
          (break)))
      (if (not (`local.HasDefectL`))
        (`KismetArrayLibrary.Array_Add` (`self.ActiveBirthDefects`) (make `DataTableRowHandle` "/Game/TheBiogenSurvivor/Blueprints/Mutations/BirthDefectList.BirthDefectList" (`local.DefectNameL`)))))
    (bind _outmutationdetails (`self.MergeMutationStats` (`self.ActiveBirthDefects`)))
    (`self.ApplyStatModifiers` _outmutationdetails)
    ;[1 1 1] Set vision attributes of birth defects
    (bind _asbp_sgkcontroller_2 (cast `/Game/SurvivalGameKitV2/Blueprints/Characters/BP_SGKController` (`self.GetOwner`)))
    (bind _asbp_tbsmaster_character_2 (cast `/Game/TheBiogenSurvivor/Blueprints/Character/BP_TBSMasterCharacter` (`/Game/SurvivalGameKitV2/Blueprints/Characters/BP_SGKController.MasterCharacter` _asbp_sgkcontroller_2)))
    (bind (_ppsettings _apply_pp) (`/Game/TheBiogenSurvivor/Blueprints/Other/Interfaces/BP_TBSFunctions.TBS GetMutationVisionSettings` (`/Game/TheBiogenSurvivor/Blueprints/Components/BP_PlayerMutations_TBS.ActiveBirthDefects` (`/Game/SurvivalGameKitV2/Blueprints/Characters/BP_SGKController.BP_PlayerMutations_TBS` _asbp_sgkcontroller_2))))
    (if _apply_pp
      (set `PostProcessComponent.Settings` _ppsettings (`/Game/TheBiogenSurvivor/Blueprints/Character/BP_TBSMasterCharacter.PostProcess` _asbp_tbsmaster_character_2)))))

(fn `SetNextMutationsToActive`
  (bind _outmutationdetails (`self.MergeMutationStats` (`self.NextMutations`)))
  (`self.SetStatsFromBaseValues` _outmutationdetails)
  (set `self.ActiveMutations` (`self.NextMutations`)))

(fn `SetStatsFromBaseValues`
  (params (Mutations :type "/Game/TheBiogenSurvivor/Blueprints/Other/Structs/S_MutationDetails Structure"))
  (bind (_name _shortname _description _type _mutationicon _maxhungerdelta _hungerreductiondelta _hungerreductiontimedelta _maxthirstdelta _thirstreductiondelta _thirstreductiontimedelta _maxhealthdelta _maxstaminadelta _staminarechargedelta _movementspeeddelta _usehealthregen _healthregenamount _healthregenminhunger _healthregenminthirst _healthregenticktime _falldamagedelta) (break `/Game/TheBiogenSurvivor/Blueprints/Other/Structs/S_MutationDetails` Mutations))
  (bind (_clientinteracthitresult _disablecharmovement _inventoryopen _interactedactor _currenthealth _currenthunger _currentthirst _currentstamina _currentcharacterstate _ismoving _sprintkeydown _usestaminatimer _rechargestaminatimer _blockinput _starvationtimer _dehydrationtimer _newholdingitem _sgkcharacter _holdinginvslot _newholdinginvslot _newholdingweaponslot _currentholdingtype _newholdingtype _inattack _issplitkeydown _holdingweaponslot _equipping _removeattachmentslot _dropremoveattachent _removeslottarget _rotatedattachtarget _newattachmentid _newattachment _deathcontroller _swapattachment _attachingitem _respawnedcharacter _deadbodytimer _playername _deadcharacter _craftingrecipes _respawned _deadcharacterclass _sprintchecktimer _serverhitresult _buildmode _bleeding _uiopen _tick_damage _quickmovekeydown _bleeddamagetimer _respawnpointname _cameralean _characterlean _interactiondistance _interactiontracechannel _quickslots _maxquickslots _maxhealth _startinghealth _maxstamina _startingstamina _staminareduction _staminareductiontime _staminarecharge _staminamovementstates _usethirst _thirstreduction _maxthirst _startingthirst _thirstreductiontime _dehydrationdamage _dehydrationdamagetime _usehunger _hungerreduction _maxhunger _startinghunger _starvationdamagetime _starvationdamage _hungerreductiontime _movementspeeds _rotatemovewidget _inventorytoggled _inventoryslotsize _allowdroppinghelditem _usenotificationsounds _warningnotifysound _clearinventoryondeath _deathsound _clearlearnrecipesondeath _deleteplayersaveondeath _deadbodydespawntime _interactiontracedebug _takedamagesound _usehealthregeneration _healthregenerationtickamount _minhealthregenerationhunger _minhealthregenerationthirst _regenerationticktime _usefalldamage _falldamage) (defaults `/Game/SurvivalGameKitV2/Blueprints/Components/BP_PlayerInventory` "/Game/SurvivalGameKitV2/Blueprints/Components/BP_PlayerInventory.BP_PlayerInventory_C"))
  (bind _inventory (`self.PlayerInventory`)
    (:`exec`
      (set `/Game/SurvivalGameKitV2/Blueprints/Components/BP_PlayerInventory.MaxHunger` (+ _maxhungerdelta _maxhunger) _inventory)
      (bind _outstatreduction (`/Game/TheBiogenSurvivor/Blueprints/Other/Interfaces/BP_TBSFunctions.TBS Add Stat Reductions` _hungerreduction _hungerreductiondelta))
      (set `/Game/SurvivalGameKitV2/Blueprints/Components/BP_PlayerInventory.HungerReduction` _outstatreduction _inventory)
      (set `/Game/SurvivalGameKitV2/Blueprints/Components/BP_PlayerInventory.HungerReductionTime` (+ _hungerreductiontimedelta _hungerreductiontime) _inventory)
      (set `/Game/SurvivalGameKitV2/Blueprints/Components/BP_PlayerInventory.MaxThirst` (+ _maxthirstdelta _maxthirst) _inventory)
      (bind _outstatreduction_2 (`/Game/TheBiogenSurvivor/Blueprints/Other/Interfaces/BP_TBSFunctions.TBS Add Stat Reductions` _thirstreduction _thirstreductiondelta))
      (set `/Game/SurvivalGameKitV2/Blueprints/Components/BP_PlayerInventory.ThirstReduction` _outstatreduction_2 _inventory)
      (set `/Game/SurvivalGameKitV2/Blueprints/Components/BP_PlayerInventory.ThirstReductionTime` (+ _thirstreductiontimedelta _thirstreductiontime) _inventory)
      (set `/Game/SurvivalGameKitV2/Blueprints/Components/BP_PlayerInventory.MaxHealth` (+ _maxhealthdelta _maxhealth) _inventory)
      (set `/Game/SurvivalGameKitV2/Blueprints/Components/BP_PlayerInventory.MaxStamina` (+ _maxstaminadelta _maxstamina) _inventory)
      (bind _outrechargestates (`/Game/TheBiogenSurvivor/Blueprints/Other/Interfaces/BP_TBSFunctions.TBS AddStaminaRecharge` _staminarecharge _staminarechargedelta))
      (set `/Game/SurvivalGameKitV2/Blueprints/Components/BP_PlayerInventory.StaminaRecharge` _outrechargestates _inventory)
      (bind _outmovespeed (`/Game/TheBiogenSurvivor/Blueprints/Other/Interfaces/BP_TBSFunctions.TBS Add Movement Speeds` _movementspeeddelta _movementspeeds))
      (set `/Game/SurvivalGameKitV2/Blueprints/Components/BP_PlayerInventory.MovementSpeeds` _outmovespeed _inventory)
      (set `/Game/SurvivalGameKitV2/Blueprints/Components/BP_PlayerInventory.UseHealthRegeneration` (or _usehealthregen _usehealthregeneration) _inventory)
      (set `/Game/SurvivalGameKitV2/Blueprints/Components/BP_PlayerInventory.HealthRegenerationTickAmount` (+ _healthregenamount _healthregenerationtickamount) _inventory)
      (set `/Game/SurvivalGameKitV2/Blueprints/Components/BP_PlayerInventory.MinHealthRegenerationHunger` (+ _healthregenminhunger _minhealthregenerationhunger) _inventory)
      (set `/Game/SurvivalGameKitV2/Blueprints/Components/BP_PlayerInventory.MinHealthRegenerationThirst` (+ _healthregenminthirst _minhealthregenerationthirst) _inventory)
      (set `/Game/SurvivalGameKitV2/Blueprints/Components/BP_PlayerInventory.RegenerationTickTime` (+ _healthregenticktime _regenerationticktime) _inventory)
      (set `/Game/SurvivalGameKitV2/Blueprints/Components/BP_PlayerInventory.FallDamage` (+ _falldamagedelta _falldamage) _inventory))))