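; Shared helper function library for The Biogen Survivor, centred on the mutation system.
; Data table lookups resolve item processing, mutation progress, tiered unlock fractions and queued mutations, keeping one per type.
; Mutation stat deltas merge by summing maps per key, while active mutations drive consumable actions, vision post-processing and multiplicative damage modifiers.
; Other helpers spawn research, stat and status-effect widgets and total item counts across equipped-gear inventories.
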(fn `TBS Add Movement Speeds`
  (params (InMoveSpeeds1 :type "Map of /Game/SurvivalGameKitV2/Blueprints/Other/Enum/E_CharacterState Enum to Float (double-precision)") (InMoveSpeeds2 :type "Map of /Game/SurvivalGameKitV2/Blueprints/Other/Enum/E_CharacterState Enum to Float (double-precision)") (__WorldContext :type "Object Object Reference"))
  (returns (OutMoveSpeed :type "Map of /Game/SurvivalGameKitV2/Blueprints/Other/Enum/E_CharacterState Enum to Float (double-precision)"))
  (locals (MoveSpeedL :type "Map of /Game/SurvivalGameKitV2/Blueprints/Other/Enum/E_CharacterState Enum to Float (double-precision)"))
  (bind _movespeedl (`local.MoveSpeedL`))
  (bind _keys (`BlueprintMapLibrary.Map_Keys` InMoveSpeeds1))
  (for _array_element _keys
    (`BlueprintMapLibrary.Map_Add` (`local.MoveSpeedL`) _array_element (`BlueprintMapLibrary.Map_Find` (`local.InMoveSpeeds1`) _array_element)))
  (bind _keys_2 (`BlueprintMapLibrary.Map_Keys` InMoveSpeeds2))
  (for _array_element_2 _keys_2
    (bind (_value _returnvalue) (`BlueprintMapLibrary.Map_Find` (`local.MoveSpeedL`) _array_element_2))
    (if _returnvalue
      (bind _value_2 (`BlueprintMapLibrary.Map_Find` (`local.InMoveSpeeds2`) _array_element_2))
      (`BlueprintMapLibrary.Map_Add` _movespeedl _array_element_2 (+ _value _value_2))
      (else
        (`BlueprintMapLibrary.Map_Add` _movespeedl _array_element_2 _value_2))))
  (return (`local.MoveSpeedL`)))

(fn `TBS Add Mutation To Next`
  (params (PlayerInventory :type "/Game/TheBiogenSurvivor/Blueprints/Components/BP_PlayerMutations_TBS Object Reference") (MutationName :type Name))
  (locals (MutationTypeL :type "/Game/TheBiogenSurvivor/Blueprints/Other/Enum/E_MutationType Enum") (RemoveIndexL :type Integer) (HasMutationType :type Boolean))
  (set `local.HasMutationType` false)
  (bind _returnvalue (`|GetDataTableRow` "/Game/TheBiogenSurvivor/Blueprints/Mutations/MutationList.MutationList" MutationName)
    (:`then`
      (set `local.MutationTypeL` (`.Type_68_6A110AA147C0618865BD2884492EBE5A` (break `/Game/TheBiogenSurvivor/Blueprints/Other/Structs/S_MutationDetails` _returnvalue)))
      (for (_array_element _array_index) (`/Game/TheBiogenSurvivor/Blueprints/Components/BP_PlayerMutations_TBS.NextMutations` (`local.PlayerInventory`))
        (bind _returnvalue_2 (`|GetDataTableRow` "/Game/TheBiogenSurvivor/Blueprints/Mutations/MutationList.MutationList" (`.RowName` (break `DataTableRowHandle` _array_element)))
          (:`then`
            (if (`|EnumEquality` (`.Type_68_6A110AA147C0618865BD2884492EBE5A` (break `/Game/TheBiogenSurvivor/Blueprints/Other/Structs/S_MutationDetails` _returnvalue_2)) (`local.MutationTypeL`))
              (set `local.RemoveIndexL` _array_index)
              (set `local.HasMutationType` true)
              (break)))))
      (if (`local.HasMutationType`)
        (`KismetArrayLibrary.Array_Remove` (`/Game/TheBiogenSurvivor/Blueprints/Components/BP_PlayerMutations_TBS.NextMutations` (`local.PlayerInventory`)) (`local.RemoveIndexL`)))
      (`KismetArrayLibrary.Array_Add` (`/Game/TheBiogenSurvivor/Blueprints/Components/BP_PlayerMutations_TBS.NextMutations` (`local.PlayerInventory`)) (make `DataTableRowHandle` "/Game/TheBiogenSurvivor/Blueprints/Mutations/MutationList.MutationList" (`local.MutationName`))))))

(fn `TBS Add Stat Reductions`
  (params (InReductions1 :type "Array of /Game/SurvivalGameKitV2/Blueprints/Other/Structs/S_StatReduction Structure") (InReductions2 :type "Array of /Game/SurvivalGameKitV2/Blueprints/Other/Structs/S_StatReduction Structure") (__WorldContext :type "Object Object Reference"))
  (returns (OutStatReduction :type "Array of /Game/SurvivalGameKitV2/Blueprints/Other/Structs/S_StatReduction Structure"))
  (locals (ReductionL :type "Array of /Game/SurvivalGameKitV2/Blueprints/Other/Structs/S_StatReduction Structure") (ItemAdded :type Boolean) (ReductionMapL :type "Map of /Game/SurvivalGameKitV2/Blueprints/Other/Enum/E_CharacterState Enum to Float (double-precision)"))
  (for _array_element InReductions1
    (bind (_characterstate _amount) (break `/Game/SurvivalGameKitV2/Blueprints/Other/Structs/S_StatReduction` _array_element))
    (`BlueprintMapLibrary.Map_Add` (`local.ReductionMapL`) _characterstate _amount))
  (for _array_element_2 InReductions2
    (bind (_characterstate_2 _amount_2) (break `/Game/SurvivalGameKitV2/Blueprints/Other/Structs/S_StatReduction` _array_element_2))
    (bind (_value _returnvalue) (`BlueprintMapLibrary.Map_Find` (`local.ReductionMapL`) _characterstate_2))
    (if _returnvalue
      (`BlueprintMapLibrary.Map_Add` (`local.ReductionMapL`) _characterstate_2 (+ _value _amount_2))
      (else
        (`BlueprintMapLibrary.Map_Add` (`local.ReductionMapL`) _characterstate_2 _amount_2))))
  (bind _keys (`BlueprintMapLibrary.Map_Keys` (`local.ReductionMapL`)))
  (for _array_element_3 _keys
    (`KismetArrayLibrary.Array_Add` (`local.ReductionL`) (make `/Game/SurvivalGameKitV2/Blueprints/Other/Structs/S_StatReduction` _array_element_3 (`BlueprintMapLibrary.Map_Find` (`local.ReductionMapL`) _array_element_3))))
  (return (`local.ReductionL`)))

(fn `TBS AddDiseaseResistances`
  (params (DiseaseResistances1 :type "Map of Name to Float (double-precision)") (DiseaseResistances2 :type "Map of Name to Float (double-precision)"))
  (returns (OutDiseaseResistances :type "Map of Name to Float (double-precision)"))
  (locals (RestancesL :type "Map of Name to Float (double-precision)") (CurrentDiseaseL :type Name))
  (bind (_value _returnvalue) (`BlueprintMapLibrary.Map_Find` (`local.RestancesL`) (`local.CurrentDiseaseL`)))
  (bind _keys (`BlueprintMapLibrary.Map_Keys` DiseaseResistances1))
  (for _array_element _keys
    (`BlueprintMapLibrary.Map_Add` (`local.RestancesL`) _array_element (`BlueprintMapLibrary.Map_Find` (`local.DiseaseResistances1`) _array_element)))
  (bind _keys_2 (`BlueprintMapLibrary.Map_Keys` DiseaseResistances2))
  (for _array_element_2 _keys_2
    (set `local.CurrentDiseaseL` _array_element_2)
    (if _returnvalue
      (`BlueprintMapLibrary.Map_Add` (`local.RestancesL`) (`local.CurrentDiseaseL`) (+ _value (`BlueprintMapLibrary.Map_Find` (`local.DiseaseResistances2`) (`local.CurrentDiseaseL`))))
      (else
        (`BlueprintMapLibrary.Map_Add` (`local.RestancesL`) (`local.CurrentDiseaseL`) (`BlueprintMapLibrary.Map_Find` (`local.DiseaseResistances2`) (`local.CurrentDiseaseL`))))))
  (return (`local.RestancesL`)))

(fn `TBS AddMutationStats`
  (params (InMutations :type "Array of DataTableRowHandle Structure") (__WorldContext :type "Object Object Reference"))
  (returns (OutMutationDetails :type "/Game/TheBiogenSurvivor/Blueprints/Other/Structs/S_MutationDetails Structure"))
  (locals (MutationDetailsL :type "/Game/TheBiogenSurvivor/Blueprints/Other/Structs/S_MutationDetails Structure"))
  (bind (_mutationdetailsl_name _mutationdetailsl_shortname _mutationdetailsl_description _mutationdetailsl_type _mutationdetailsl_mutationicon _mutationdetailsl_maxhungerdelta _mutationdetailsl_hungerreductiondelta _mutationdetailsl_hungerreductiontimedelta _mutationdetailsl_maxthirstdelta _mutationdetailsl_thirstreductiondelta _mutationdetailsl_thirstreductiontimedelta _mutationdetailsl_maxhealthdelta _mutationdetailsl_maxstaminadelta _mutationdetailsl_staminarechargedelta _mutationdetailsl_movementspeeddelta _mutationdetailsl_usehealthregen _mutationdetailsl_healthregenamount _mutationdetailsl_healthregenminhunger _mutationdetailsl_healthregenminthirst _mutationdetailsl_healthregenticktime _mutationdetailsl_falldamagedelta _mutationdetailsl_hasspecial _mutationdetailsl_specialdescription _mutationdetailsl_jumppowerdelta _mutationdetailsl_diseaseresistancedelta) (break `/Game/TheBiogenSurvivor/Blueprints/Other/Structs/S_MutationDetails` (`local.MutationDetailsL`)))
  (for _array_element InMutations
    (bind (_datatable _rowname) (break `DataTableRowHandle` _array_element))
    (bind _returnvalue (`|GetDataTableRow` _datatable _rowname)
      (:`then`
        (bind (_name _shortname _description _type _mutationicon _maxhungerdelta _hungerreductiondelta _hungerreductiontimedelta _maxthirstdelta _thirstreductiondelta _thirstreductiontimedelta _maxhealthdelta _maxstaminadelta _staminarechargedelta _movementspeeddelta _usehealthregen _healthregenamount _healthregenminhunger _healthregenminthirst _healthregenticktime _falldamagedelta _hasspecial _specialdescription _jumppowerdelta _diseaseresistancedelta) (break `/Game/TheBiogenSurvivor/Blueprints/Other/Structs/S_MutationDetails` _returnvalue))
        (bind _outstatreduction (`self.TBS Add Stat Reductions` _hungerreductiondelta _mutationdetailsl_hungerreductiondelta))
        (bind _outstatreduction_2 (`self.TBS Add Stat Reductions` _thirstreductiondelta _mutationdetailsl_thirstreductiondelta))
        (bind _outmovespeed (`self.TBS Add Movement Speeds` _movementspeeddelta _mutationdetailsl_movementspeeddelta))
        (bind _outdiseaseresistances (`self.TBS AddDiseaseResistances` _mutationdetailsl_diseaseresistancedelta _diseaseresistancedelta))
        (set `local.MutationDetailsL` (make `/Game/TheBiogenSurvivor/Blueprints/Other/Structs/S_MutationDetails` "" "" "" "NewEnumerator0" null (+ _maxhungerdelta _mutationdetailsl_maxhungerdelta) _outstatreduction (+ _hungerreductiontimedelta _mutationdetailsl_hungerreductiontimedelta) (+ _maxthirstdelta _mutationdetailsl_maxthirstdelta) _outstatreduction_2 (+ _thirstreductiontimedelta _mutationdetailsl_thirstreductiontimedelta) (+ _maxhealthdelta _mutationdetailsl_maxhealthdelta) (+ _maxstaminadelta _mutationdetailsl_maxstaminadelta) (+ _staminarechargedelta _mutationdetailsl_staminarechargedelta) _outmovespeed (or _usehealthregen _mutationdetailsl_usehealthregen) (+ _healthregenamount _mutationdetailsl_healthregenamount) (+ _healthregenminhunger _mutationdetailsl_healthregenminhunger) (+ _healthregenminthirst _mutationdetailsl_healthregenminthirst) (+ _healthregenticktime _mutationdetailsl_healthregenticktime) (+ _falldamagedelta _mutationdetailsl_falldamagedelta) false _ (+ _jumppowerdelta _mutationdetailsl_jumppowerdelta) _outdiseaseresistances)))))
  (return (`local.MutationDetailsL`)))

(fn `TBS AddResearchToSet`
  (params (ResearchSet :type "HorizontalBox Object Reference") (MutationName :type Name) (RequiredProgress :type "Float (double-precision)") (CompletedProgress :type "Float (double-precision)") (OwningPlayer :type "PlayerController Object Reference"))
  (locals (NewMutationListingL :type "/Game/TheBiogenSurvivor/Blueprints/Widgets/BP_ResearchProgress Object Reference"))
  (bind _returnvalue (`|CreateWidget` "/Game/TheBiogenSurvivor/Blueprints/Widgets/BP_ResearchProgress.BP_ResearchProgress_C" OwningPlayer))
  (bind _output_get (set `local.NewMutationListingL` _returnvalue))
  (`/Game/TheBiogenSurvivor/Blueprints/Widgets/BP_ResearchProgress.InitializeResearchListing` _output_get (`local.MutationName`))
  (`/Game/TheBiogenSurvivor/Blueprints/Widgets/BP_ResearchProgress.UpdateFloat` (`local.NewMutationListingL`) (/ (`local.CompletedProgress`) (`local.RequiredProgress`)))
  (bind _returnvalue_2 (`PanelWidget.AddChild` (`local.ResearchSet`) (`local.NewMutationListingL`)))
  (bind _ashorizontal_box_slot (cast `HorizontalBoxSlot` _returnvalue_2))
  (`HorizontalBoxSlot.SetSize` _ashorizontal_box_slot (make `SlateChildSize` 1.0)))

(fn `TBS AddStaminaRecharge`
  (params (StaminaRechargeStates :type "Map of /Game/SurvivalGameKitV2/Blueprints/Other/Enum/E_CharacterState Enum to Float (double-precision)") (RechargeDelta :type "Float (double-precision)") (__WorldContext :type "Object Object Reference"))
  (returns (OutRechargeStates :type "Map of /Game/SurvivalGameKitV2/Blueprints/Other/Enum/E_CharacterState Enum to Float (double-precision)"))
  (locals (RechargeStatesL :type "Map of /Game/SurvivalGameKitV2/Blueprints/Other/Enum/E_CharacterState Enum to Float (double-precision)"))
  (bind _keys (`BlueprintMapLibrary.Map_Keys` StaminaRechargeStates))
  (for _array_element _keys
    (`BlueprintMapLibrary.Map_Add` (`local.RechargeStatesL`) _array_element (+ (`BlueprintMapLibrary.Map_Find` (`local.StaminaRechargeStates`) _array_element) (`local.RechargeDelta`))))
  (return (`local.RechargeStatesL`)))

(fn `TBS AddStatToStatList`
  (params (OwningPlayer :type "PlayerController Object Reference") (StatList :type "VerticalBox Object Reference") (StatName :type Text) (StatValue :type "Float (double-precision)") (StatMax :type "Float (double-precision)") (IsPrimary :type Boolean))
  (locals (EntryWidgetL :type "/Game/TheBiogenSurvivor/Blueprints/Widgets/BP_StatEntry Object Reference"))
  (bind _returnvalue (`|CreateWidget` "/Game/TheBiogenSurvivor/Blueprints/Widgets/BP_StatEntry.BP_StatEntry_C" (`local.OwningPlayer`)))
  (bind _output_get (set `local.EntryWidgetL` _returnvalue))
  (`/Game/TheBiogenSurvivor/Blueprints/Widgets/BP_StatEntry.InitializeEntry` _output_get (`local.StatName`) (`local.StatValue`) (`local.StatMax`) (`local.IsPrimary`))
  (`PanelWidget.AddChild` (`local.StatList`) (`local.EntryWidgetL`)))

(fn `TBS AddStatToTooltip`
  (params (OwningPlayer :type "PlayerController Object Reference") (StatList :type "VerticalBox Object Reference") (StatName :type Text) (StatValue :type "Float (double-precision)"))
  (locals (EntryWidgetL :type "/Game/TheBiogenSurvivor/Blueprints/Widgets/BP_MutationTooltipEntry Object Reference"))
  (if (!= StatValue 0.0)
    (bind _returnvalue (`|CreateWidget` "/Game/TheBiogenSurvivor/Blueprints/Widgets/BP_MutationTooltipEntry.BP_MutationTooltipEntry_C" (`local.OwningPlayer`)))
    (bind _output_get (set `local.EntryWidgetL` _returnvalue))
    (`/Game/TheBiogenSurvivor/Blueprints/Widgets/BP_MutationTooltipEntry.InitializeEntry` _output_get (`local.StatName`) (`local.StatValue`))
    (`PanelWidget.AddChild` (`local.StatList`) (`local.EntryWidgetL`))))

(fn `TBS AddStatusEffectToList`
  (params (OwningPlayer :type "PlayerController Object Reference") (StatusEffectList :type "VerticalBox Object Reference") (StatusEffectName :type Text) (StatusEffectDescription :type Text))
  (locals (StatusEffectWidgetL :type "/Game/TheBiogenSurvivor/Blueprints/Widgets/BP_StatusEffectEntry Object Reference"))
  (bind _returnvalue (`|CreateWidget` "/Game/TheBiogenSurvivor/Blueprints/Widgets/BP_StatusEffectEntry.BP_StatusEffectEntry_C" OwningPlayer))
  (bind _output_get (set `local.StatusEffectWidgetL` _returnvalue))
  (`/Game/TheBiogenSurvivor/Blueprints/Widgets/BP_StatusEffectEntry.InitializeEntry` _output_get (`local.StatusEffectName`) (`local.StatusEffectDescription`))
  (`PanelWidget.AddChild` (`local.StatusEffectList`) (`local.StatusEffectWidgetL`)))

(fn `TBS GetMutationConsumable`
  (params (ItemID :type Name) (Owner :type "PlayerController Object Reference"))
  (returns (`Consumable Details` :type "/Game/SurvivalGameKitV2/Blueprints/Other/Structs/S_ConsumableDetails Structure") (Found :type Boolean))
  (bind _asbp_sgkcontroller (cast `/Game/SurvivalGameKitV2/Blueprints/Characters/BP_SGKController` Owner)
    (:`then`
      (for _array_element (`/Game/TheBiogenSurvivor/Blueprints/Components/BP_PlayerMutations_TBS.ActiveMutations` (`/Game/SurvivalGameKitV2/Blueprints/Characters/BP_SGKController.BP_PlayerMutations_TBS` _asbp_sgkcontroller))
        (bind (_datatable _rowname) (break `DataTableRowHandle` _array_element))
        (bind _returnvalue (`|GetDataTableRow` "/Game/TheBiogenSurvivor/Blueprints/Mutations/MutationList.MutationList" _rowname)
          (:`then`
            (if (`|EnumEquality` (`.Type_68_6A110AA147C0618865BD2884492EBE5A` (break `/Game/TheBiogenSurvivor/Blueprints/Other/Structs/S_MutationDetails` _returnvalue)) "NewEnumerator7")
              (bind _returnvalue_2 (`|GetDataTableRow` "/Game/TheBiogenSurvivor/Blueprints/Mutations/MutationConsumablesList.MutationConsumablesList" _rowname)
                (:`then`
                  (bind (_value _returnvalue_3) (`BlueprintMapLibrary.Map_Find` (`.Consumables_10_B3BDC80E41E1BCAD51BCB78CD695446C` (break `/Game/TheBiogenSurvivor/Blueprints/Other/Structs/S_MutationConsumablesDetails` _returnvalue_2)) (`local.ItemID`)))
                  (return _value _returnvalue_3)))
              (else
                (`KismetSystemLibrary.PrintString` null "Mutation not digestive"))))
          (:`RowNotFound`
            (`KismetSystemLibrary.PrintString` null "Could not find mutation")))))
    (:`CastFailed`
      (`KismetSystemLibrary.PrintString` null "Could not cast to controller"))))

(fn `TBS GetMutationDamageModifier`
  (params (Player :type "PlayerController Object Reference") (DamageType :type "/Game/SurvivalGameKitV2/Blueprints/Other/Enum/E_DamageType Enum" :default "NewEnumerator3"))
  (returns (Modifier :type "Float (double-precision)"))
  (locals (DamageModifierL :type "Float (double-precision)" :default 1.0))
  (bind _asbp_sgkcontroller (cast `/Game/SurvivalGameKitV2/Blueprints/Characters/BP_SGKController` Player)
    (:`then`
      (for _array_element (`/Game/TheBiogenSurvivor/Blueprints/Components/BP_PlayerMutations_TBS.ActiveMutations` (`/Game/SurvivalGameKitV2/Blueprints/Characters/BP_SGKController.BP_PlayerMutations_TBS` _asbp_sgkcontroller))
        (bind _returnvalue (`|GetDataTableRow` "/Game/TheBiogenSurvivor/Blueprints/Mutations/MutationDamageModifiers.MutationDamageModifiers" (`.RowName` (break `DataTableRowHandle` _array_element)))
          (:`then`
            (bind (_damagetype _multiplier) (break `/Game/TheBiogenSurvivor/Blueprints/Other/Structs/S_DamageModifier` _returnvalue))
            (if (`|EnumEquality` (`local.DamageType`) _damagetype)
              (set `local.DamageModifierL` (* (`local.DamageModifierL`) _multiplier))))))
      (return (`local.DamageModifierL`)))
    (:`CastFailed`
      (`KismetSystemLibrary.PrintString` null "Could not cast to controller"))))

(fn `TBS GetMutationItemActions`
  (params (InActions :type "Array of /Game/SurvivalGameKitV2/Blueprints/Other/Structs/S_InventoryAction Structure") (ItemID :type Name) (PlayerController :type "PlayerController Object Reference"))
  (returns (Actions :type "Array of /Game/SurvivalGameKitV2/Blueprints/Other/Structs/S_InventoryAction Structure"))
  (locals (FoundConsumeActionL :type Boolean) (RemoveIndexL :type Integer))
  (set `local.FoundConsumeActionL` false)
  (bind (_consumable_details _found) (`self.TBS GetMutationConsumable` ItemID PlayerController))
  (if _found
    (if (`.CanConsume_1_F33B573C44E7F10E734CE98A8F8B397B` (break `/Game/SurvivalGameKitV2/Blueprints/Other/Structs/S_ConsumableDetails` _consumable_details))
      (for _array_element (`local.InActions`)
        (if (`|EnumEquality` (`.InventoryActions_11_09EA4A134331DF405C8B59A59F4D242C` (break `/Game/SurvivalGameKitV2/Blueprints/Other/Structs/S_InventoryAction` _array_element)) "NewEnumerator5")
          (set `local.FoundConsumeActionL` true)
          (break)))
      (if (not (`local.FoundConsumeActionL`))
        (`KismetArrayLibrary.Array_Add` (`local.InActions`) (make `/Game/SurvivalGameKitV2/Blueprints/Other/Structs/S_InventoryAction` "NewEnumerator5" "EAT"))
        (return (`local.InActions`)))
      (else
        (for (_array_element_2 _array_index) (`local.InActions`)
          (if (`|EnumEquality` (`.InventoryActions_11_09EA4A134331DF405C8B59A59F4D242C` (break `/Game/SurvivalGameKitV2/Blueprints/Other/Structs/S_InventoryAction` _array_element_2)) "NewEnumerator5")
            (set `local.FoundConsumeActionL` true)
            (set `local.RemoveIndexL` _array_index)
            (break)))
        (if (`local.FoundConsumeActionL`)
          (`KismetArrayLibrary.Array_Remove` (`local.InActions`) (`local.RemoveIndexL`))
          (return (`local.InActions`)))))
    (else
      (return (`local.InActions`)))))

(fn `TBS GetMutationsProgress`
  (params (MutationProgress :type "Map of Name to Float (double-precision)"))
  (returns (Mutations :type "Map of Name to Float (double-precision)"))
  (locals (MutationsL :type "Map of Name to Float (double-precision)") (RowNameL :type Name) (ProgressL :type "Float (double-precision)"))
  (bind (_value _returnvalue) (`BlueprintMapLibrary.Map_Find` (`local.MutationProgress`) (`local.RowNameL`)))
  (bind _keys (`BlueprintMapLibrary.Map_Keys` MutationProgress))
  (for _array_element _keys
    (set `local.RowNameL` _array_element)
    (if _returnvalue
      (set `local.ProgressL` _value)
      (bind _returnvalue_2 (`|GetDataTableRow` "/Game/TheBiogenSurvivor/Blueprints/Mutations/MutationUnlockList.MutationUnlockList" (`local.RowNameL`))
        (:`then`
          (bind (_progressitems _requiredt1 _unlockt1 _requiredt2 _unlockt2 _requiredt3 _unlockt3) (break `/Game/TheBiogenSurvivor/Blueprints/Other/Structs/S_MutationUnlockDetails` _returnvalue_2))
          (if (>= (`local.ProgressL`) _requiredt1)
            (bind (_datatable _rowname) (break `DataTableRowHandle` _unlockt1))
            (`BlueprintMapLibrary.Map_Add` (`local.MutationsL`) _rowname 1.0)
            (else
              (`BlueprintMapLibrary.Map_Add` (`local.MutationsL`) _rowname (/ (`local.ProgressL`) _requiredt1))))
          (if (> _requiredt2 0.0)
            (if (>= (`local.ProgressL`) _requiredt2)
              (bind (_datatable_2 _rowname_2) (break `DataTableRowHandle` _unlockt2))
              (`BlueprintMapLibrary.Map_Add` (`local.MutationsL`) _rowname_2 1.0)
              (else
                (`BlueprintMapLibrary.Map_Add` (`local.MutationsL`) _rowname_2 (/ (`local.ProgressL`) _requiredt2))))
            (if (> _requiredt3 0.0)
              (if (>= (`local.ProgressL`) _requiredt3)
                (bind (_datatable_3 _rowname_3) (break `DataTableRowHandle` _unlockt3))
                (`BlueprintMapLibrary.Map_Add` (`local.MutationsL`) _rowname_3 1.0)
                (else
                  (`BlueprintMapLibrary.Map_Add` (`local.MutationsL`) _rowname_3 (/ (`local.ProgressL`) _requiredt3))))))))))
  (return (`local.MutationsL`)))

(fn `TBS GetMutationVisionSettings`
  (params (ActiveMutations :type "Array of DataTableRowHandle Structure"))
  (returns (PPSettings :type "PostProcessSettings Structure") (`Apply PP` :type Boolean))
  (locals (`NightVision PP` :type "PostProcessSettings Structure" :default (struct :`bOverride_SceneColorTint` true :`bOverride_BloomIntensity` true :`bOverride_AutoExposureBias` true :`bOverride_VignetteIntensity` true :`BloomMethod` "BM_SOG" :`AutoExposureMethod` "AEM_Histogram" :`TemperatureType` "TEMP_WhiteBalance" :`WhiteTemp` 6500.0 :`ColorSaturation` (struct :`X` 1.0 :`Y` 1.0 :`Z` 1.0 :`W` 1.0) :`ColorContrast` (struct :`X` 1.0 :`Y` 1.0 :`Z` 1.0 :`W` 1.0) :`ColorGamma` (struct :`X` 1.0 :`Y` 1.0 :`Z` 1.0 :`W` 1.0) :`ColorGain` (struct :`X` 1.0 :`Y` 1.0 :`Z` 1.0 :`W` 1.0) :`ColorOffset` (struct) :`ColorSaturationShadows` (struct :`X` 1.0 :`Y` 1.0 :`Z` 1.0 :`W` 1.0) :`ColorContrastShadows` (struct :`X` 1.0 :`Y` 1.0 :`Z` 1.0 :`W` 1.0) :`ColorGammaShadows` (struct :`X` 1.0 :`Y` 1.0 :`Z` 1.0 :`W` 1.0) :`ColorGainShadows` (struct :`X` 1.0 :`Y` 1.0 :`Z` 1.0 :`W` 1.0) :`ColorOffsetShadows` (struct) :`ColorSaturationMidtones` (struct :`X` 1.0 :`Y` 1.0 :`Z` 1.0 :`W` 1.0) :`ColorContrastMidtones` (struct :`X` 1.0 :`Y` 1.0 :`Z` 1.0 :`W` 1.0) :`ColorGammaMidtones` (struct :`X` 1.0 :`Y` 1.0 :`Z` 1.0 :`W` 1.0) :`ColorGainMidtones` (struct :`X` 1.0 :`Y` 1.0 :`Z` 1.0 :`W` 1.0) :`ColorOffsetMidtones` (struct) :`ColorSaturationHighlights` (struct :`X` 1.0 :`Y` 1.0 :`Z` 1.0 :`W` 1.0) :`ColorContrastHighlights` (struct :`X` 1.0 :`Y` 1.0 :`Z` 1.0 :`W` 1.0) :`ColorGammaHighlights` (struct :`X` 1.0 :`Y` 1.0 :`Z` 1.0 :`W` 1.0) :`ColorGainHighlights` (struct :`X` 1.0 :`Y` 1.0 :`Z` 1.0 :`W` 1.0) :`ColorOffsetHighlights` (struct) :`ColorCorrectionHighlightsMin` 0.5 :`ColorCorrectionHighlightsMax` 1.0 :`ColorCorrectionShadowsMax` 0.09 :`BlueCorrection` 0.6 :`ExpandGamut` 1.0 :`ToneCurveAmount` 1.0 :`FilmSlope` 0.88 :`FilmToe` 0.55 :`FilmShoulder` 0.26 :`FilmWhiteClip` 0.04 :`SceneColorTint` (struct :`R` 0.369792 :`G` 0.369792 :`B` 0.369792 :`A` 1.0) :`BloomIntensity` 3.0 :`BloomThreshold` -1.0 :`BloomSizeScale` 4.0 :`Bloom1Size` 0.3 :`Bloom2Size` 1.0 :`Bloom3Size` 2.0 :`Bloom4Size` 10.0 :`Bloom5Size` 30.0 :`Bloom6Size` 64.0 :`Bloom1Tint` (struct :`R` 0.3465 :`G` 0.3465 :`B` 0.3465 :`A` 1.0) :`Bloom2Tint` (struct :`R` 0.138 :`G` 0.138 :`B` 0.138 :`A` 1.0) :`Bloom3Tint` (struct :`R` 0.1176 :`G` 0.1176 :`B` 0.1176 :`A` 1.0) :`Bloom4Tint` (struct :`R` 0.066 :`G` 0.066 :`B` 0.066 :`A` 1.0) :`Bloom5Tint` (struct :`R` 0.066 :`G` 0.066 :`B` 0.066 :`A` 1.0) :`Bloom6Tint` (struct :`R` 0.061 :`G` 0.061 :`B` 0.061 :`A` 1.0) :`BloomConvolutionScatterDispersion` 1.0 :`BloomConvolutionSize` 1.0 :`BloomConvolutionCenterUV` (0.5 0.5) :`BloomConvolutionPreFilterMin` 7.0 :`BloomConvolutionPreFilterMax` 15000.0 :`BloomConvolutionPreFilterMult` 15.0 :`BloomConvolutionBufferScale` 0.133 :`BloomDirtMaskTint` (struct :`R` 0.5 :`G` 0.5 :`B` 0.5 :`A` 1.0) :`DynamicGlobalIlluminationMethod` "Lumen" :`IndirectLightingColor` (struct :`R` 1.0 :`G` 1.0 :`B` 1.0 :`A` 1.0) :`IndirectLightingIntensity` 1.0 :`LumenSceneLightingQuality` 1.0 :`LumenSceneDetail` 1.0 :`LumenSceneViewDistance` 20000.0 :`LumenSceneLightingUpdateSpeed` 1.0 :`LumenFinalGatherQuality` 1.0 :`LumenFinalGatherLightingUpdateSpeed` 1.0 :`LumenMaxTraceDistance` 20000.0 :`RayTracingGIType` "Disabled" :`RayTracingGIMaxBounces` 1 :`RayTracingGISamplesPerPixel` 4 :`ReflectionMethod` "Lumen" :`LumenReflectionQuality` 1.0 :`LumenRayLightingMode` "Default" :`ScreenSpaceReflectionIntensity` 100.0 :`ScreenSpaceReflectionQuality` 50.0 :`ScreenSpaceReflectionMaxRoughness` 0.6 :`RayTracingReflectionsMaxRoughness` 0.6 :`RayTracingReflectionsMaxBounces` 1 :`RayTracingReflectionsSamplesPerPixel` 1 :`RayTracingReflectionsShadows` "Hard_shadows" :`AmbientCubemapTint` (struct :`R` 1.0 :`G` 1.0 :`B` 1.0 :`A` 1.0) :`AmbientCubemapIntensity` 1.0 :`CameraShutterSpeed` 60.0 :`CameraISO` 100.0 :`DepthOfFieldFstop` 4.0 :`DepthOfFieldMinFstop` 1.2 :`DepthOfFieldBladeCount` 5 :`AutoExposureBias` 3.0 :`AutoExposureApplyPhysicalCameraExposure` true :`AutoExposureLowPercent` 10.0 :`AutoExposureHighPercent` 90.0 :`AutoExposureMinBrightness` 0.03 :`AutoExposureMaxBrightness` 8.0 :`AutoExposureSpeedUp` 3.0 :`AutoExposureSpeedDown` 1.0 :`HistogramLogMin` -8.0 :`HistogramLogMax` 4.0 :`LocalExposureContrastScale` 1.0 :`LocalExposureDetailStrength` 1.0 :`LocalExposureBlurredLuminanceBlend` 0.6 :`LocalExposureBlurredLuminanceKernelSizePercent` 50.0 :`LensFlareIntensity` 1.0 :`LensFlareTint` (struct :`R` 1.0 :`G` 1.0 :`B` 1.0 :`A` 1.0) :`LensFlareBokehSize` 3.0 :`LensFlareThreshold` 8.0 :`LensFlareTints[0]` (struct :`R` 1.0 :`G` 0.8 :`B` 0.4 :`A` 0.6) :`LensFlareTints[1]` (struct :`R` 1.0 :`G` 1.0 :`B` 0.6 :`A` 0.53) :`LensFlareTints[2]` (struct :`R` 0.8 :`G` 0.8 :`B` 1.0 :`A` 0.46) :`LensFlareTints[3]` (struct :`R` 0.5 :`G` 1.0 :`B` 0.4 :`A` 0.39) :`LensFlareTints[4]` (struct :`R` 0.5 :`G` 0.8 :`B` 1.0 :`A` 0.31) :`LensFlareTints[5]` (struct :`R` 0.9 :`G` 1.0 :`B` 0.8 :`A` 0.27) :`LensFlareTints[6]` (struct :`R` 1.0 :`G` 0.8 :`B` 0.4 :`A` 0.22) :`LensFlareTints[7]` (struct :`R` 0.9 :`G` 0.7 :`B` 0.7 :`A` 0.15) :`VignetteIntensity` 0.6 :`FilmGrainIntensityShadows` 1.0 :`FilmGrainIntensityMidtones` 1.0 :`FilmGrainIntensityHighlights` 1.0 :`FilmGrainShadowsMax` 0.09 :`FilmGrainHighlightsMin` 0.5 :`FilmGrainHighlightsMax` 1.0 :`FilmGrainTexelSize` 1.0 :`AmbientOcclusionIntensity` 0.5 :`AmbientOcclusionStaticFraction` 1.0 :`AmbientOcclusionRadius` 200.0 :`AmbientOcclusionFadeDistance` 8000.0 :`AmbientOcclusionFadeRadius` 5000.0 :`AmbientOcclusionPower` 2.0 :`AmbientOcclusionBias` 3.0 :`AmbientOcclusionQuality` 50.0 :`AmbientOcclusionMipBlend` 0.6 :`AmbientOcclusionMipScale` 1.7 :`AmbientOcclusionMipThreshold` 0.01 :`AmbientOcclusionTemporalBlendWeight` 0.1 :`RayTracingAOSamplesPerPixel` 1 :`RayTracingAOIntensity` 1.0 :`RayTracingAORadius` 200.0 :`ColorGradingIntensity` 1.0 :`DepthOfFieldSensorWidth` 24.576 :`DepthOfFieldDepthBlurAmount` 1.0 :`DepthOfFieldNearTransitionRegion` 300.0 :`DepthOfFieldFarTransitionRegion` 500.0 :`DepthOfFieldNearBlurSize` 15.0 :`DepthOfFieldFarBlurSize` 15.0 :`DepthOfFieldOcclusion` 0.4 :`DepthOfFieldVignetteSize` 200.0 :`MotionBlurAmount` 0.5 :`MotionBlurMax` 5.0 :`MotionBlurTargetFPS` 30 :`TranslucencyType` "Raster" :`RayTracingTranslucencyMaxRoughness` 0.6 :`RayTracingTranslucencyRefractionRays` 3 :`RayTracingTranslucencySamplesPerPixel` 1 :`RayTracingTranslucencyShadows` "Hard_shadows" :`RayTracingTranslucencyRefraction` true :`PathTracingMaxBounces` 32 :`PathTracingSamplesPerPixel` 16384 :`PathTracingFilterWidth` 3.0 :`PathTracingEnableEmissive` true :`PathTracingMaxPathExposure` 30.0 :`PathTracingEnableDenoiser` true :`WeightedBlendables` (struct))) (`HeatVision PP` :type "PostProcessSettings Structure" :default (struct :`BloomMethod` "BM_SOG" :`AutoExposureMethod` "AEM_Histogram" :`TemperatureType` "TEMP_WhiteBalance" :`WhiteTemp` 6500.0 :`ColorSaturation` (struct :`X` 1.0 :`Y` 1.0 :`Z` 1.0 :`W` 1.0) :`ColorContrast` (struct :`X` 1.0 :`Y` 1.0 :`Z` 1.0 :`W` 1.0) :`ColorGamma` (struct :`X` 1.0 :`Y` 1.0 :`Z` 1.0 :`W` 1.0) :`ColorGain` (struct :`X` 1.0 :`Y` 1.0 :`Z` 1.0 :`W` 1.0) :`ColorOffset` (struct) :`ColorSaturationShadows` (struct :`X` 1.0 :`Y` 1.0 :`Z` 1.0 :`W` 1.0) :`ColorContrastShadows` (struct :`X` 1.0 :`Y` 1.0 :`Z` 1.0 :`W` 1.0) :`ColorGammaShadows` (struct :`X` 1.0 :`Y` 1.0 :`Z` 1.0 :`W` 1.0) :`ColorGainShadows` (struct :`X` 1.0 :`Y` 1.0 :`Z` 1.0 :`W` 1.0) :`ColorOffsetShadows` (struct) :`ColorSaturationMidtones` (struct :`X` 1.0 :`Y` 1.0 :`Z` 1.0 :`W` 1.0) :`ColorContrastMidtones` (struct :`X` 1.0 :`Y` 1.0 :`Z` 1.0 :`W` 1.0) :`ColorGammaMidtones` (struct :`X` 1.0 :`Y` 1.0 :`Z` 1.0 :`W` 1.0) :`ColorGainMidtones` (struct :`X` 1.0 :`Y` 1.0 :`Z` 1.0 :`W` 1.0) :`ColorOffsetMidtones` (struct) :`ColorSaturationHighlights` (struct :`X` 1.0 :`Y` 1.0 :`Z` 1.0 :`W` 1.0) :`ColorContrastHighlights` (struct :`X` 1.0 :`Y` 1.0 :`Z` 1.0 :`W` 1.0) :`ColorGammaHighlights` (struct :`X` 1.0 :`Y` 1.0 :`Z` 1.0 :`W` 1.0) :`ColorGainHighlights` (struct :`X` 1.0 :`Y` 1.0 :`Z` 1.0 :`W` 1.0) :`ColorOffsetHighlights` (struct) :`ColorCorrectionHighlightsMin` 0.5 :`ColorCorrectionHighlightsMax` 1.0 :`ColorCorrectionShadowsMax` 0.09 :`BlueCorrection` 0.6 :`ExpandGamut` 1.0 :`ToneCurveAmount` 1.0 :`FilmSlope` 0.88 :`FilmToe` 0.55 :`FilmShoulder` 0.26 :`FilmWhiteClip` 0.04 :`SceneColorTint` (struct :`R` 1.0 :`G` 1.0 :`B` 1.0 :`A` 1.0) :`BloomIntensity` 0.675 :`BloomThreshold` -1.0 :`BloomSizeScale` 4.0 :`Bloom1Size` 0.3 :`Bloom2Size` 1.0 :`Bloom3Size` 2.0 :`Bloom4Size` 10.0 :`Bloom5Size` 30.0 :`Bloom6Size` 64.0 :`Bloom1Tint` (struct :`R` 0.3465 :`G` 0.3465 :`B` 0.3465 :`A` 1.0) :`Bloom2Tint` (struct :`R` 0.138 :`G` 0.138 :`B` 0.138 :`A` 1.0) :`Bloom3Tint` (struct :`R` 0.1176 :`G` 0.1176 :`B` 0.1176 :`A` 1.0) :`Bloom4Tint` (struct :`R` 0.066 :`G` 0.066 :`B` 0.066 :`A` 1.0) :`Bloom5Tint` (struct :`R` 0.066 :`G` 0.066 :`B` 0.066 :`A` 1.0) :`Bloom6Tint` (struct :`R` 0.061 :`G` 0.061 :`B` 0.061 :`A` 1.0) :`BloomConvolutionScatterDispersion` 1.0 :`BloomConvolutionSize` 1.0 :`BloomConvolutionCenterUV` (0.5 0.5) :`BloomConvolutionPreFilterMin` 7.0 :`BloomConvolutionPreFilterMax` 15000.0 :`BloomConvolutionPreFilterMult` 15.0 :`BloomConvolutionBufferScale` 0.133 :`BloomDirtMaskTint` (struct :`R` 0.5 :`G` 0.5 :`B` 0.5 :`A` 1.0) :`DynamicGlobalIlluminationMethod` "Lumen" :`IndirectLightingColor` (struct :`R` 1.0 :`G` 1.0 :`B` 1.0 :`A` 1.0) :`IndirectLightingIntensity` 1.0 :`LumenSceneLightingQuality` 1.0 :`LumenSceneDetail` 1.0 :`LumenSceneViewDistance` 20000.0 :`LumenSceneLightingUpdateSpeed` 1.0 :`LumenFinalGatherQuality` 1.0 :`LumenFinalGatherLightingUpdateSpeed` 1.0 :`LumenMaxTraceDistance` 20000.0 :`RayTracingGIType` "Disabled" :`RayTracingGIMaxBounces` 1 :`RayTracingGISamplesPerPixel` 4 :`ReflectionMethod` "Lumen" :`LumenReflectionQuality` 1.0 :`LumenRayLightingMode` "Default" :`ScreenSpaceReflectionIntensity` 100.0 :`ScreenSpaceReflectionQuality` 50.0 :`ScreenSpaceReflectionMaxRoughness` 0.6 :`RayTracingReflectionsMaxRoughness` 0.6 :`RayTracingReflectionsMaxBounces` 1 :`RayTracingReflectionsSamplesPerPixel` 1 :`RayTracingReflectionsShadows` "Hard_shadows" :`AmbientCubemapTint` (struct :`R` 1.0 :`G` 1.0 :`B` 1.0 :`A` 1.0) :`AmbientCubemapIntensity` 1.0 :`CameraShutterSpeed` 60.0 :`CameraISO` 100.0 :`DepthOfFieldFstop` 4.0 :`DepthOfFieldMinFstop` 1.2 :`DepthOfFieldBladeCount` 5 :`AutoExposureBias` 1.0 :`AutoExposureApplyPhysicalCameraExposure` true :`AutoExposureLowPercent` 10.0 :`AutoExposureHighPercent` 90.0 :`AutoExposureMinBrightness` 0.03 :`AutoExposureMaxBrightness` 8.0 :`AutoExposureSpeedUp` 3.0 :`AutoExposureSpeedDown` 1.0 :`HistogramLogMin` -8.0 :`HistogramLogMax` 4.0 :`LocalExposureContrastScale` 1.0 :`LocalExposureDetailStrength` 1.0 :`LocalExposureBlurredLuminanceBlend` 0.6 :`LocalExposureBlurredLuminanceKernelSizePercent` 50.0 :`LensFlareIntensity` 1.0 :`LensFlareTint` (struct :`R` 1.0 :`G` 1.0 :`B` 1.0 :`A` 1.0) :`LensFlareBokehSize` 3.0 :`LensFlareThreshold` 8.0 :`LensFlareTints[0]` (struct :`R` 1.0 :`G` 0.8 :`B` 0.4 :`A` 0.6) :`LensFlareTints[1]` (struct :`R` 1.0 :`G` 1.0 :`B` 0.6 :`A` 0.53) :`LensFlareTints[2]` (struct :`R` 0.8 :`G` 0.8 :`B` 1.0 :`A` 0.46) :`LensFlareTints[3]` (struct :`R` 0.5 :`G` 1.0 :`B` 0.4 :`A` 0.39) :`LensFlareTints[4]` (struct :`R` 0.5 :`G` 0.8 :`B` 1.0 :`A` 0.31) :`LensFlareTints[5]` (struct :`R` 0.9 :`G` 1.0 :`B` 0.8 :`A` 0.27) :`LensFlareTints[6]` (struct :`R` 1.0 :`G` 0.8 :`B` 0.4 :`A` 0.22) :`LensFlareTints[7]` (struct :`R` 0.9 :`G` 0.7 :`B` 0.7 :`A` 0.15) :`VignetteIntensity` 0.4 :`FilmGrainIntensityShadows` 1.0 :`FilmGrainIntensityMidtones` 1.0 :`FilmGrainIntensityHighlights` 1.0 :`FilmGrainShadowsMax` 0.09 :`FilmGrainHighlightsMin` 0.5 :`FilmGrainHighlightsMax` 1.0 :`FilmGrainTexelSize` 1.0 :`AmbientOcclusionIntensity` 0.5 :`AmbientOcclusionStaticFraction` 1.0 :`AmbientOcclusionRadius` 200.0 :`AmbientOcclusionFadeDistance` 8000.0 :`AmbientOcclusionFadeRadius` 5000.0 :`AmbientOcclusionPower` 2.0 :`AmbientOcclusionBias` 3.0 :`AmbientOcclusionQuality` 50.0 :`AmbientOcclusionMipBlend` 0.6 :`AmbientOcclusionMipScale` 1.7 :`AmbientOcclusionMipThreshold` 0.01 :`AmbientOcclusionTemporalBlendWeight` 0.1 :`RayTracingAOSamplesPerPixel` 1 :`RayTracingAOIntensity` 1.0 :`RayTracingAORadius` 200.0 :`ColorGradingIntensity` 1.0 :`DepthOfFieldSensorWidth` 24.576 :`DepthOfFieldDepthBlurAmount` 1.0 :`DepthOfFieldNearTransitionRegion` 300.0 :`DepthOfFieldFarTransitionRegion` 500.0 :`DepthOfFieldNearBlurSize` 15.0 :`DepthOfFieldFarBlurSize` 15.0 :`DepthOfFieldOcclusion` 0.4 :`DepthOfFieldVignetteSize` 200.0 :`MotionBlurAmount` 0.5 :`MotionBlurMax` 5.0 :`MotionBlurTargetFPS` 30 :`TranslucencyType` "Raster" :`RayTracingTranslucencyMaxRoughness` 0.6 :`RayTracingTranslucencyRefractionRays` 3 :`RayTracingTranslucencySamplesPerPixel` 1 :`RayTracingTranslucencyShadows` "Hard_shadows" :`RayTracingTranslucencyRefraction` true :`PathTracingMaxBounces` 32 :`PathTracingSamplesPerPixel` 16384 :`PathTracingFilterWidth` 3.0 :`PathTracingEnableEmissive` true :`PathTracingMaxPathExposure` 30.0 :`PathTracingEnableDenoiser` true :`WeightedBlendables` (struct :`Array` (struct :`(Weight` "1.000000,Object=MaterialInstanceConstant'\"/Game/TheBiogenSurvivor/Materials/Thermal_PP_Inst.Thermal_PP_Inst\"')")))) (`Default PP` :type "PostProcessSettings Structure" :default (struct :`bOverride_ColorSaturation` true :`BloomMethod` "BM_SOG" :`AutoExposureMethod` "AEM_Histogram" :`TemperatureType` "TEMP_WhiteBalance" :`WhiteTemp` 6500.0 :`ColorSaturation` (struct :`X` 1.0 :`Y` 1.0 :`Z` 1.0 :`W` 1.0) :`ColorContrast` (struct :`X` 1.0 :`Y` 1.0 :`Z` 1.0 :`W` 1.0) :`ColorGamma` (struct :`X` 1.0 :`Y` 1.0 :`Z` 1.0 :`W` 1.0) :`ColorGain` (struct :`X` 1.0 :`Y` 1.0 :`Z` 1.0 :`W` 1.0) :`ColorOffset` (struct) :`ColorSaturationShadows` (struct :`X` 1.0 :`Y` 1.0 :`Z` 1.0 :`W` 1.0) :`ColorContrastShadows` (struct :`X` 1.0 :`Y` 1.0 :`Z` 1.0 :`W` 1.0) :`ColorGammaShadows` (struct :`X` 1.0 :`Y` 1.0 :`Z` 1.0 :`W` 1.0) :`ColorGainShadows` (struct :`X` 1.0 :`Y` 1.0 :`Z` 1.0 :`W` 1.0) :`ColorOffsetShadows` (struct) :`ColorSaturationMidtones` (struct :`X` 1.0 :`Y` 1.0 :`Z` 1.0 :`W` 1.0) :`ColorContrastMidtones` (struct :`X` 1.0 :`Y` 1.0 :`Z` 1.0 :`W` 1.0) :`ColorGammaMidtones` (struct :`X` 1.0 :`Y` 1.0 :`Z` 1.0 :`W` 1.0) :`ColorGainMidtones` (struct :`X` 1.0 :`Y` 1.0 :`Z` 1.0 :`W` 1.0) :`ColorOffsetMidtones` (struct) :`ColorSaturationHighlights` (struct :`X` 1.0 :`Y` 1.0 :`Z` 1.0 :`W` 1.0) :`ColorContrastHighlights` (struct :`X` 1.0 :`Y` 1.0 :`Z` 1.0 :`W` 1.0) :`ColorGammaHighlights` (struct :`X` 1.0 :`Y` 1.0 :`Z` 1.0 :`W` 1.0) :`ColorGainHighlights` (struct :`X` 1.0 :`Y` 1.0 :`Z` 1.0 :`W` 1.0) :`ColorOffsetHighlights` (struct) :`ColorCorrectionHighlightsMin` 0.5 :`ColorCorrectionHighlightsMax` 1.0 :`ColorCorrectionShadowsMax` 0.09 :`BlueCorrection` 0.6 :`ExpandGamut` 1.0 :`ToneCurveAmount` 1.0 :`FilmSlope` 0.88 :`FilmToe` 0.55 :`FilmShoulder` 0.26 :`FilmWhiteClip` 0.04 :`SceneColorTint` (struct :`R` 1.0 :`G` 1.0 :`B` 1.0 :`A` 1.0) :`BloomIntensity` 0.675 :`BloomThreshold` -1.0 :`BloomSizeScale` 4.0 :`Bloom1Size` 0.3 :`Bloom2Size` 1.0 :`Bloom3Size` 2.0 :`Bloom4Size` 10.0 :`Bloom5Size` 30.0 :`Bloom6Size` 64.0 :`Bloom1Tint` (struct :`R` 0.3465 :`G` 0.3465 :`B` 0.3465 :`A` 1.0) :`Bloom2Tint` (struct :`R` 0.138 :`G` 0.138 :`B` 0.138 :`A` 1.0) :`Bloom3Tint` (struct :`R` 0.1176 :`G` 0.1176 :`B` 0.1176 :`A` 1.0) :`Bloom4Tint` (struct :`R` 0.066 :`G` 0.066 :`B` 0.066 :`A` 1.0) :`Bloom5Tint` (struct :`R` 0.066 :`G` 0.066 :`B` 0.066 :`A` 1.0) :`Bloom6Tint` (struct :`R` 0.061 :`G` 0.061 :`B` 0.061 :`A` 1.0) :`BloomConvolutionScatterDispersion` 1.0 :`BloomConvolutionSize` 1.0 :`BloomConvolutionCenterUV` (0.5 0.5) :`BloomConvolutionPreFilterMin` 7.0 :`BloomConvolutionPreFilterMax` 15000.0 :`BloomConvolutionPreFilterMult` 15.0 :`BloomConvolutionBufferScale` 0.133 :`BloomDirtMaskTint` (struct :`R` 0.5 :`G` 0.5 :`B` 0.5 :`A` 1.0) :`DynamicGlobalIlluminationMethod` "Lumen" :`IndirectLightingColor` (struct :`R` 1.0 :`G` 1.0 :`B` 1.0 :`A` 1.0) :`IndirectLightingIntensity` 1.0 :`LumenSceneLightingQuality` 1.0 :`LumenSceneDetail` 1.0 :`LumenSceneViewDistance` 20000.0 :`LumenSceneLightingUpdateSpeed` 1.0 :`LumenFinalGatherQuality` 1.0 :`LumenFinalGatherLightingUpdateSpeed` 1.0 :`LumenMaxTraceDistance` 20000.0 :`RayTracingGIType` "Disabled" :`RayTracingGIMaxBounces` 1 :`RayTracingGISamplesPerPixel` 4 :`ReflectionMethod` "Lumen" :`LumenReflectionQuality` 1.0 :`LumenRayLightingMode` "Default" :`ScreenSpaceReflectionIntensity` 100.0 :`ScreenSpaceReflectionQuality` 50.0 :`ScreenSpaceReflectionMaxRoughness` 0.6 :`RayTracingReflectionsMaxRoughness` 0.6 :`RayTracingReflectionsMaxBounces` 1 :`RayTracingReflectionsSamplesPerPixel` 1 :`RayTracingReflectionsShadows` "Hard_shadows" :`AmbientCubemapTint` (struct :`R` 1.0 :`G` 1.0 :`B` 1.0 :`A` 1.0) :`AmbientCubemapIntensity` 1.0 :`CameraShutterSpeed` 60.0 :`CameraISO` 100.0 :`DepthOfFieldFstop` 4.0 :`DepthOfFieldMinFstop` 1.2 :`DepthOfFieldBladeCount` 5 :`AutoExposureBias` 1.0 :`AutoExposureApplyPhysicalCameraExposure` true :`AutoExposureLowPercent` 10.0 :`AutoExposureHighPercent` 90.0 :`AutoExposureMinBrightness` 0.03 :`AutoExposureMaxBrightness` 8.0 :`AutoExposureSpeedUp` 3.0 :`AutoExposureSpeedDown` 1.0 :`HistogramLogMin` -8.0 :`HistogramLogMax` 4.0 :`LocalExposureContrastScale` 1.0 :`LocalExposureDetailStrength` 1.0 :`LocalExposureBlurredLuminanceBlend` 0.6 :`LocalExposureBlurredLuminanceKernelSizePercent` 50.0 :`LensFlareIntensity` 1.0 :`LensFlareTint` (struct :`R` 1.0 :`G` 1.0 :`B` 1.0 :`A` 1.0) :`LensFlareBokehSize` 3.0 :`LensFlareThreshold` 8.0 :`LensFlareTints[0]` (struct :`R` 1.0 :`G` 0.8 :`B` 0.4 :`A` 0.6) :`LensFlareTints[1]` (struct :`R` 1.0 :`G` 1.0 :`B` 0.6 :`A` 0.53) :`LensFlareTints[2]` (struct :`R` 0.8 :`G` 0.8 :`B` 1.0 :`A` 0.46) :`LensFlareTints[3]` (struct :`R` 0.5 :`G` 1.0 :`B` 0.4 :`A` 0.39) :`LensFlareTints[4]` (struct :`R` 0.5 :`G` 0.8 :`B` 1.0 :`A` 0.31) :`LensFlareTints[5]` (struct :`R` 0.9 :`G` 1.0 :`B` 0.8 :`A` 0.27) :`LensFlareTints[6]` (struct :`R` 1.0 :`G` 0.8 :`B` 0.4 :`A` 0.22) :`LensFlareTints[7]` (struct :`R` 0.9 :`G` 0.7 :`B` 0.7 :`A` 0.15) :`VignetteIntensity` 0.4 :`FilmGrainIntensityShadows` 1.0 :`FilmGrainIntensityMidtones` 1.0 :`FilmGrainIntensityHighlights` 1.0 :`FilmGrainShadowsMax` 0.09 :`FilmGrainHighlightsMin` 0.5 :`FilmGrainHighlightsMax` 1.0 :`FilmGrainTexelSize` 1.0 :`AmbientOcclusionIntensity` 0.5 :`AmbientOcclusionStaticFraction` 1.0 :`AmbientOcclusionRadius` 200.0 :`AmbientOcclusionFadeDistance` 8000.0 :`AmbientOcclusionFadeRadius` 5000.0 :`AmbientOcclusionPower` 2.0 :`AmbientOcclusionBias` 3.0 :`AmbientOcclusionQuality` 50.0 :`AmbientOcclusionMipBlend` 0.6 :`AmbientOcclusionMipScale` 1.7 :`AmbientOcclusionMipThreshold` 0.01 :`AmbientOcclusionTemporalBlendWeight` 0.1 :`RayTracingAOSamplesPerPixel` 1 :`RayTracingAOIntensity` 1.0 :`RayTracingAORadius` 200.0 :`ColorGradingIntensity` 1.0 :`DepthOfFieldSensorWidth` 24.576 :`DepthOfFieldDepthBlurAmount` 1.0 :`DepthOfFieldNearTransitionRegion` 300.0 :`DepthOfFieldFarTransitionRegion` 500.0 :`DepthOfFieldNearBlurSize` 15.0 :`DepthOfFieldFarBlurSize` 15.0 :`DepthOfFieldOcclusion` 0.4 :`DepthOfFieldVignetteSize` 200.0 :`MotionBlurAmount` 0.5 :`MotionBlurMax` 5.0 :`MotionBlurTargetFPS` 30 :`TranslucencyType` "Raster" :`RayTracingTranslucencyMaxRoughness` 0.6 :`RayTracingTranslucencyRefractionRays` 3 :`RayTracingTranslucencySamplesPerPixel` 1 :`RayTracingTranslucencyShadows` "Hard_shadows" :`RayTracingTranslucencyRefraction` true :`PathTracingMaxBounces` 32 :`PathTracingSamplesPerPixel` 16384 :`PathTracingFilterWidth` 3.0 :`PathTracingEnableEmissive` true :`PathTracingMaxPathExposure` 30.0 :`PathTracingEnableDenoiser` true :`WeightedBlendables` (struct))))
  (for _array_element ActiveMutations
    (bind (_datatable _rowname) (break `DataTableRowHandle` _array_element))
    (bind _returnvalue (`|GetDataTableRow` _datatable _rowname)
      (:`then`
        (if (`|EnumEquality` (`.Type_68_6A110AA147C0618865BD2884492EBE5A` (break `/Game/TheBiogenSurvivor/Blueprints/Other/Structs/S_MutationDetails` _returnvalue)) "NewEnumerator1")
          (bind _returnvalue_2 (`|GetDataTableRow` "/Game/TheBiogenSurvivor/Blueprints/Mutations/MutationVisionList.MutationVisionList" _rowname)
            (:`then`
              (return (`.PostProcessing_5_00E0E0DA45040332192DF19E34794352` (break `/Game/TheBiogenSurvivor/Blueprints/Other/Structs/S_MutationVision` _returnvalue_2)) true)))))))
  (return (`local.Default PP`) false))

(fn `TBS ItemMutationProgress`
  (params (__WorldContext :type "Object Object Reference")))

(fn `TBS MutationProgress`
  (params (Item :type "/Game/SurvivalGameKitV2/Blueprints/Other/Structs/S_InvItem Structure") (__WorldContext :type "Object Object Reference"))
  (returns (MutationsProgress :type "Array of /Game/TheBiogenSurvivor/Blueprints/Other/Structs/S_MutationProgress Structure") (HasMutationProgress :type Boolean))
  (locals (output :type "Array of /Game/TheBiogenSurvivor/Blueprints/Other/Structs/S_MutationProgress Structure"))
  (bind _output (`local.output`))
  (bind _outrownames (`DataTableFunctionLibrary.GetDataTableRowNames` "/Game/TheBiogenSurvivor/Blueprints/Mutations/MutationUnlockList.MutationUnlockList"))
  (for _array_element _outrownames
    (bind _returnvalue (`|GetDataTableRow` "/Game/TheBiogenSurvivor/Blueprints/Mutations/MutationUnlockList.MutationUnlockList" _array_element)
      (:`then`
        (for _array_element_2 (`.ProgressItems_24_D38824A64524A8B4C6ADBEA4C0254894` (break `/Game/TheBiogenSurvivor/Blueprints/Other/Structs/S_MutationUnlockDetails` _returnvalue))
          (bind (_item _progressvalue) (break `/Game/TheBiogenSurvivor/Blueprints/Other/Structs/S_MutationUnlockItemDetails` _array_element_2))
          (if (== (`.RowName` (break `DataTableRowHandle` _item)) (`.ID_2_84C2CB8945979246059C568DCD463423` (break `/Game/SurvivalGameKitV2/Blueprints/Other/Structs/S_InvItem` (`local.Item`))))
            (`KismetArrayLibrary.Array_Add` (`local.output`) (make `/Game/TheBiogenSurvivor/Blueprints/Other/Structs/S_MutationProgress` _array_element _progressvalue)))))))
  (return _output (> (`KismetArrayLibrary.Array_Length` _output) 0)))

(fn `TBS ProcessingItem`
  (params (Item :type "/Game/SurvivalGameKitV2/Blueprints/Other/Structs/S_InvItem Structure") (__WorldContext :type "Object Object Reference"))
  (returns (`Return Value` :type Boolean) (`Processing Item` :type "/Game/TheBiogenSurvivor/Blueprints/Other/Structs/S_ProcessingItem Structure"))
  (locals (`Processing Item L` :type "/Game/TheBiogenSurvivor/Blueprints/Other/Structs/S_ProcessingItem Structure"))
  (bind _outrownames (`DataTableFunctionLibrary.GetDataTableRowNames` "/Game/TheBiogenSurvivor/Blueprints/Mutations/ProcessingItemList.ProcessingItemList"))
  (for _array_element _outrownames
    (bind _returnvalue (`|GetDataTableRow` "/Game/TheBiogenSurvivor/Blueprints/Mutations/ProcessingItemList.ProcessingItemList" _array_element)
      (:`then`
        (set `local.Processing Item L` _returnvalue)
        (if (== (`.RowName` (break `DataTableRowHandle` (`.StartingItem_11_1581F7DB44E1EE628672AC9EBC5289E6` (break `/Game/TheBiogenSurvivor/Blueprints/Other/Structs/S_ProcessingItem` _returnvalue)))) (`.ID_2_84C2CB8945979246059C568DCD463423` (break `/Game/SurvivalGameKitV2/Blueprints/Other/Structs/S_InvItem` (`local.Item`))))
          (return true (`local.Processing Item L`)))))))

(fn `TBSGet Total Amount in Inventory`
  (params (InvItem :type "/Game/SurvivalGameKitV2/Blueprints/Other/Structs/S_InvItem Structure") (PlayerInventory :type "/Game/TheBiogenSurvivor/Blueprints/Components/BP_TBS_PlayerInventory Object Reference"))
  (returns (Amount :type Integer))
  (locals (AmountL :type Integer) (SlotElementL :type "/Game/SurvivalGameKitV2/Blueprints/Other/Structs/S_InvSlot Structure") (InventoryL :type "/Game/SurvivalGameKitV2/Blueprints/Components/BP_MasterInventory Object Reference"))
  (set `local.AmountL` 0)
  (`|ExecutionSequence`
    (:`then_0`
      (set `local.InventoryL` (`local.PlayerInventory`)))
    (:`then_1`
      (set `local.InventoryL` (`.MasterInventory_8_17FFB7D341FAF2689C1BABA12E3BA9F5` (break `/Game/SurvivalGameKitV2/Blueprints/Other/Structs/S_InvItem` (`.Item_9_08D0FEA54FF8147DD55DE08559E54FAB` (break `/Game/SurvivalGameKitV2/Blueprints/Other/Structs/S_EquipmentSlot` (`/Game/SurvivalGameKitV2/Blueprints/Components/BP_EquipmentInventory.BackpackEquipmentSlot` PlayerInventory)))))))
    (:`then_2`
      (set `local.InventoryL` (`.MasterInventory_8_17FFB7D341FAF2689C1BABA12E3BA9F5` (break `/Game/SurvivalGameKitV2/Blueprints/Other/Structs/S_InvItem` (`.Item_9_08D0FEA54FF8147DD55DE08559E54FAB` (break `/Game/SurvivalGameKitV2/Blueprints/Other/Structs/S_EquipmentSlot` (`/Game/SurvivalGameKitV2/Blueprints/Components/BP_EquipmentInventory.EyewearEquipmentSlot` PlayerInventory)))))))
    (:`then_3`
      (set `local.InventoryL` (`.MasterInventory_8_17FFB7D341FAF2689C1BABA12E3BA9F5` (break `/Game/SurvivalGameKitV2/Blueprints/Other/Structs/S_InvItem` (`.Item_9_08D0FEA54FF8147DD55DE08559E54FAB` (break `/Game/SurvivalGameKitV2/Blueprints/Other/Structs/S_EquipmentSlot` (`/Game/SurvivalGameKitV2/Blueprints/Components/BP_EquipmentInventory.GlovesEquipmentSlot` PlayerInventory)))))))
    (:`then_4`
      (set `local.InventoryL` (`.MasterInventory_8_17FFB7D341FAF2689C1BABA12E3BA9F5` (break `/Game/SurvivalGameKitV2/Blueprints/Other/Structs/S_InvItem` (`.Item_9_08D0FEA54FF8147DD55DE08559E54FAB` (break `/Game/SurvivalGameKitV2/Blueprints/Other/Structs/S_EquipmentSlot` (`/Game/SurvivalGameKitV2/Blueprints/Components/BP_EquipmentInventory.HelmetEquipmentSlot` PlayerInventory)))))))
    (:`then_5`
      (set `local.InventoryL` (`.MasterInventory_8_17FFB7D341FAF2689C1BABA12E3BA9F5` (break `/Game/SurvivalGameKitV2/Blueprints/Other/Structs/S_InvItem` (`.Item_9_08D0FEA54FF8147DD55DE08559E54FAB` (break `/Game/SurvivalGameKitV2/Blueprints/Other/Structs/S_EquipmentSlot` (`/Game/SurvivalGameKitV2/Blueprints/Components/BP_EquipmentInventory.PantsEquipmentSlot` PlayerInventory)))))))
    (:`then_6`
      (set `local.InventoryL` (`.MasterInventory_8_17FFB7D341FAF2689C1BABA12E3BA9F5` (break `/Game/SurvivalGameKitV2/Blueprints/Other/Structs/S_InvItem` (`.Item_9_08D0FEA54FF8147DD55DE08559E54FAB` (break `/Game/SurvivalGameKitV2/Blueprints/Other/Structs/S_EquipmentSlot` (`/Game/SurvivalGameKitV2/Blueprints/Components/BP_EquipmentInventory.ShirtEquipmentSlot` PlayerInventory)))))))
    (:`then_7`
      (set `local.InventoryL` (`.MasterInventory_8_17FFB7D341FAF2689C1BABA12E3BA9F5` (break `/Game/SurvivalGameKitV2/Blueprints/Other/Structs/S_InvItem` (`.Item_9_08D0FEA54FF8147DD55DE08559E54FAB` (break `/Game/SurvivalGameKitV2/Blueprints/Other/Structs/S_EquipmentSlot` (`/Game/SurvivalGameKitV2/Blueprints/Components/BP_EquipmentInventory.ShoesEquipmentSlot` PlayerInventory)))))))
    (:`then_8`
      (set `local.InventoryL` (`.MasterInventory_8_17FFB7D341FAF2689C1BABA12E3BA9F5` (break `/Game/SurvivalGameKitV2/Blueprints/Other/Structs/S_InvItem` (`.Item_9_08D0FEA54FF8147DD55DE08559E54FAB` (break `/Game/SurvivalGameKitV2/Blueprints/Other/Structs/S_EquipmentSlot` (`/Game/SurvivalGameKitV2/Blueprints/Components/BP_EquipmentInventory.TacticalRigEquipmentSlot` PlayerInventory)))))))
    (:`then_9`
      (return (`local.AmountL`))))
  (`/Engine/EditorBlueprintResources/StandardMacros.IsValid` (`local.InventoryL`)
    (:`Is Valid`
      (bind _totalamount (`/Game/SurvivalGameKitV2/Blueprints/Components/BP_MasterInventory.TotalItemAmount` (`local.InventoryL`) (`local.InvItem`)))
      (set `local.AmountL` (+ _totalamount (`local.AmountL`))))))