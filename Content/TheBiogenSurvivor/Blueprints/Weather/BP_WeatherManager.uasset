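; Weather manager that cycles rain on and off at random intervals and durations.
; Timers set the Rain flag, which Tick polls to drive a DoOnce-guarded ToggleRain macro that spawns a BP_RainSystem at a random horizontal position and fixed height.
; A timeline ramps rain intensity up and back down; when the reverse finishes, it destroys the rain actor and schedules the next shower.
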(event `self.ReceiveBeginPlay`
  (`KismetSystemLibrary.K2_SetTimer` null "StartRaining" (`KismetMathLibrary.RandomFloatInRange` (`self.MinFirstRainStart`) (`self.MaxFirstRainStart`))))

(event `self.ReceiveTick`
  (params (DeltaSeconds :type "Float (single-precision)"))
  (if (`self.Rain`)
    (`self.ToggleRain` :!label _label)
    (else
      (goto _label :!via `Stop`))))

(event `RainfallIntensity`
  (params (Increase :type Boolean))
  (bind _rainsystem (`self.RainSystem`))
  (bind _rainsystem_2 (`self.RainSystem`))
  (if Increase
    (bind (_direction _alpha) (`Timeline|RainTimeline` :!label _label_2)
      (:`Update`
        (`/Engine/EditorBlueprintResources/StandardMacros.IsValid` _rainsystem
          (:`Is Valid`
            (bind _asbp_rain_system (cast `/Game/TheBiogenSurvivor/Blueprints/Weather/BP_RainSystem` _rainsystem))
            (`/Game/TheBiogenSurvivor/Blueprints/Weather/BP_RainSystem.UpdateRainIntensity` _asbp_rain_system _alpha))))
      (:`Finished`
        (if (`|EnumEquality` _direction "Backward")
          (`/Engine/EditorBlueprintResources/StandardMacros.IsValid` _rainsystem_2
            (:`Is Valid`
              (`self.K2_DestroyActor` _rainsystem_2)
              (`KismetSystemLibrary.K2_SetTimer` null "StartRaining" (`KismetMathLibrary.RandomFloatInRange` (`self.MinTimeBetweenRain`) (`self.MaxTimeBetweenRain`))))))))
    (else
      (goto _label_2 :!via `Reverse`))))

(fn `StartRaining`
  (set `self.Rain` true)
  (`KismetSystemLibrary.K2_SetTimer` null "StopRaining" (`KismetMathLibrary.RandomFloatInRange` (`self.MinRainTime`) (`self.MaxRainTime`))))

(fn `StopRaining`
  (set `self.Rain` false))

(fn `UserConstructionScript`)