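; BP_RainSystem is a rain volume that gives survivor characters rain effects and waters farm build parts inside its RainBox.
; Entering characters get a Niagara rain system with attached sound, both destroyed on exit, though only one RainSound reference is stored.
; Tick moves each effect to its character and adds water to overlapping farm parts, scaled by RainIntensity.
; UpdateRainIntensity sets that intensity, sound volume and particle spawn rate.
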(event `self.ReceiveTick`
  (params (DeltaSeconds :type "Float (single-precision)"))
  (`|ExecutionSequence`
    (:`then_0`
      (for _array_element (`PrimitiveComponent.GetOverlappingActors` (`self.RainBox`) "/Game/TheBiogenSurvivor/Blueprints/Character/BP_TBSMasterCharacter.BP_TBSMasterCharacter_C")
        (bind _asbp_tbsmaster_character (cast `/Game/TheBiogenSurvivor/Blueprints/Character/BP_TBSMasterCharacter` _array_element))
        (`self.SetRainLocation` _asbp_tbsmaster_character)))
    (:`then_1`
      (for _array_element_2 (`PrimitiveComponent.GetOverlappingActors` (`self.RainBox`) "/Game/TheBiogenSurvivor/Blueprints/BuildParts/BP_MasterFarmBuildPart.BP_MasterFarmBuildPart_C")
        (bind _asbp_master_farm_build_part (cast `/Game/TheBiogenSurvivor/Blueprints/BuildParts/BP_MasterFarmBuildPart` _array_element_2))
        (`/Game/TheBiogenSurvivor/Blueprints/BuildParts/BP_MasterFarmBuildPart.BPI_AddWater` _asbp_master_farm_build_part (* DeltaSeconds (`self.RainIntensity`)))))))

(event `self.RainBox.OnComponentBeginOverlap`
  (params (OverlappedComponent :type "PrimitiveComponent Object Reference") (OtherActor :type "Actor Object Reference") (OtherComp :type "PrimitiveComponent Object Reference") (OtherBodyIndex :type Integer) (bFromSweep :type Boolean) (SweepResult :type "HitResult Structure (by ref)"))
  (bind _asbp_tbsmaster_character (cast `/Game/TheBiogenSurvivor/Blueprints/Character/BP_TBSMasterCharacter` OtherActor))
  (bind _returnvalue (`NiagaraFunctionLibrary.SpawnSystemAtLocation` "/Game/TheBiogenSurvivor/Effects/NS_Rain.NS_Rain" (`self.K2_GetActorLocation` _asbp_tbsmaster_character)))
  (bind _output_get (set `/Game/TheBiogenSurvivor/Blueprints/Character/BP_TBSMasterCharacter.WeatherEffect` _returnvalue _asbp_tbsmaster_character))
  (bind _returnvalue_2 (`GameplayStatics.SpawnSoundAttached` "/Game/Audio/Environment/A_Rain_Cue.A_Rain_Cue" _output_get "None" (0.0 0.0 0.0) (struct) "KeepRelativeOffset" false 1.0 1.0 0.0 null null))
  (set `self.RainSound` _returnvalue_2))

(event `self.RainBox.OnComponentEndOverlap`
  (params (OverlappedComponent :type "PrimitiveComponent Object Reference") (OtherActor :type "Actor Object Reference") (OtherComp :type "PrimitiveComponent Object Reference") (OtherBodyIndex :type Integer))
  (bind _rainsound (`self.RainSound`))
  (`|ExecutionSequence`
    (:`then_0`
      (`/Engine/EditorBlueprintResources/StandardMacros.IsValid` _rainsound
        (:`Is Valid`
          (`AudioComponent.Stop` _rainsound)
          (`ActorComponent.K2_DestroyComponent` _rainsound))))
    (:`then_1`
      (bind _asbp_tbsmaster_character (cast `/Game/TheBiogenSurvivor/Blueprints/Character/BP_TBSMasterCharacter` OtherActor))
      (`ActorComponent.K2_DestroyComponent` (`/Game/TheBiogenSurvivor/Blueprints/Character/BP_TBSMasterCharacter.WeatherEffect` _asbp_tbsmaster_character)))))

(fn `SetRainLocation`
  (params (Player :type "/Game/TheBiogenSurvivor/Blueprints/Character/BP_TBSMasterCharacter Object Reference"))
  (bind _weathereffect (`/Game/TheBiogenSurvivor/Blueprints/Character/BP_TBSMasterCharacter.WeatherEffect` Player))
  (if (and (`KismetSystemLibrary.IsValid` _weathereffect) (`KismetSystemLibrary.IsValid` Player))
    (`SceneComponent.K2_SetWorldLocation` _weathereffect (`self.K2_GetActorLocation` Player) false false)))

(fn `UpdateRainIntensity`
  (params (Intensity :type "Float (double-precision)"))
  (bind _rainsound (`self.RainSound`))
  (bind _output_get (set `self.RainIntensity` Intensity))
  (`/Engine/EditorBlueprintResources/StandardMacros.IsValid` _rainsound
    (:`Is Valid`
      (`AudioComponent.SetVolumeMultiplier` _rainsound (`KismetMathLibrary.Lerp` 0.0 1.0 _output_get)))
    (:`Is Not Valid`
      _))
  (for _array_element (`PrimitiveComponent.GetOverlappingActors` (`self.RainBox`) "/Game/TheBiogenSurvivor/Blueprints/Character/BP_TBSMasterCharacter.BP_TBSMasterCharacter_C")
    (bind _asbp_tbsmaster_character (cast `/Game/TheBiogenSurvivor/Blueprints/Character/BP_TBSMasterCharacter` _array_element))
    (`NiagaraComponent.SetVariableFloat` (`/Game/TheBiogenSurvivor/Blueprints/Character/BP_TBSMasterCharacter.WeatherEffect` _asbp_tbsmaster_character) "User.SpawnRate" (* _output_get 500.0))))

(fn `UserConstructionScript`)