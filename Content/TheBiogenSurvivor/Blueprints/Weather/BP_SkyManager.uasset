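; Sky manager actor that runs a dynamic day cycle by rotating the Sun's pitch over time and wrapping it at 360 degrees.
; Tick updates the sky sphere and scales sun and skylight intensity from sun pitch; it is disabled at BeginPlay without a valid, dynamic Sun.
; It registers with the game mode's SGK save system, retrying if missing, but loading found level data just zeroes the sun rotation.
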(event `self.ReceiveBeginPlay`
  (set `self.SunCurrentRotation` (`self.SunDefaultRotation`))
  (`self.InitializeComponentSaveSystem`)
  (if (not (and (`KismetSystemLibrary.IsValid` (`self.Sun`)) (`self.DynamicSun`)))
    (`self.SetActorTickEnabled` false)))

(event `self.ReceiveTick`
  (params (DeltaSeconds :type "Float (single-precision)"))
  (bind (_suncurrentrotation_roll _suncurrentrotation_pitch) (`KismetMathLibrary.BreakRotator` (`self.SunCurrentRotation`)))
  (bind (_suncurrentrotation_roll_2 _suncurrentrotation_pitch_2) (`KismetMathLibrary.BreakRotator` (`self.SunCurrentRotation`)))
  (bind (_suncurrentrotation_roll_3 _suncurrentrotation_pitch_3 _suncurrentrotation_yaw) (`KismetMathLibrary.BreakRotator` (`self.SunCurrentRotation`)))
  (bind _returnvalue (/ (- 175.0 (`KismetMathLibrary.FClamp` (+ (.pitch (`self.K2_GetActorRotation` (`self.Sun`))) 90.0) 0.0 175.0)) 175.0))
  (if (`self.DynamicSun`)
    (bind _output_get (set `self.SunCurrentRotation` (`KismetMathLibrary.MakeRotator` 0.0 (`KismetMathLibrary.FClamp` (+ (* DeltaSeconds (`self.SunSpeed`)) _suncurrentrotation_pitch) 0.0 360.0))))
    (`self.K2_SetActorRotation` (`self.Sun`) _output_get false)
    (`/Engine/EngineSky/BP_Sky_Sphere.UpdateSunDirection` (`self.SkySphere`))
    (`SkyLightComponent.SetIntensity` (`SkyLight.LightComponent` (`self.SkyLight`)) _returnvalue)
    (`LightComponent.SetIntensity` (`Light.LightComponent` (`self.Sun`)) (* _returnvalue 1.0))
    (if (>= _suncurrentrotation_pitch_2 360.0)
      (set `self.SunCurrentRotation` (`KismetMathLibrary.MakeRotator` _suncurrentrotation_roll_3 0.0 _suncurrentrotation_yaw)))))

(event `/Game/SurvivalGameKitV2/Blueprints/Other/Interfaces/BP_SGKSaveInterface.SGKSave`
  (params (Save :type "/Game/SurvivalGameKitV2/Blueprints/Saving/BP_SGKSaveGame Object Reference"))
  (`self.SaveComponentData` Save))

(event `InitializeComponentSaveSystem`
  (bind _savegame (message `/Game/SurvivalGameKitV2/Blueprints/Other/Interfaces/BP_SGKGameModeInterface.SGK GetSaveGame` (`GameplayStatics.GetGameMode`) :!label _label))
  (bind _output_get (set `self.SaveSystem` _savegame))
  (`/Engine/EditorBlueprintResources/StandardMacros.IsValid` _output_get
    (:`Is Valid`
      (`KismetArrayLibrary.Array_AddUnique` (`/Game/SurvivalGameKitV2/Blueprints/Saving/BP_SaveSystem.SaveActors` (`self.SaveSystem`)) self)
      (add `/Game/SurvivalGameKitV2/Blueprints/Saving/BP_SaveSystem.LoadData` (`self.SaveSystem`) (delegate `LoadComponent`))
      (if (`/Game/SurvivalGameKitV2/Blueprints/Saving/BP_SaveSystem.PlayerLoadSave` (`self.SaveSystem`))
        (`self.LoadComponentData` (`/Game/SurvivalGameKitV2/Blueprints/Saving/BP_SaveSystem.LoadedSaveGameData` (`self.SaveSystem`)))))
    (:`Is Not Valid`
      (`/Engine/EditorBlueprintResources/StandardMacros.Do N` 10
        (:`Exit`
          (`KismetSystemLibrary.Delay` 0.2)
          (goto _label))))))

(event `LoadComponent`
  (params (SaveGame :type "/Game/SurvivalGameKitV2/Blueprints/Saving/BP_SGKSaveGame Object Reference"))
  (`self.InGameLoadComponentData` SaveGame))

(fn `Debug`
  (bind (_suncurrentrotation_roll _suncurrentrotation_pitch) (`KismetMathLibrary.BreakRotator` (`self.SunCurrentRotation`)))
  (`KismetSystemLibrary.PrintString` (`KismetStringLibrary.Concat_StrStr` "Sun Current Pitch: " (`KismetStringLibrary.Conv_DoubleToString` _suncurrentrotation_pitch)) true false (struct :`R` 1.0 :`A` 1.0) 0.1)
  (return))

(fn `InGameLoadComponentData`
  (params (Save :type "/Game/SurvivalGameKitV2/Blueprints/Saving/BP_SGKSaveGame Object Reference"))
  (`self.LoadComponentData` Save))

(fn `LoadComponentData`
  (params (SaveGame :type "/Game/SurvivalGameKitV2/Blueprints/Saving/BP_SGKSaveGame Object Reference"))
  (returns (LoadComplete :type Boolean))
  (locals (StorageSaveDataL :type "/Game/SurvivalGameKitV2/Blueprints/Other/Structs/S_LevelSaveData Structure"))
  (bind _returnvalue (`GameplayStatics.GetCurrentLevelName` true))
  (bind _savefound (`/Game/SurvivalGameKitV2/Blueprints/Saving/BP_SGKSaveGame.SelectLevelSaveData` (`local.SaveGame`) _returnvalue))
  (if _savefound
    (set `self.SunCurrentRotation` (struct))
    (return true)
    (else
      (return false))))

(fn `SaveComponentData`
  (params (SaveGame :type "/Game/SurvivalGameKitV2/Blueprints/Saving/BP_SGKSaveGame Object Reference"))
  (locals (LevelSaveDataL :type "/Game/SurvivalGameKitV2/Blueprints/Other/Structs/S_LevelSaveData Structure"))
  (bind _returnvalue (`GameplayStatics.GetCurrentLevelName` true))
  (bind (_savefound _levelsavedata) (`/Game/SurvivalGameKitV2/Blueprints/Saving/BP_SGKSaveGame.SelectLevelSaveData` (`local.SaveGame`) _returnvalue))
  (if _savefound
    (set `local.LevelSaveDataL` _levelsavedata)
    (else
      (setmembers `/Game/SurvivalGameKitV2/Blueprints/Other/Structs/S_LevelSaveData` :`StructRef` (`local.LevelSaveDataL`) :`Level Name` _returnvalue)))
  (bind _structout (setmembers `/Game/SurvivalGameKitV2/Blueprints/Other/Structs/S_LevelSaveData` :`StructRef` (`local.LevelSaveDataL`)))
  (`/Game/SurvivalGameKitV2/Blueprints/Saving/BP_SGKSaveGame.SetLevelData` (`local.SaveGame`) _structout))

(fn `UserConstructionScript`)