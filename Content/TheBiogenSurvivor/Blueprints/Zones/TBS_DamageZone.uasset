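; TBS_DamageZone is a damage volume that overrides its parent's DamageOverlappingActors so player mutations can reduce or negate the damage.
; When enabled with positive damage, it sends an SGK damage message to each actor overlapping DamageZone.
; For master characters, damage is scaled by the controller's mutation modifier for that damage type and rounded; those without an SGK controller are not damaged.
; Other actors take base damage.
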(fn `DamageOverlappingActors`
  (locals (HasMutationL :type Boolean) (DamageActorL :type "Actor Object Reference"))
  (if (`self.Enabled`)
    (if (> (`self.Damage`) 0)
      (for _array_element (`PrimitiveComponent.GetOverlappingActors` (`self.DamageZone`) null)
        (bind _output_get (set `local.DamageActorL` _array_element))
        ;[1 1 1] Check if this is a character, and if the character has a mutation that negates the damage
        (bind _asbp_tbsmaster_character (cast `/Game/TheBiogenSurvivor/Blueprints/Character/BP_TBSMasterCharacter` _output_get)
          (:`then`
            (bind _asbp_sgkcontroller (cast `/Game/SurvivalGameKitV2/Blueprints/Characters/BP_SGKController` (`Pawn.GetController` _asbp_tbsmaster_character)))
            (bind _modifier (`/Game/TheBiogenSurvivor/Blueprints/Other/Interfaces/BP_TBSFunctions.TBS GetMutationDamageModifier` _asbp_sgkcontroller (`self.DamageType`)))
            (message `/Game/SurvivalGameKitV2/Blueprints/Other/Interfaces/BP_SGKDamageInterface.SGK Damage` (`local.DamageActorL`) (`KismetMathLibrary.Conv_Int64ToInt` (`KismetMathLibrary.Round64` (* (`self.Damage`) _modifier))) null null (`self.DamageType`) "NewEnumerator6"))
          (:`CastFailed`
            (message `/Game/SurvivalGameKitV2/Blueprints/Other/Interfaces/BP_SGKDamageInterface.SGK Damage` (`local.DamageActorL`) (`self.Damage`) null null (`self.DamageType`) "NewEnumerator6")))))))

(fn `UserConstructionScript`
  (`parent.UserConstructionScript`))