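; Save game for The Biogen Survivor that overrides player saving to record stats, location, recipes, equipment and inventory by player name.
; Dead characters are skipped, and a missing character component falls back to the last known transform.
; Nested containers and weapon attachments are flattened into an indexed list that grows while it is processed.
; SavePlayerMutations packs mutation data into a struct, but is called here without input and its result is unused.
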(fn `SavePlayerInventory`
  (params (PlayerInventory :type "/Game/SurvivalGameKitV2/Blueprints/Components/BP_PlayerInventory Object Reference") (Level :type String))
  (locals (PlayerSaveL :type "/Game/SurvivalGameKitV2/Blueprints/Other/Structs/S_PlayerSave Structure") (CurrentInvL :type "/Game/SurvivalGameKitV2/Blueprints/Other/Structs/S_OtherInvSaves Structure") (InvSlotL :type "/Game/SurvivalGameKitV2/Blueprints/Other/Structs/S_InvSlot Structure") (NewInvSlotElementL :type "/Game/SurvivalGameKitV2/Blueprints/Other/Structs/S_InvSaveSlot Structure") (OtherInventoryL :type "/Game/SurvivalGameKitV2/Blueprints/Components/BP_MasterInventory Object Reference") (OtherInventorySavesL :type "Array of /Game/SurvivalGameKitV2/Blueprints/Other/Structs/S_InvSave Structure") (EquipmentSlotL :type "/Game/SurvivalGameKitV2/Blueprints/Other/Enum/E_EquipmentType Enum"))
  (bind _playerinventory (`local.PlayerInventory`))
  (bind _otherinventoryl (`local.OtherInventoryL`))
  (bind _playerinventory_2 (`local.PlayerInventory`))
  (bind _returnvalue (`GameplayStatics.GetObjectClass` _otherinventoryl))
  (bind _sgkcharacter (`/Game/SurvivalGameKitV2/Blueprints/Components/BP_PlayerInventory.SGKCharacter` _playerinventory_2))
  (bind ((`ID_2_84C2CB8945979246059C568DCD463423` _id) (`Amount_5_62DB2267439500D86A52E0B2266494D2` _amount) (`QuickBindIndex_16_7A1D8FC742EA4742106A33A874F67F34` _quickbindindex) (`Rotated_18_66B00C8648A7E3BEB56C4282929D015D` _rotated) (`UseAmount_21_73BF7A6447A384E099761EA48F7DB753` _useamount) (`Durability_30_E9AF67CA4E71F502EF4B18A440FA0385` _durability) (`DecayTime_33_E35E189B4E5F129EEECA28AE05E99A93` _decaytime)) (break `/Game/SurvivalGameKitV2/Blueprints/Other/Structs/S_InvItem` (`.Item_10_95D912F14C7740665FD844AF7EA87327` (break `/Game/SurvivalGameKitV2/Blueprints/Other/Structs/S_InvSlot` (`local.InvSlotL`)))))
  ;[1 1 1] Check player character isnt dead
  (bind _charactercomponent (`/Game/SurvivalGameKitV2/Blueprints/Components/BP_PlayerInventory.CharacterComponent` PlayerInventory)
    (:`then`
      (if (not (`/Game/SurvivalGameKitV2/Blueprints/Components/BP_CharacterComponent.CharacterDead` _charactercomponent))
        ;[1 1 1] Set player stats to save game
        (setmembers `/Game/SurvivalGameKitV2/Blueprints/Other/Structs/S_PlayerSave` :`StructRef` (`local.PlayerSaveL`) :`Name` (`/Game/SurvivalGameKitV2/Blueprints/Components/BP_PlayerInventory.PlayerName` _playerinventory_2) :`Health` (`/Game/SurvivalGameKitV2/Blueprints/Components/BP_PlayerInventory.CurrentHealth` _playerinventory_2) :`Hunger` (`/Game/SurvivalGameKitV2/Blueprints/Components/BP_PlayerInventory.CurrentHunger` _playerinventory_2) :`Thirst` (`/Game/SurvivalGameKitV2/Blueprints/Components/BP_PlayerInventory.CurrentThirst` _playerinventory_2) :`ItemCount` (`/Game/SurvivalGameKitV2/Blueprints/Components/BP_MasterInventory.ItemCount` _playerinventory_2) :`Weight` (`/Game/SurvivalGameKitV2/Blueprints/Components/BP_MasterInventory.CurrentWeight` _playerinventory_2) :`Location` (`Actor.K2_GetActorLocation` _sgkcharacter) :`Rotation` (`Actor.K2_GetActorRotation` _sgkcharacter) :`RespawnPoint` (`/Game/SurvivalGameKitV2/Blueprints/Components/BP_PlayerInventory.RespawnPointName` _playerinventory_2) :`LastLevel` (`local.Level`))
        ;[1 1 1] Set players known recipe to save game
        (for _array_element (`/Game/SurvivalGameKitV2/Blueprints/Components/BP_PlayerInventory.CraftingRecipes` (`local.PlayerInventory`)) :!label _label
          (`KismetArrayLibrary.Array_Add` (`.Recipes_38_88EA9C334CE363FE1A4C31BEEA09F22F` (break `/Game/SurvivalGameKitV2/Blueprints/Other/Structs/S_PlayerSave` (`local.PlayerSaveL`))) (`.RowName` (break `DataTableRowHandle` _array_element))))
        ;[1 1 1] Go though player inventory and get all items and there data then set it to save game
        (bind (_inventorysavedata _newotherinventories) (`self.GatherInventoryData` (`/Game/SurvivalGameKitV2/Blueprints/Components/BP_MasterInventory.Inventory` (`local.PlayerInventory`)) (`local.OtherInventorySavesL`)))
        (set `local.OtherInventorySavesL` _newotherinventories)
        (setmembers `/Game/SurvivalGameKitV2/Blueprints/Other/Structs/S_EquipmentSave` :`StructRef` (`.EquipmentSave_22_5DDA6D314B8E0EFEA5EAC280E49BCDFD` (break `/Game/SurvivalGameKitV2/Blueprints/Other/Structs/S_PlayerSave` (`local.PlayerSaveL`))) :`Inventory` _inventorysavedata)
        ;[1 1 1] Go though player inventory and get all equipment items and there data then set it to save game
        (bind (_equipmentsaveslots _newotherinventories_2) (`self.SaveEquipmentSlots` (`local.PlayerInventory`) (`local.OtherInventorySavesL`)))
        (setmembers `/Game/SurvivalGameKitV2/Blueprints/Other/Structs/S_EquipmentSave` :`StructRef` (`.EquipmentSave_22_5DDA6D314B8E0EFEA5EAC280E49BCDFD` (break `/Game/SurvivalGameKitV2/Blueprints/Other/Structs/S_PlayerSave` (`local.PlayerSaveL`))) :`EquipmentSlots` _equipmentsaveslots)
        (bind _output_get (set `local.OtherInventorySavesL` _newotherinventories_2))
        ;[1 1 1] Go though player inventory and get all weapon items and there data then set it to save game
        (bind (_weaponsaveslots _newotherinventories_3) (`self.SaveWeaponSlots` (`local.PlayerInventory`) _output_get))
        (set `local.OtherInventorySavesL` _newotherinventories_3)
        (setmembers `/Game/SurvivalGameKitV2/Blueprints/Other/Structs/S_EquipmentSave` :`StructRef` (`.EquipmentSave_22_5DDA6D314B8E0EFEA5EAC280E49BCDFD` (break `/Game/SurvivalGameKitV2/Blueprints/Other/Structs/S_PlayerSave` (`local.PlayerSaveL`))) :`WeaponSlots` _weaponsaveslots)
        ;[1 1 1] Loop though all container items inventories to find items and other items with containers
        (for _array_element_2 (`local.OtherInventorySavesL`)
          (bind (_index _inventory) (break `/Game/SurvivalGameKitV2/Blueprints/Other/Structs/S_InvSave` _array_element_2))
          (bind _output_get_2 (set `local.OtherInventoryL` _inventory))
          (`/Engine/EditorBlueprintResources/StandardMacros.IsValid` _output_get_2
            (:`Is Valid`
              (bind _asbp_master_item_inventory (cast `/Game/SurvivalGameKitV2/Blueprints/Components/BP_MasterItemInventory` _output_get_2)
                (:`then`
                  (setmembers `/Game/SurvivalGameKitV2/Blueprints/Other/Structs/S_OtherInvSaves` :`StructRef` (`local.CurrentInvL`) :`Index` _index :`Code` (`/Game/SurvivalGameKitV2/Blueprints/Components/BP_MasterItemInventory.SelfItem` _asbp_master_item_inventory)))
                (:`CastFailed`
                  (setmembers `/Game/SurvivalGameKitV2/Blueprints/Other/Structs/S_OtherInvSaves` :`StructRef` (`local.CurrentInvL`) :`Index` _index)))
              (for _array_element_3 (`/Game/SurvivalGameKitV2/Blueprints/Components/BP_MasterInventory.Inventory` (`local.OtherInventoryL`))
                (bind _output_get_3 (set `local.InvSlotL` _array_element_3))
                (bind ((`RootIndex_4_31C49987405FF01267287D9E3381FC5E` _rootindex) (`SelfIndex_2_277281E743D41F5A7B4963B58ABB6819` _selfindex) (`Item_10_95D912F14C7740665FD844AF7EA87327` _item)) (break `/Game/SurvivalGameKitV2/Blueprints/Other/Structs/S_InvSlot` _output_get_3))
                ;[1 1 1] Only check for full slots, then set item details
                (if (== _rootindex _selfindex)
                  (if (> (`.Amount_5_62DB2267439500D86A52E0B2266494D2` (break `/Game/SurvivalGameKitV2/Blueprints/Other/Structs/S_InvItem` _item)) 0)
                    (set `local.NewInvSlotElementL` (make `/Game/SurvivalGameKitV2/Blueprints/Other/Structs/S_InvSaveSlot` _id _amount _quickbindindex _rotated _useamount _durability (`.RootIndex_4_31C49987405FF01267287D9E3381FC5E` (break `/Game/SurvivalGameKitV2/Blueprints/Other/Structs/S_InvSlot` (`local.InvSlotL`))) -1 _decaytime))
                    ;[1 1 1] Check if item is container, if so add it to other inventory for saving later then add item to current containers save
                    (`/Engine/EditorBlueprintResources/StandardMacros.IsValid` (`.MasterInventory_8_17FFB7D341FAF2689C1BABA12E3BA9F5` (break `/Game/SurvivalGameKitV2/Blueprints/Other/Structs/S_InvItem` (`.Item_10_95D912F14C7740665FD844AF7EA87327` (break `/Game/SurvivalGameKitV2/Blueprints/Other/Structs/S_InvSlot` (`local.InvSlotL`)))))
                      (:`Is Valid`
                        (bind _returnvalue_2 (`KismetArrayLibrary.Array_Add` (`local.OtherInventorySavesL`)))
                        (`KismetArrayLibrary.Array_Set` (`local.OtherInventorySavesL`) _returnvalue_2 (make `/Game/SurvivalGameKitV2/Blueprints/Other/Structs/S_InvSave` _returnvalue_2 (`.MasterInventory_8_17FFB7D341FAF2689C1BABA12E3BA9F5` (break `/Game/SurvivalGameKitV2/Blueprints/Other/Structs/S_InvItem` (`.Item_10_95D912F14C7740665FD844AF7EA87327` (break `/Game/SurvivalGameKitV2/Blueprints/Other/Structs/S_InvSlot` (`local.InvSlotL`)))))) true)
                        (setmembers `/Game/SurvivalGameKitV2/Blueprints/Other/Structs/S_InvSaveSlot` :`StructRef` (`local.NewInvSlotElementL`) :`InvIndex` _returnvalue_2))
                      (:`Is Not Valid`
                        _))
                    (`KismetArrayLibrary.Array_Add` (`.Inventory_7_7766F73341404F28636081A6E71E7F86` (break `/Game/SurvivalGameKitV2/Blueprints/Other/Structs/S_OtherInvSaves` (`local.CurrentInvL`))) (`local.NewInvSlotElementL`))
                    (set `local.NewInvSlotElementL` (struct)))))
              ;[1 1 1] Check if item is a weapon, if so then save weapon attachments and set that data to save then set inventory weight and item count and add the inventory save to save game
              (if (or (`KismetMathLibrary.ClassIsChildOf` _returnvalue "/Game/SurvivalGameKitV2/Blueprints/Components/BP_WeaponInventory.BP_WeaponInventory_C") (== _returnvalue "/Game/SurvivalGameKitV2/Blueprints/Components/BP_WeaponInventory.BP_WeaponInventory_C"))
                (bind _asbp_weapon_inventory (cast `/Game/SurvivalGameKitV2/Blueprints/Components/BP_WeaponInventory` _otherinventoryl)
                  (:`then`
                    (bind (_otherinventorysavesl1 _attachmentsaveslotsl1) (`self.GatherAttachmentData` _asbp_weapon_inventory (`local.OtherInventorySavesL`)))
                    (set `local.OtherInventorySavesL` _otherinventorysavesl1)
                    (bind _structout (setmembers `/Game/SurvivalGameKitV2/Blueprints/Other/Structs/S_OtherInvSaves` :`StructRef` (`local.CurrentInvL`) :`Weight` (`/Game/SurvivalGameKitV2/Blueprints/Components/BP_MasterInventory.CurrentWeight` (`local.OtherInventoryL`)) :`ItemCount` (`/Game/SurvivalGameKitV2/Blueprints/Components/BP_MasterInventory.ItemCount` (`local.OtherInventoryL`)) :`Attachments` _attachmentsaveslotsl1 :`FireMode` (`/Game/SurvivalGameKitV2/Blueprints/Components/BP_WeaponInventory.WeaponFireMode` _asbp_weapon_inventory)))
                    (set `local.CurrentInvL` _structout))
                  (:`CastFailed`
                    (setmembers `/Game/SurvivalGameKitV2/Blueprints/Other/Structs/S_OtherInvSaves` :`StructRef` (`local.CurrentInvL`) :`Weight` (`/Game/SurvivalGameKitV2/Blueprints/Components/BP_MasterInventory.CurrentWeight` (`local.OtherInventoryL`)) :`ItemCount` (`/Game/SurvivalGameKitV2/Blueprints/Components/BP_MasterInventory.ItemCount` (`local.OtherInventoryL`)) :!label _label_2)))
                (else
                  (goto _label_2)))
              (`KismetArrayLibrary.Array_Add` (`.OtherInventorys_15_02C7D96443E404994290448C883E6183` (break `/Game/SurvivalGameKitV2/Blueprints/Other/Structs/S_EquipmentSave` (`.EquipmentSave_22_5DDA6D314B8E0EFEA5EAC280E49BCDFD` (break `/Game/SurvivalGameKitV2/Blueprints/Other/Structs/S_PlayerSave` (`local.PlayerSaveL`))))) (`local.CurrentInvL`))
              (set `local.CurrentInvL` (struct)))))
        (`self.SavePlayerMutations` null)
        ;[1 1 1] Check if save exists for player already and save to it, if not the create new save for player data
        (for (_array_element_4 _array_index) (`self.PlayerSaves`)
          (if (`KismetTextLibrary.EqualEqual_TextText` (`.Name_7_840382AF42E3FEEB857A569E1725A821` (break `/Game/SurvivalGameKitV2/Blueprints/Other/Structs/S_PlayerSave` _array_element_4)) (`.Name_7_840382AF42E3FEEB857A569E1725A821` (break `/Game/SurvivalGameKitV2/Blueprints/Other/Structs/S_PlayerSave` (`local.PlayerSaveL`))))
            (`KismetArrayLibrary.Array_Set` (`self.PlayerSaves`) _array_index (`local.PlayerSaveL`) true)
            (return)))
        (`KismetArrayLibrary.Array_Add` (`self.PlayerSaves`) (`local.PlayerSaveL`))))
    (:`else`
      (setmembers `/Game/SurvivalGameKitV2/Blueprints/Other/Structs/S_PlayerSave` :`StructRef` (`local.PlayerSaveL`) :`Name` (`/Game/SurvivalGameKitV2/Blueprints/Components/BP_PlayerInventory.PlayerName` _playerinventory) :`Health` (`/Game/SurvivalGameKitV2/Blueprints/Components/BP_PlayerInventory.CurrentHealth` _playerinventory) :`Hunger` (`/Game/SurvivalGameKitV2/Blueprints/Components/BP_PlayerInventory.CurrentHunger` _playerinventory) :`Thirst` (`/Game/SurvivalGameKitV2/Blueprints/Components/BP_PlayerInventory.CurrentThirst` _playerinventory) :`ItemCount` (`/Game/SurvivalGameKitV2/Blueprints/Components/BP_MasterInventory.ItemCount` _playerinventory) :`Weight` (`/Game/SurvivalGameKitV2/Blueprints/Components/BP_MasterInventory.CurrentWeight` _playerinventory) :`Location` (`/Game/SurvivalGameKitV2/Blueprints/Components/BP_PlayerInventory.LastCharacterLocation` _playerinventory) :`Rotation` (`/Game/SurvivalGameKitV2/Blueprints/Components/BP_PlayerInventory.LastCharacterRotation` _playerinventory) :`RespawnPoint` (`/Game/SurvivalGameKitV2/Blueprints/Components/BP_PlayerInventory.RespawnPointName` _playerinventory) :`LastLevel` (`local.Level`))
      (goto _label))))

(fn `SavePlayerMutations`
  (params (PlayerMutations :type "/Game/TheBiogenSurvivor/Blueprints/Components/BP_PlayerMutations_TBS Object Reference"))
  (returns (MutationsSave :type "/Game/TheBiogenSurvivor/Blueprints/Other/Structs/S_MutationsSave Structure"))
  (locals (MutationsSaveL :type "/Game/TheBiogenSurvivor/Blueprints/Other/Structs/S_MutationsSave Structure"))
  (bind _playermutations (`local.PlayerMutations`))
  (`/Engine/EditorBlueprintResources/StandardMacros.IsValid` PlayerMutations
    (:`Is Valid`
      (bind _structout (setmembers `/Game/TheBiogenSurvivor/Blueprints/Other/Structs/S_MutationsSave` :`StructRef` (`local.MutationsSaveL`) :`ActiveMutations` (`/Game/TheBiogenSurvivor/Blueprints/Components/BP_PlayerMutations_TBS.ActiveMutations` _playermutations) :`ActiveBirthDefects` (`/Game/TheBiogenSurvivor/Blueprints/Components/BP_PlayerMutations_TBS.ActiveBirthDefects` _playermutations) :`NextMutations` (`/Game/TheBiogenSurvivor/Blueprints/Components/BP_PlayerMutations_TBS.NextMutations` _playermutations) :`ActiveCancers` (`/Game/TheBiogenSurvivor/Blueprints/Components/BP_PlayerMutations_TBS.ActiveCancers` _playermutations)))
      (return _structout))))