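; Custom game state that runs the time-of-day clock for the level's BP_CustomSunSky.
; On BeginPlay it finds the sun sky actor and converts its hours, minutes and seconds into a running seconds total.
; A looping timer, paced by a ticks-per-second variable, advances that total by a configurable step and writes the time back to the sun sky.
; The total resets to zero upon reaching a full day.
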(event `self.ReceiveBeginPlay`
  (bind _returnvalue (`GameplayStatics.GetActorOfClass` "/Game/TheBiogenSurvivor/SunSky/BP_CustomSunSky.BP_CustomSunSky_C"))
  (bind _output_get (set `self.SunSky` _returnvalue))
  (set `self.TimeOfDaySeconds` (`KismetMathLibrary.FTrunc` (`KismetMathLibrary.GetTotalSeconds` (`KismetMathLibrary.MakeTimespan` 0 (`/Game/TheBiogenSurvivor/SunSky/BP_CustomSunSky.Hours` _output_get) (`/Game/TheBiogenSurvivor/SunSky/BP_CustomSunSky.Minutes` _output_get) (`/Game/TheBiogenSurvivor/SunSky/BP_CustomSunSky.Seconds` _output_get)))))
  (`KismetSystemLibrary.K2_SetTimerDelegate` (delegate `TimeUpdate`) (/ 1.0 (`self.TimeAmountToTickPerSec`)) true))

(event `TimeUpdate`
  (bind _sunsky (`self.SunSky`))
  (bind _output_get (set `self.TimeOfDaySeconds` (+ (`self.TimeOfDaySeconds`) (`self.AmountOfSecondsToAddPerTick`))))
  (bind (_days _hours _minutes _seconds) (`KismetMathLibrary.BreakTimespan` (`KismetMathLibrary.MakeTimespan` 0 0 0 _output_get)))
  (set `/Game/TheBiogenSurvivor/SunSky/BP_CustomSunSky.Hours` _hours _sunsky)
  (set `/Game/TheBiogenSurvivor/SunSky/BP_CustomSunSky.Minutes` _minutes _sunsky)
  (set `/Game/TheBiogenSurvivor/SunSky/BP_CustomSunSky.Seconds` _seconds _sunsky)
  (if (>= (`self.TimeOfDaySeconds`) 86400)
    (set `self.TimeOfDaySeconds` 0)))

(fn `UserConstructionScript`)