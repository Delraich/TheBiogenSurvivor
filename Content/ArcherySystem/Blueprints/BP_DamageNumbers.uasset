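; BP_DamageNumbers is an archery system actor that shows a floating damage number and removes itself when the animation ends.
; On BeginPlay it passes the damage text and headshot flag to its WB_DamageNumber widget, then picks a random end offset and scale, with headshots scaling larger.
; A timeline moves the widget, scales it and fades it out, then destroys the actor.
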(event `self.ReceiveBeginPlay`
  (bind (_xoffsetminmax_x _xoffsetminmax_y) (`KismetMathLibrary.BreakVector2D` (`self.XOffsetMinMax`)))
  (bind (_yoffsetminmax_x _yoffsetminmax_y) (`KismetMathLibrary.BreakVector2D` (`self.YOffsetMinMax`)))
  (bind (_zoffsetminmax_x _zoffsetminmax_y) (`KismetMathLibrary.BreakVector2D` (`self.ZOffsetMinMax`)))
  (bind _endscale (`self.EndScale`))
  (bind _returnvalue (`SceneComponent.K2_GetComponentLocation` (`self.DefaultSceneRoot`)))
  ;[1 1 1] Communicate damage info
  (bind _aswb_damage_number (cast `/Game/ArcherySystem/Assets/Widgets/WB_DamageNumber` (`WidgetComponent.GetUserWidgetObject` (`self.Widget`))))
  (`TextBlock.SetText` (`/Game/ArcherySystem/Assets/Widgets/WB_DamageNumber.TextBlock_1` _aswb_damage_number) (`self.DamageNumbers`))
  (`/Game/ArcherySystem/Assets/Widgets/WB_DamageNumber.UpdateText` _aswb_damage_number (`self.Headshot?`))
  ;[1 1 1] Animate damage text
  (set `self.EndScale` (* (+ 0.5 (`KismetMathLibrary.RandomFloatInRange` 0.2 1.2)) (select `bool` (`self.Headshot?`) :`false` 0.5 :`true` 1.0)))
  (set `self.StartLocation` _returnvalue)
  (set `self.EndLocation` (+ _returnvalue (`KismetMathLibrary.MakeVector` (`KismetMathLibrary.RandomFloatInRange` _xoffsetminmax_x _xoffsetminmax_y) (`KismetMathLibrary.RandomFloatInRange` _yoffsetminmax_x _yoffsetminmax_y) (`KismetMathLibrary.RandomFloatInRange` _zoffsetminmax_x _zoffsetminmax_y)) (0.0 0.0 80.0)))
  (bind (_direction _newtrack_0 _newtrack_1) (`Timeline|Lerp` :!via `PlayFromStart`)
    (:`Update`
      (`SceneComponent.K2_SetWorldLocation` (`self.Widget`) (`KismetMathLibrary.VLerp` (`self.StartLocation`) (`self.EndLocation`) _newtrack_0) false false)
      (`Widget.SetRenderScale` _aswb_damage_number (`KismetMathLibrary.Conv_VectorToVector2D` (`KismetMathLibrary.VLerp` (0.5 0.5 0.5) (`KismetMathLibrary.MakeVector` _endscale _endscale _endscale) _newtrack_1)))
      (`Widget.SetRenderOpacity` (`/Game/ArcherySystem/Assets/Widgets/WB_DamageNumber.SizeBox_44` _aswb_damage_number) (`KismetMathLibrary.Lerp` 1.0 0.0 _newtrack_0)))
    (:`Finished`
      (`self.K2_DestroyActor`) ; I also set the lifespan to 2 seconds just in case this doesn't get called.
    )))

(fn `UserConstructionScript`)