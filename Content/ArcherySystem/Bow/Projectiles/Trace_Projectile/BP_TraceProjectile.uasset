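; BP_TraceProjectile is a visual arrow projectile for the bow in the archery system, flying between a given start and end location.
; A custom begin-play event, meant to work with dedicated servers, stores both points and rotates the arrow toward the target.
; A timeline at a set play rate lerps the arrow along the path without sweeping, then destroys the actor.
; The particle effect activates after a brief delay via MultiCastEnable.
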(event `MultiCastEnable`
  ;[0 0.4054 1] Beginplay
  (`ActorComponent.Activate` (`self.ParticleSystem`) false))

(event `BeginPlayCustom`
  (params (`Start Location` :type "Vector Structure") (EndLocation :type "Vector Structure"))
  ;[0 0.4054 1] Beginplay
  (set `self.Start Location` `Start Location`)
  (set `self.EndLocation` EndLocation)
  (`|ExecutionSequence`
    (:`then_0`
      (`KismetSystemLibrary.Delay` 0.05) ; A little delay makes it look a bit better.
      (`self.MultiCastEnable`))
    (:`then_1`
      (`SceneComponent.K2_SetWorldRotation` (`self.Arrow`) (`KismetMathLibrary.FindLookAtRotation` (`self.Start Location`) (`self.EndLocation`)) false false)
      (`TimelineComponent.SetPlayRate` (`self.MoveToEndLocation`) (`self.PlayRate`))
      (bind (_direction _arrow_shot) (`Timeline|MoveToEndLocation` :!via `PlayFromStart`)
        (:`Update`
          (`SceneComponent.K2_SetWorldLocation` (`self.Arrow`) (`KismetMathLibrary.VLerp` (`self.Start Location`) (`self.EndLocation`) _arrow_shot) false false))
        (:`Finished`
          (`self.K2_DestroyActor`))))))

(fn `UserConstructionScript`)